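; Debug actor for the tactical grid that overlays tile and pathfinding info as text and highlights discovered and analysed tiles.
; On BeginPlay it finds BP_Grid and binds to its tile and pathfinding update events.
; Toggle setters refresh all tiles, spawning one cached TextRenderActor per walkable tile, scaled to its longest entry, and removing unneeded ones.
; Highlights work by adding or removing tile states on the grid itself.
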(event EventBeginPlay
  (bind _returnvalue (Actor|GetActorOfClass "/Game/TacticalStrategy/Blueprints/Core/Grid/BP_Grid.BP_Grid_C"))
  (bind _output_get (Variables|Default|SetGrid _returnvalue))
  (EventDispatchers|AssignOnTileDataUpdated _output_get (EventDispatchers|CreateEvent :!event FUpdateTextonTile))
  (EventDispatchers|BindEventtoOnTileStateUpdated _output_get (EventDispatchers|CreateEvent :!event FUpdateStateonTile))
  (EventDispatchers|BindEventtoOnGridDestroyed _output_get (EventDispatchers|CreateEvent :!event FClearAllTextActors))
  (EventDispatchers|BindEventtoOnPathFindingDataUpdated (Variables|/Game/TacticalStrategy/Blueprints/Core/Grid/BP_Grid.BP_Grid_C|GetGridPathfinding (Variables|Default|GetGrid)) (EventDispatchers|CreateEvent :!event FUpdateStateonTile))
  (EventDispatchers|BindEventtoOnPathFindingDataCleared (Variables|/Game/TacticalStrategy/Blueprints/Core/Grid/BP_Grid.BP_Grid_C|GetGridPathfinding (Variables|Default|GetGrid)) (EventDispatchers|CreateEvent :!event FUpdateStateonAllTile))
  (EventDispatchers|BindEventtoOnPathFindingDataUpdated (Variables|/Game/TacticalStrategy/Blueprints/Core/Grid/BP_Grid.BP_Grid_C|GetGridPathfinding (Variables|Default|GetGrid)) (EventDispatchers|CreateEvent :!event FUpdateTextonTile))
  (EventDispatchers|BindEventtoOnPathFindingDataCleared (Variables|/Game/TacticalStrategy/Blueprints/Core/Grid/BP_Grid.BP_Grid_C|GetGridPathfinding (Variables|Default|GetGrid)) (EventDispatchers|CreateEvent :!event FUpdateTextonAllTiles)))

(fn ConstructionScript)

(fn FGetTextActor
  (params (Index :type Int%20Point%20Structure))
  (bind _output_get (LocalVariables|SetActor (.Value (Utilities|Map|Find (Variables|Default|GetSpawnTexts) Index))))
  (Utilities|IsValid _output_get
    (:Is%20Valid
      (return (LocalVariables|GetActor)))
    (:Is%20Not%20Valid
      (bind _returnvalue (Game|SpawnActorfromClass "/Script/Engine.TextRenderActor" (Math|Transform|MakeTransform "0, 0, 0" "0, 0, 0" "1.000000,1.000000,1.000000") "AlwaysSpawn" "MultiplyWithRoot" 0 0))
      (Utilities|IsValid _returnvalue
        (:Is%20Valid
          (LocalVariables|SetActor _returnvalue)
          (Utilities|Map|Add (Variables|Default|GetSpawnTexts) Index (LocalVariables|GetActor))
          (Actor|Tick|SetActorTickEnabled (LocalVariables|GetActor))
          (Collision|SetActorEnableCollision (LocalVariables|GetActor) false)
          (Rendering|Components|TextRender|SetHorizontalAlignment (Variables|/Script/Engine.TextRenderActor|GetTextRender (LocalVariables|GetActor)) "EHTA_Center")
          (Class|TextRenderComponent|SetVerticalAlignment (Variables|/Script/Engine.TextRenderActor|GetTextRender (LocalVariables|GetActor)) "EVRTA_TextCenter")
          (return (LocalVariables|GetActor)))
        (:Is%20Not%20Valid
          (return 0))))))

(fn FDestroyTextActor
  (params (Index :type Int%20Point%20Structure))
  (bind _output_get (LocalVariables|SetActor (.Value (Utilities|Map|Find (Variables|Default|GetSpawnTexts) Index))))
  (Utilities|IsValid _output_get
    (:Is%20Valid
      (Actor|DestroyActor _output_get)
      (Utilities|Map|Remove (Variables|Default|GetSpawnTexts) Index))))

(fn FClearAllTextActors
  (bind _values (Utilities|Map|Values (Variables|Default|GetSpawnTexts)))
  (for _array_element _values
    (Actor|DestroyActor _array_element))
  (Utilities|Map|Clear (Variables|Default|GetSpawnTexts)))

(fn FUpdateTextonTile
  (params (Index :type Int%20Point%20Structure))
  (bind _returnvalue (Utilities|String|ToString(Integer) (.y Index)))
  (bind _returnvalue_2 (Utilities|String|ToString(Integer) (.x Index)))
  (bind _returnvalue_3 (Utilities|String|Append _returnvalue_2 "," _returnvalue))
  (if (CallFunction|FWanttoDisplayAnyText)
    (Variables|Default|GetGrid
      (:then
        _)
      (:else
        (bind _returnvalue_4 (Actor|GetActorOfClass "/Game/TacticalStrategy/Blueprints/Core/Grid/BP_Grid.BP_Grid_C"))
        (Variables|Default|SetGrid _returnvalue_4)))
    (if (.ReturnValue (Utilities|Map|Find (Variables|/Game/TacticalStrategy/Blueprints/Core/Grid/BP_Grid.BP_Grid_C|GetGridTiles (Variables|Default|GetGrid)) Index))
      (LocalVariables|SetData (.Value (Utilities|Map|Find (Variables|/Game/TacticalStrategy/Blueprints/Core/Grid/BP_Grid.BP_Grid_C|GetGridTiles (Variables|Default|GetGrid)) Index)))
      (if (CallFunction|FIsTileTypeWalkable (.tiletype (LocalVariables|GetData)))
        (bind _textrender (CallFunction|FGetTextActor Index))
        (LocalVariables|SetTextRender _textrender)
        (Utilities|FlowControl|Sequence
          (:then_0
            (Utilities|FlowControl|Sequence
              (:then_0
                (if (Variables|Default|GetbSetShowTileIndexes)
                  (Utilities|Array|Add (LocalVariables|GetText) _returnvalue_3)
                  (Utilities|Array|Add (LocalVariables|GetTextLength) (Utilities|String|Len _returnvalue_3))))
              (:then_1
                (if (Variables|Default|GetbShowTileType)
                  (if (Utilities|Enum|NotEqual(Enum) (.tiletype (LocalVariables|GetData)) "NewEnumerator1")
                    (Utilities|Array|Add (LocalVariables|GetText) (Utilities|String|EnumtoString (.tiletype (LocalVariables|GetData))))
                    (Utilities|Array|Add (LocalVariables|GetTextLength) (Utilities|String|Len (Utilities|String|EnumtoString (.tiletype (LocalVariables|GetData))))))))
              (:then_2
                (if (Math|Boolean|ORBoolean (Variables|Default|GetbSetShowCostToEnterTile) (Variables|Default|GetbSetShowMinCostToTarget) (Variables|Default|GetbSetShowCostFromStart) (Variables|Default|GetbSetShowSortOrder))
                  (if (.ReturnValue (Utilities|Map|Find (Variables|/Game/TacticalStrategy/Blueprints/Core/Grid/BP_GridPathfinding.BP_GridPathfinding_C|GetPathFindingData (Variables|/Game/TacticalStrategy/Blueprints/Core/Grid/BP_Grid.BP_Grid_C|GetGridPathfinding (Variables|Default|GetGrid))) Index))
                    (LocalVariables|SetPathFindingData (.Value (Utilities|Map|Find (Variables|/Game/TacticalStrategy/Blueprints/Core/Grid/BP_GridPathfinding.BP_GridPathfinding_C|GetPathFindingData (Variables|/Game/TacticalStrategy/Blueprints/Core/Grid/BP_Grid.BP_Grid_C|GetGridPathfinding (Variables|Default|GetGrid))) Index)))
                    (Utilities|FlowControl|Sequence
                      (:then_0
                        (if (Variables|Default|GetbSetShowCostToEnterTile)
                          (Utilities|Array|Add (LocalVariables|GetText) (Utilities|String|Append "Enter: " (Utilities|String|ToString(Integer) (.CostToEnterTile (Utilities|Struct|BreakStruct_PathfindingData (LocalVariables|GetPathFindingData))))))
                          (Utilities|Array|Add (LocalVariables|GetTextLength) (Utilities|String|Len (Utilities|String|Append "Enter: " (Utilities|String|ToString(Integer) (.CostToEnterTile (Utilities|Struct|BreakStruct_PathfindingData (LocalVariables|GetPathFindingData)))))))))
                      (:then_1
                        (if (Variables|Default|GetbSetShowMinCostToTarget)
                          (if (!= (.MinimumCostToTarget (Utilities|Struct|BreakStruct_PathfindingData (LocalVariables|GetPathFindingData))) 99999)
                            (Utilities|Array|Add (LocalVariables|GetText) (Utilities|String|Append "Min: " (Utilities|String|ToString(Integer) (.MinimumCostToTarget (Utilities|Struct|BreakStruct_PathfindingData (LocalVariables|GetPathFindingData))))))
                            (Utilities|Array|Add (LocalVariables|GetTextLength) (Utilities|String|Len (Utilities|String|Append "Min: " (Utilities|String|ToString(Integer) (.MinimumCostToTarget (Utilities|Struct|BreakStruct_PathfindingData (LocalVariables|GetPathFindingData))))))))))
                      (:then_2
                        (if (Variables|Default|GetbSetShowCostFromStart)
                          (if (!= (.MinimumCostToTarget (Utilities|Struct|BreakStruct_PathfindingData (LocalVariables|GetPathFindingData))) 99999)
                            (Utilities|Array|Add (LocalVariables|GetText) (Utilities|String|Append "Start: " (Utilities|String|ToString(Integer) (.MinimumCostToTarget (Utilities|Struct|BreakStruct_PathfindingData (LocalVariables|GetPathFindingData))))))
                            (Utilities|Array|Add (LocalVariables|GetTextLength) (Utilities|String|Len (Utilities|String|Append "Start: " (Utilities|String|ToString(Integer) (.MinimumCostToTarget (Utilities|Struct|BreakStruct_PathfindingData (LocalVariables|GetPathFindingData))))))))))
                      (:then_3
                        (if (Variables|Default|GetbSetShowSortOrder)
                          (if (!= (Utilities|Array|FindItem (Variables|/Game/TacticalStrategy/Blueprints/Core/Grid/BP_GridPathfinding.BP_GridPathfinding_C|GetDiscoveredTileIndexes (Variables|/Game/TacticalStrategy/Blueprints/Core/Grid/BP_Grid.BP_Grid_C|GetGridPathfinding (Variables|Default|GetGrid))) Index) -1)
                            (Utilities|Array|Add (LocalVariables|GetText) (Utilities|String|Append "Sort: " (Utilities|String|ToString(Integer) (Utilities|Array|FindItem (Variables|/Game/TacticalStrategy/Blueprints/Core/Grid/BP_GridPathfinding.BP_GridPathfinding_C|GetDiscoveredTileIndexes (Variables|/Game/TacticalStrategy/Blueprints/Core/Grid/BP_Grid.BP_Grid_C|GetGridPathfinding (Variables|Default|GetGrid))) Index)) "( " (Utilities|String|ToString(Integer) (Utilities|Array|Get(acopy) (Variables|/Game/TacticalStrategy/Blueprints/Core/Grid/BP_GridPathfinding.BP_GridPathfinding_C|GetDiscoveredTileSortingCost (Variables|/Game/TacticalStrategy/Blueprints/Core/Grid/BP_Grid.BP_Grid_C|GetGridPathfinding (Variables|Default|GetGrid))) (Utilities|Array|FindItem (Variables|/Game/TacticalStrategy/Blueprints/Core/Grid/BP_GridPathfinding.BP_GridPathfinding_C|GetDiscoveredTileIndexes (Variables|/Game/TacticalStrategy/Blueprints/Core/Grid/BP_Grid.BP_Grid_C|GetGridPathfinding (Variables|Default|GetGrid))) Index))) " )"))
                            (Utilities|Array|Add (LocalVariables|GetTextLength) (Utilities|String|Len (Utilities|String|Append "Sort: " (Utilities|String|ToString(Integer) (Utilities|Array|FindItem (Variables|/Game/TacticalStrategy/Blueprints/Core/Grid/BP_GridPathfinding.BP_GridPathfinding_C|GetDiscoveredTileIndexes (Variables|/Game/TacticalStrategy/Blueprints/Core/Grid/BP_Grid.BP_Grid_C|GetGridPathfinding (Variables|Default|GetGrid))) Index)) "( " (Utilities|String|ToString(Integer) (Utilities|Array|Get(acopy) (Variables|/Game/TacticalStrategy/Blueprints/Core/Grid/BP_GridPathfinding.BP_GridPathfinding_C|GetDiscoveredTileSortingCost (Variables|/Game/TacticalStrategy/Blueprints/Core/Grid/BP_Grid.BP_Grid_C|GetGridPathfinding (Variables|Default|GetGrid))) (Utilities|Array|FindItem (Variables|/Game/TacticalStrategy/Blueprints/Core/Grid/BP_GridPathfinding.BP_GridPathfinding_C|GetDiscoveredTileIndexes (Variables|/Game/TacticalStrategy/Blueprints/Core/Grid/BP_Grid.BP_Grid_C|GetGridPathfinding (Variables|Default|GetGrid))) Index))) " )"))))))))))))
          (:then_1
            (if (> (Utilities|Array|Length (LocalVariables|GetText)) 0)
              (LocalVariables|GetTextRender
                (:then
                  (Rendering|Components|TextRender|SetText (Variables|/Script/Engine.TextRenderActor|GetTextRender (LocalVariables|GetTextRender)) (Utilities|Text|ToText(String) (Utilities|String|JoinStringArray (LocalVariables|GetText) " 
 ")))
                  (Transformation|SetActorTransform (LocalVariables|GetTextRender) (Math|Transform|MakeTransform (+ (.location (.transform (LocalVariables|GetData))) "0.000000,0.000000,1.000000") "90.000000,180.000000,0.000000" (Math|Conversions|ToVector(Float) (/ (.y (Variables|/Game/TacticalStrategy/Blueprints/Core/Grid/BP_Grid.BP_Grid_C|GetGrid%20Tile%20Size (Variables|Default|GetGrid))) (* (.MaxValue (Math|Integer|MaxOfIntArray (LocalVariables|GetTextLength))) 30))))))
                (:else))
              (else
                (CallFunction|FDestroyTextActor Index)))))
        (else
          (CallFunction|FDestroyTextActor Index :!label _label)))
      (else
        (goto _label)))))

(fn FUpdateTextonAllTiles
  (if (CallFunction|FWanttoDisplayAnyText)
    (bind _grid (Variables|Default|GetGrid)
      (:then
        (bind _keys (Utilities|Map|Keys (Variables|/Game/TacticalStrategy/Blueprints/Core/Grid/BP_Grid.BP_Grid_C|GetGridTiles _grid)))
        (for _array_element _keys
          (CallFunction|FUpdateTextonTile _array_element)))
      (:else))
    (else
      (CallFunction|FClearAllTextActors))))

(fn FWanttoDisplayAnyText
  (return (Math|Boolean|ORBoolean (Variables|Default|GetbSetShowTileIndexes) (Variables|Default|GetbSetShowCostToEnterTile) (Variables|Default|GetbSetShowMinCostToTarget) (Variables|Default|GetbSetShowCostFromStart) (Variables|Default|GetbSetShowSortOrder) (Variables|Default|GetbShowTileType))))

(fn FUpdateStateonTile
  (params (Index :type Int%20Point%20Structure))
  (Utilities|FlowControl|Sequence
    (:then_0
      (if (Variables|Default|GetbSetShowDiscoveredTiles)
        (if (Utilities|Array|ContainsItem (Variables|/Game/TacticalStrategy/Blueprints/Core/Grid/BP_GridPathfinding.BP_GridPathfinding_C|GetDiscoveredTileIndexes (Variables|/Game/TacticalStrategy/Blueprints/Core/Grid/BP_Grid.BP_Grid_C|GetGridPathfinding (Variables|Default|GetGrid))) Index)
          (Default|FAddStatetoTile (Variables|Default|GetGrid) Index "NewEnumerator6")
          (else
            (Default|FRemoveStatefromTile (Variables|Default|GetGrid) Index "NewEnumerator6" :!label _label)))
        (else
          (goto _label))))
    (:then_1
      (if (Variables|Default|GetbSetShowAnalysedTiles)
        (if (Utilities|Array|ContainsItem (Variables|/Game/TacticalStrategy/Blueprints/Core/Grid/BP_GridPathfinding.BP_GridPathfinding_C|GetAnalysedTileIndexes (Variables|/Game/TacticalStrategy/Blueprints/Core/Grid/BP_Grid.BP_Grid_C|GetGridPathfinding (Variables|Default|GetGrid))) Index)
          (Default|FAddStatetoTile (Variables|Default|GetGrid) Index "NewEnumerator7")
          (else
            (Default|FRemoveStatefromTile (Variables|Default|GetGrid) Index "NewEnumerator7" :!label _label_2)))
        (else
          (goto _label_2))))))

(fn FUpdateStateonAllTile
  (bind _grid (Variables|Default|GetGrid))
  (if (or (Variables|Default|GetbSetShowDiscoveredTiles) (Variables|Default|GetbSetShowAnalysedTiles))
    (bind _keys (Utilities|Map|Keys (Variables|/Game/TacticalStrategy/Blueprints/Core/Grid/BP_Grid.BP_Grid_C|GetGridTiles (Variables|Default|GetGrid))))
    (for _array_element _keys
      (CallFunction|FUpdateStateonTile _array_element))
    (else
      (Default|FClearStatefromTiles _grid "NewEnumerator6")
      (Default|FClearStatefromTiles _grid "NewEnumerator7"))))

(fn FSetShowTileText
  (params (bSetShowTileIndexes :type Boolean) (bSetShowCostToEnterTile :type Boolean) (bSetShowMinCostToTarget :type Boolean) (bSetShowCostFromStart :type Boolean) (bSetShowSortOrder :type Boolean) (bShowTileType :type Boolean))
  (Utilities|FlowControl|Sequence
    (:then_0
      (Variables|Default|SetbSetShowTileIndexes bSetShowTileIndexes)
      (Variables|Default|SetbSetShowCostToEnterTile bSetShowCostToEnterTile)
      (Variables|Default|SetbSetShowMinCostToTarget bSetShowMinCostToTarget)
      (Variables|Default|SetbSetShowCostFromStart bSetShowCostFromStart)
      (Variables|Default|SetbSetShowSortOrder bSetShowSortOrder)
      (Variables|Default|SetbShowTileType bShowTileType))
    (:then_1
      (CallFunction|FUpdateTextonAllTiles))))

(fn FSetShowTileStates
  (params (bShowDiscoveredTiles :type Boolean) (bShowAnalysedTiles :type Boolean))
  (Variables|Default|SetbSetShowDiscoveredTiles bShowDiscoveredTiles)
  (Variables|Default|SetbSetShowAnalysedTiles bShowAnalysedTiles)
  (CallFunction|FUpdateStateonAllTile))