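; BP_GridVisual renders the strategy grid through two BP_GridMeshInst child actors: a flat, ground-offset layer and a tactical view.
; Per-tile updates replace instances in both, with flat tiles only for walkable types.
; Tactical meshes scale in Z from the grid's lowest height, coloured by tile type.
; Tactical mode hides actors tagged "NotTactical", toggles mesh collision and lazily rebuilds tactical tiles when flagged stale.
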(event EventBeginPlay
  (Actor|Tick|SetActorTickEnabled false))

(fn ConstructionScript)

(fn FInitializeGridVisual
  (params (Grid :type BP%20Grid%20Object%20Reference))
  (Variables|Default|SetGrid Grid)
  (Variables|Default|SetGrid%20Mesh%20Inst (.AsBP%20Grid%20Mesh%20Inst (Utilities|Casting|CastToBP_GridMeshInst (Variables|/Script/Engine.ChildActorComponent|GetChildActor (Variables|Default|GetChildActor_GridMeshInst)))))
  (Variables|Default|SetGridMeshInstTactical (.AsBP%20Grid%20Mesh%20Inst (Utilities|Casting|CastToBP_GridMeshInst (Variables|/Script/Engine.ChildActorComponent|GetChildActor (Variables|Default|GetChildActor_GridMesh_Tactical)))))
  (if (.RowFound (Default|FGetCurrentShapeData (Variables|Default|GetGrid)))
    (Utilities|FlowControl|Sequence
      (:then_0
        (Default|FInitializeGridMeshInst (Variables|Default|GetGrid%20Mesh%20Inst) (.flatmesh (.ReturnValue (Default|FGetCurrentShapeData (Variables|Default|GetGrid)))) (.flatmaterial (.ReturnValue (Default|FGetCurrentShapeData (Variables|Default|GetGrid)))) false "QueryOnly"))
      (:then_1
        (Default|FInitializeGridMeshInst (Variables|Default|GetGridMeshInstTactical) (.mesh (.ReturnValue (Default|FGetCurrentShapeData (Variables|Default|GetGrid)))) (.meshmaterial (.ReturnValue (Default|FGetCurrentShapeData (Variables|Default|GetGrid)))) true "QueryOnly"))
      (:then_2
        (Transformation|SetActorLocation "0, 0, 0" false false) ; Center grid in world
        (CallFunction|FSetOffsetfromGround (Variables|Default|GetOffsetFromGround))
        (CallFunction|FSetGridlowestZ 0.0)
        (CallFunction|FSetIsTactical (Variables|Default|GetbIsTactical))))))

(fn FSetOffsetfromGround
  (params (Offset :type Float%20%28double-precision%29))
  (Variables|Default|SetOffsetFromGround Offset)
  (Transformation|SetRelativeLocation (Variables|Default|GetChildActor_GridMeshInst) (Math|Vector|MakeVector 0.0 0.0 (Variables|Default|GetOffsetFromGround)) false false))

(fn FDestroyGridVisual
  (Utilities|FlowControl|Sequence
    (:then_0
      (bind _grid_mesh_inst (Variables|Default|GetGrid%20Mesh%20Inst)
        (:then
          (Default|FClearInstances _grid_mesh_inst))
        (:else)))
    (:then_1
      (bind _gridmeshinsttactical (Variables|Default|GetGridMeshInstTactical)
        (:then
          (Default|FClearInstances _gridmeshinsttactical))
        (:else)))
    (:then_2
      (CallFunction|FSetGridlowestZ 0.0))))

(fn FUpdateTileVisual
  (params (Data :type Struct%20Tile%20Data%20Structure))
  (Utilities|FlowControl|Sequence
    (:then_0
      (bind _grid_mesh_inst (Variables|Default|GetGrid%20Mesh%20Inst)
        (:then
          (Default|FRemoveInstance _grid_mesh_inst (.index Data))
          (if (CallFunction|FIsTileTypeWalkable (.tiletype Data))
            (Default|FAddInstance (Variables|Default|GetGrid%20Mesh%20Inst) (.index Data) (.tiletype Data) (.transform Data) (.states Data))))
        (:else)))
    (:then_1
      (CallFunction|FUpdateTileVisualTactical Data))))

(fn FUpdateTileVisualTactical
  (params (Data :type Struct%20Tile%20Data%20Structure))
  (bind _grid (Variables|Default|GetGrid))
  (bind _location (Math|Transform|BreakTransform (.transform Data)))
  (bind (_location_2 _rotation _scale) (Math|Transform|BreakTransform (.transform Data)))
  (bind _returnvalue (Default|FGetCurrentShapeData _grid))
  (bind _meshsize (Utilities|Struct|BreakStruct_GridShapeData _returnvalue))
  (bind _z (Math|Vector|BreakVector _meshsize))
  (Utilities|FlowControl|Sequence
    (:then_0
      (if (< (.z _location) (Variables|Default|GetGridLowestZ))
        (CallFunction|FSetGridlowestZ (.z _location))))
    (:then_1
      (if (Variables|Default|GetbIsTactical)
        (bind _gridmeshinsttactical (Variables|Default|GetGridMeshInstTactical)
          (:then
            (Default|FRemoveInstance _gridmeshinsttactical (.index Data))
            (if (Utilities|Enum|NotEqual(Enum) (.tiletype Data) "NewEnumerator0")
              (Default|FAddInstance (Variables|Default|GetGridMeshInstTactical) (.index Data) (.tiletype Data) (Math|Transform|MakeTransform _location_2 _rotation (Math|Vector|MakeVector (.x _scale) (.y _scale) (/ (+ (- (.Z (Math|Vector|BreakVector (.Location (Math|Transform|BreakTransform (.transform Data))))) (Variables|Default|GetGridLowestZ)) _z) _z))) (.states Data))))
          (:else))
        (else
          (Variables|Default|SetbNeedToRegenerateTacticalOnEnable true))))))

(fn FSetGridlowestZ
  (params (Z :type Float%20%28double-precision%29))
  (Variables|Default|SetGridLowestZ Z)
  (Variables|Default|SetbNeedToRegenerateTacticalOnEnable true))

(fn FSetIsTactical
  (params (bIsTactical :type Boolean))
  (Variables|Default|SetbIsTactical bIsTactical)
  (Development|SetHiddeninGame (Variables|Default|GetChildActor_GridMesh_Tactical) (not (Variables|Default|GetbIsTactical)) false)
  (bind _outactors (Actor|GetAllActorswithTag "NotTactical"))
  (for _array_element _outactors
    (Rendering|SetActorHiddenInGame _array_element (Variables|Default|GetbIsTactical)))
  (Utilities|FlowControl|Sequence
    (:then_0
      (if (and (Variables|Default|GetbIsTactical) (Variables|Default|GetbNeedToRegenerateTacticalOnEnable))
        (Variables|Default|SetbNeedToRegenerateTacticalOnEnable false)
        (bind _grid (Variables|Default|GetGrid)
          (:then
            (bind _values (Utilities|Map|Values (Variables|/Game/TacticalStrategy/Blueprints/Core/Grid/BP_Grid.BP_Grid_C|GetGridTiles _grid)))
            (for _array_element_2 _values
              (CallFunction|FUpdateTileVisualTactical _array_element_2)))
          (:else))))
    (:then_1
      (bind _gridmeshinsttactical (Variables|Default|GetGridMeshInstTactical)
        (:then
          (Collision|SetCollisionEnabled (Variables|/Game/TacticalStrategy/Blueprints/Core/Grid/Utilities/BP_GridMeshInst.BP_GridMeshInst_C|GetInstancedStaticMesh _gridmeshinsttactical) (select bIsTactical "QueryOnly" "NoCollision")))
        (:else)))))