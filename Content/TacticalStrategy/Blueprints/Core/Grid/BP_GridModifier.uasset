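; BP_GridModifier is a grid marker actor for the tactical grid, representing a tile type such as normal, obstacle, higher movement cost or flying-only.
; Its construction script looks up the mesh for its Shape, then colors it by Type as a filled material.
; It overlaps or blocks two custom trace channels and blocks Pawns only for obstacles.
; When shape data is found, the actor is also hidden in game.
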(fn ConstructionScript
  (bind _staticmesh (Variables|Default|GetStaticMesh))
  (bind _staticmesh_2 (Variables|Default|GetStaticMesh))
  (bind _shape (Variables|Public|GetShape))
  (bind (_rowfound _returnvalue) (CallFunction|FGetShapeData _shape))
  (if _rowfound
    (Components|StaticMesh|SetStaticMesh _staticmesh (.mesh _returnvalue))
    (Rendering|Material|SetVectorParameterValueonMaterials _staticmesh "Color" (Math|Conversions|ToVector(LinearColor) (Utilities|Select :Index (Variables|Public|GetType) :NewEnumerator0 "" :NewEnumerator1 "(R=1.000000,G=1.000000,B=1.000000,A=1.000000)" :NewEnumerator2 "(R=1.000000,G=0.000000,B=0.000000,A=1.000000)" :NewEnumerator3 "(R=1.000000,G=0.445431,B=0.044729,A=1.000000)" :NewEnumerator4 "(R=0.578125,G=0.137305,B=0.000000,A=1.000000)" :NewEnumerator5 "(R=1.000000,G=0.317708,B=0.886214,A=1.000000)")))
    (Rendering|Material|SetScalarParameterValueonMaterials (Variables|Default|GetStaticMesh) "bIsFilled" 1.0)
    (Collision|SetCollisionResponsetoChannel _staticmesh_2 "ECC_GameTraceChannel1" "ECR_Overlap")
    (Collision|SetCollisionResponsetoChannel _staticmesh_2 "ECC_GameTraceChannel4" "ECR_Block")
    (Collision|SetCollisionResponsetoChannel _staticmesh_2 "ECC_Pawn" (select (Utilities|Enum|Equal(Enum) (Variables|Public|GetType) "NewEnumerator2") "ECR_Block" "ECR_Ignore"))
    (Rendering|SetActorHiddenInGame true)))