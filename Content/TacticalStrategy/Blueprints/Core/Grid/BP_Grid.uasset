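; BP_Grid is the tactical strategy grid actor that generates and stores square, hexagon or triangle tiles.
; Construction links child visual and pathfinding actors, then spawns tiles, optionally sphere-tracing for ground height and tile type via BP_GridModifier.
; Tile edits update the tile map, state-to-index lookup and visual, then fire change events.
; Shape-specific math maps indices to world positions and cursor hits back to indices, with hexagons using doubled Y coordinates.
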(fn ConstructionScript
  (Utilities|FlowControl|Sequence
    (:then_0
      (Variables|Default|SetGridVisual (.AsBP%20Grid%20Visual (Utilities|Casting|CastToBP_GridVisual (Variables|/Script/Engine.ChildActorComponent|GetChildActor (Variables|Default|GetChildActor_GridVisual))))))
    (:then_1
      (bind _output_get (Variables|Default|SetGridPathfinding_Reachables (.AsBP%20Grid%20Pathfinding (Utilities|Casting|CastToBP_GridPathfinding (Variables|/Script/Engine.ChildActorComponent|GetChildActor (Variables|Default|GetChildActor_GridPathfinding_Reachables))))))
      (Variables|/Game/TacticalStrategy/Blueprints/Core/Grid/BP_GridPathfinding.BP_GridPathfinding_C|SetGrid _output_get self))
    (:then_2
      (bind _output_get_2 (Variables|Default|SetGridPathfinding (.AsBP%20Grid%20Pathfinding (Utilities|Casting|CastToBP_GridPathfinding (Variables|/Script/Engine.ChildActorComponent|GetChildActor (Variables|Default|GetChildActor_GridPathfinding))))))
      (Variables|/Game/TacticalStrategy/Blueprints/Core/Grid/BP_GridPathfinding.BP_GridPathfinding_C|SetGrid _output_get_2 self))
    (:then_3
      (bind _output_get_3 (Variables|Default|SetGridPathfinding_Ai (.AsBP%20Grid%20Pathfinding (Utilities|Casting|CastToBP_GridPathfinding (Variables|/Script/Engine.ChildActorComponent|GetChildActor (Variables|Default|GetChildActor_GridPathfinding_Ai))))))
      (Variables|/Game/TacticalStrategy/Blueprints/Core/Grid/BP_GridPathfinding.BP_GridPathfinding_C|SetGrid _output_get_3 self))
    (:then_4
      (CallFunction|FSpawnGrid (Transformation|GetActorLocation) (Variables|Public|GetGrid%20Tile%20Size) (Variables|Public|GetGrid%20Tile%20Count) (Variables|Public|GetGrid%20Shape) (Variables|Public|GetbUseEnvironment) (Variables|Public|GetbDisplayTacticalEnvironment)))))

(fn FSpawnGrid
  (params (CenterLocation :type Vector) (TileSize :type Vector) (TileCount :type Int%20Point%20Structure) (Shape :type E_GridShape%20Enum :default "NewEnumerator0") (bUseEnvironment :type Boolean) (bDisplayTacticalEnvironment :type Boolean))
  (Variables|Public|SetGrid%20Center%20Location CenterLocation)
  (Variables|Public|SetGrid%20Tile%20Size TileSize)
  (Variables|Public|SetGrid%20Tile%20Count TileCount)
  (Variables|Public|SetGrid%20Shape Shape)
  (Variables|Public|SetbUseEnvironment bUseEnvironment)
  (Variables|Public|SetbDisplayTacticalEnvironment bDisplayTacticalEnvironment)
  (Utilities|FlowControl|Sequence
    (:then_0
      (CallFunction|FDestroyGrid)
      (if (.RowFound (CallFunction|FGetCurrentShapeData))
        (Variables|/Game/TacticalStrategy/Blueprints/Core/Grid/BP_GridVisual.BP_GridVisual_C|SetbIsTactical (Variables|Default|GetGridVisual) (Variables|Public|GetbDisplayTacticalEnvironment))
        (if (Utilities|Enum|NotEqual(Enum) (Variables|Public|GetGrid%20Shape) "NewEnumerator0")
          (Default|FInitializeGridVisual (Variables|Default|GetGridVisual) self)
          (bind (_center _bottomleft) (CallFunction|FCalculateCenterandBottomLeft))
          (Variables|Public|SetGrid%20Center%20Location _center)
          (Variables|Private|SetGrid%20Bottom%20Left%20Corner%20Location _bottomleft)
          (for _index (range 0 (- (.x (Variables|Public|GetGrid%20Tile%20Count)) 1))
            (LocalVariables|SetX _index)
            (if (Utilities|Enum|NotEqual(Enum) (Variables|Public|GetGrid%20Shape) "NewEnumerator2")
              (for _index_2 (range 0 (- (.y (Variables|Public|GetGrid%20Tile%20Count)) 1))
                (LocalVariables|SetY _index_2)
                (if (.RowFound (CallFunction|FGetCurrentShapeData))
                  (LocalVariables|SetIndex (Utilities|Struct|MakeIntPoint (LocalVariables|GetX) (LocalVariables|GetY)))
                  (LocalVariables|SetTileTransform (Math|Transform|MakeTransform (CallFunction|FGetTileLocationfromGridIndex (LocalVariables|GetIndex)) (CallFunction|FGetTileRotationfromGridIndex (LocalVariables|GetIndex)) (CallFunction|FGetTileScale)))
                  (if bUseEnvironment
                    (bind (_tiletype _outlocation) (CallFunction|FTraceforGround (.location (LocalVariables|GetTileTransform))))
                    (CallFunction|FAddGridTile (Utilities|Struct|MakeStruct_TileData (LocalVariables|GetIndex) _tiletype (Math|Transform|MakeTransform _outlocation (.rotation (LocalVariables|GetTileTransform)) (.scale (LocalVariables|GetTileTransform))) "NewEnumerator0" 0))
                    (else
                      (CallFunction|FAddGridTile (Utilities|Struct|MakeStruct_TileData (LocalVariables|GetIndex) "NewEnumerator1" (LocalVariables|GetTileTransform) "NewEnumerator0" 0))))))
              (else
                (for _index_3 (range (Math|Integer|SelectInt 0 1 (CallFunction|FIsIntEven (LocalVariables|GetX))) (- (* (Math|Float|Round (Math|Conversions|ToFloat(Integer) (.y (Variables|Public|GetGrid%20Tile%20Count)))) 2) 1))
                  (LocalVariables|SetY _index_3)
                  (Utilities|FlowControl|Sequence
                    (:then_0
                      (if (.RowFound (CallFunction|FGetCurrentShapeData))
                        (LocalVariables|SetIndex (Utilities|Struct|MakeIntPoint (LocalVariables|GetX) (LocalVariables|GetY)))
                        (LocalVariables|SetTileTransform (Math|Transform|MakeTransform (CallFunction|FGetTileLocationfromGridIndex (LocalVariables|GetIndex)) (CallFunction|FGetTileRotationfromGridIndex (LocalVariables|GetIndex)) (CallFunction|FGetTileScale)))
                        (if bUseEnvironment
                          (bind (_tiletype_2 _outlocation_2) (CallFunction|FTraceforGround (.location (LocalVariables|GetTileTransform))))
                          (CallFunction|FAddGridTile (Utilities|Struct|MakeStruct_TileData (LocalVariables|GetIndex) _tiletype_2 (Math|Transform|MakeTransform _outlocation_2 (.rotation (LocalVariables|GetTileTransform)) (.scale (LocalVariables|GetTileTransform))) "NewEnumerator0" 0))
                          (else
                            (CallFunction|FAddGridTile (Utilities|Struct|MakeStruct_TileData (LocalVariables|GetIndex) "NewEnumerator1" (LocalVariables|GetTileTransform) "NewEnumerator0" 0))))))
                    (:then_1
                      (Math|Integer|IncrementInt _index_3))))))))))
    (:then_1
      (Default|CallOnGridGenerated))))

(fn FGetCurrentShapeData
  (bind _grid_shape (Variables|Public|GetGrid%20Shape))
  (bind (_rowfound _returnvalue) (CallFunction|FGetShapeData _grid_shape))
  (return _rowfound _returnvalue))

(fn FDestroyGrid
  (Utilities|Map|Clear (Variables|Default|GetGridTiles))
  (Default|FDestroyGridVisual (Variables|Default|GetGridVisual))
  (Default|CallOnGridDestroyed))

(fn FCalculateCenterandBottomLeft
  (bind _grid_tile_count (Variables|Public|GetGrid%20Tile%20Count))
  (Utilities|FlowControl|Sequence
    (:then_0
      (switch Utilities|FlowControl|Switch|SwitchonE_GridShape (Variables|Public|GetGrid%20Shape)
        (:NewEnumerator1
          (LocalVariables|SetC (CallFunction|FSnapVectortoVector (Variables|Public|GetGrid%20Center%20Location) (Variables|Public|GetGrid%20Tile%20Size)))
          (LocalVariables|SetBL (- (LocalVariables|GetC) (* (Variables|Public|GetGrid%20Tile%20Size) (/ (- (Variables|Public|GetGrid%20Tile%20Count) (Math|Vector2D|MakeVector2D (Math|Conversions|ToFloat(Integer) (select (CallFunction|FIsIntEven (.x _grid_tile_count)) 0 1)) (Math|Conversions|ToFloat(Integer) (select (CallFunction|FIsIntEven (.y _grid_tile_count)) 0 1)))) 2.0)))))
        (:NewEnumerator2
          (LocalVariables|SetC (CallFunction|FSnapVectortoVector (Variables|Public|GetGrid%20Center%20Location) (* (Variables|Public|GetGrid%20Tile%20Size) "1.500000,1.000000,1.000000")))
          (LocalVariables|SetBL (- (LocalVariables|GetC) (CallFunction|FSnapVectortoVector (* (Variables|Public|GetGrid%20Tile%20Size) (Math|Conversions|ToVector(Vector2D) (/ (Variables|Public|GetGrid%20Tile%20Count) "(X=3.000000,Y=3.000000)"))) (* (Variables|Public|GetGrid%20Tile%20Size) "1.500000,1.000000,1.000000")))))
        (:NewEnumerator3
          (LocalVariables|SetC (CallFunction|FSnapVectortoVector (Variables|Public|GetGrid%20Center%20Location) (* (Variables|Public|GetGrid%20Tile%20Size) "2.000000,1.000000,1.000000")))
          (LocalVariables|SetBL (- (LocalVariables|GetC) (CallFunction|FSnapVectortoVector (* (Variables|Public|GetGrid%20Tile%20Size) (Math|Conversions|ToVector(Vector2D) (/ (- (Variables|Public|GetGrid%20Tile%20Count) "(X=1.000000,Y=1.000000)") "(X=2.000000,Y=4.000000)"))) (* (Variables|Public|GetGrid%20Tile%20Size) "2.000000,1.000000,1.000000")))))))
    (:then_1
      (return (LocalVariables|GetC) (LocalVariables|GetBL)))))

(fn FGetTileRotationfromGridIndex
  (params (GridIndex :type Int%20Point%20Structure))
  (Utilities|FlowControl|Sequence
    (:then_0
      (if (Utilities|Enum|Equal(Enum) (Variables|Public|GetGrid%20Shape) "NewEnumerator3")
        (LocalVariables|SetReturnRotation (Math|Rotator|MakeRotator 0.0 0.0 (+ (Math|Float|SelectFloat 1.8e+02 0.0 (CallFunction|FIsIntEven (.x GridIndex))) (Math|Float|SelectFloat 1.8e+02 0.0 (CallFunction|FIsIntEven (.y GridIndex))))))
        (else
          (LocalVariables|SetReturnRotation "0, 0, 0"))))
    (:then_1
      (return (LocalVariables|GetReturnRotation)))))

(fn FGetTileLocationfromGridIndex
  (params (GridIndex :type Int%20Point%20Structure))
  (return (+ (Variables|Private|GetGrid%20Bottom%20Left%20Corner%20Location) (* (Math|Conversions|ToVector(Vector2D) (* GridIndex (Utilities|Select :Index (Variables|Public|GetGrid%20Shape) :NewEnumerator0 "(X=0.500000,Y=0.500000)" :NewEnumerator1 "(X=1.000000,Y=1.000000)" :NewEnumerator2 "(X=0.750000,Y=0.500000)" :NewEnumerator3 "(X=1.000000,Y=0.500000)"))) (Variables|Public|GetGrid%20Tile%20Size)))))

(fn FTraceforGround
  (params (Location :type Vector))
  (Utilities|FlowControl|Sequence
    (:then_0
      (LocalVariables|SetRadius (/ (.x (Variables|Public|GetGrid%20Tile%20Size)) (Math|Float|SelectFloat 5.0 3.0 (Utilities|Enum|Equal(Enum) (Variables|Public|GetGrid%20Shape) "NewEnumerator3"))))
      (bind _outhits (Collision|MultiSphereTraceByChannel (+ Location "0.000000,0.000000,1000.000000") (- Location "0.000000,0.000000,1000.000000") (LocalVariables|GetRadius) "TraceTypeQuery3" false 0 "None"))
      (if (> (Utilities|Array|Length _outhits) 0)
        (LocalVariables|SetRetType "NewEnumerator1")
        (LocalVariables|SetbIsHeightFound false)
        (for _array_element _outhits
          (bind _asbp_grid_modifier (Utilities|Casting|CastToBP_GridModifier (.HitActor (Collision|BreakHitResult _array_element)))
            (:then
              (LocalVariables|SetRetType (Variables|/Game/TacticalStrategy/Blueprints/Core/Grid/BP_GridModifier.BP_GridModifier_C|GetType _asbp_grid_modifier))
              (if (Variables|/Game/TacticalStrategy/Blueprints/Core/Grid/BP_GridModifier.BP_GridModifier_C|GetbUseForTileHeight _asbp_grid_modifier)
                (LocalVariables|SetbIsHeightFound true)
                (LocalVariables|SetRetZ (Math|Float|SnapToGrid(Float) (- (.Z (Math|Vector|BreakVector (.Location (Collision|BreakHitResult _array_element)))) (LocalVariables|GetRadius)) (.z (Variables|Public|GetGrid%20Tile%20Size))) :!label _label)))
            (:CastFailed
              (if (not (LocalVariables|GetbIsHeightFound))
                (goto _label)))))
        (LocalVariables|SetResOutLocation (Math|Vector|MakeVector (.x Location) (.y Location) (LocalVariables|GetRetZ)))
        (else
          (LocalVariables|SetRetType "NewEnumerator0")
          (LocalVariables|SetResOutLocation Location))))
    (:then_1
      (return (LocalVariables|GetRetType) (LocalVariables|GetResOutLocation)))))

(fn FAddGridTile
  (params (Data :type Struct%20Tile%20Data%20Structure))
  (Utilities|Map|Add (Variables|Default|GetGridTiles) (.index Data) Data)
  (Default|FUpdateTileVisual (Variables|Default|GetGridVisual) Data)
  (Default|CallOnTileDataUpdated (.index Data)))

(fn FGetCursorLocationonGrid
  (params (PlayerIndex :type Integer) (bTraceForGround :type Boolean) (bTraceEmptySpace :type Boolean))
  (bind _grid_center_location (Variables|Public|GetGrid%20Center%20Location))
  (bind _returnvalue (Game|GetPlayerController PlayerIndex))
  (bind _returnvalue_2 (Game|GetPlayerController PlayerIndex))
  (bind _returnvalue_3 (Class|KismetMathLibrary|MakePlanefromPointandNormal _grid_center_location "0.000000,0.000000,1.000000"))
  (bind (_hitresult _returnvalue_4) (Game|Player|GetHitResultUnderCursorbyChannel _returnvalue_2 "TraceTypeQuery4" true))
  (bind (_worldlocation _worlddirection) (Game|Player|ConvertMouseLocationToWorldSpace _returnvalue))
  (bind (_hitresult_2 _returnvalue_5) (Game|Player|GetHitResultUnderCursorbyChannel _returnvalue "TraceTypeQuery3" false))
  (bind _returnvalue_6 (* _worlddirection 1e+04))
  (bind _returnvalue_7 (+ _worldlocation _returnvalue_6))
  (bind (_t _intersection _returnvalue_8) (Class|KismetMathLibrary|LinePlaneIntersection _worldlocation _returnvalue_7 _returnvalue_3))
  (Utilities|FlowControl|Sequence
    (:then_0
      (if _returnvalue_4
        (return (.Location (Collision|BreakHitResult _hitresult)))))
    (:then_1
      (if bTraceForGround
        (if _returnvalue_5
          (return (.Location (Collision|BreakHitResult _hitresult_2))))))
    (:then_2
      (if bTraceEmptySpace
        (if _returnvalue_8
          (return _intersection))))
    (:then_3
      (return "-999.000000,-999.000000,-999.000000"))))

(fn FGetTileIndexfromWorldLocation
  (params (Location :type Vector))
  (Utilities|FlowControl|Sequence
    (:then_0
      (LocalVariables|SetLocationOnGrid (- Location (Variables|Private|GetGrid%20Bottom%20Left%20Corner%20Location)))
      (if (Utilities|Operators|NotEqual(!=) Location "-999.000000,-999.000000,-999.000000" 0.01)
        (switch Utilities|FlowControl|Switch|SwitchonE_GridShape (Variables|Public|GetGrid%20Shape)
          (:NewEnumerator0
            (LocalVariables|SetRetIndex (Utilities|Struct|MakeIntPoint -999 -999)))
          (:NewEnumerator1
            (LocalVariables|SetSnappedLocationOnGrid (Math|Conversions|ToVector2D(Vector) (CallFunction|FSnapVectortoVector (LocalVariables|GetLocationOnGrid) (Variables|Public|GetGrid%20Tile%20Size))))
            (LocalVariables|SetRetIndex (Class|KismetMathLibrary|ToIntPoint(Vector2D) (/ (LocalVariables|GetSnappedLocationOnGrid) (Math|Conversions|ToVector2D(Vector) (Variables|Public|GetGrid%20Tile%20Size))))))
          (:NewEnumerator2
            (LocalVariables|SetSnappedLocationOnGrid (Math|Conversions|ToVector2D(Vector) (CallFunction|FSnapVectortoVector (* (LocalVariables|GetLocationOnGrid) "1.000000,2.000000,1.000000") (* (Variables|Public|GetGrid%20Tile%20Size) "0.750000,0.250000,1.000000"))))
            (LocalVariables|SetTempIndex (/ (LocalVariables|GetSnappedLocationOnGrid) (* (Math|Conversions|ToVector2D(Vector) (Variables|Public|GetGrid%20Tile%20Size)) "(X=0.750000,Y=1.000000)")))
            (if (CallFunction|FIsFloatEven (.x (LocalVariables|GetTempIndex)))
              (LocalVariables|SetRetIndex (Utilities|Struct|MakeIntPoint (Math|Float|Truncate (.x (LocalVariables|GetTempIndex))) (* (Math|Float|Round (/ (.y (LocalVariables|GetTempIndex)) 2.0)) 2)))
              (else
                (LocalVariables|SetRetIndex (Utilities|Struct|MakeIntPoint (Math|Float|Truncate (.x (LocalVariables|GetTempIndex))) (+ (* (Math|Float|Floor (/ (.y (LocalVariables|GetTempIndex)) 2.0)) 2) 1))))))
          (:NewEnumerator3
            (LocalVariables|SetSnappedLocationOnGrid (Math|Conversions|ToVector2D(Vector) (CallFunction|FSnapVectortoVector (LocalVariables|GetLocationOnGrid) (/ (Variables|Public|GetGrid%20Tile%20Size) "1.000000,2.000000,1.000000"))))
            (LocalVariables|SetRetIndex (Class|KismetMathLibrary|ToIntPoint(Vector2D) (* (/ (LocalVariables|GetSnappedLocationOnGrid) (Math|Conversions|ToVector2D(Vector) (Variables|Public|GetGrid%20Tile%20Size))) "(X=1.000000,Y=2.000000)")))))
        (else
          (LocalVariables|SetRetIndex (Utilities|Struct|MakeIntPoint -999 -999)))))
    (:then_1
      (return (LocalVariables|GetRetIndex)))))

(fn FGetTileIndexUnderCursor
  (params (PlayerIndex :type Integer) (bTraceForGround :type Boolean) (bTraceEmptySpace :type Boolean))
  (bind _location (CallFunction|FGetCursorLocationonGrid PlayerIndex bTraceForGround bTraceEmptySpace))
  (bind _index (CallFunction|FGetTileIndexfromWorldLocation _location))
  (return _index))

(fn FAddStatetoTile
  (params (Index :type Int%20Point%20Structure) (State :type E_TileState%20Enum :default "NewEnumerator0"))
  (bind _gridtiles (Variables|Default|GetGridTiles))
  (bind (_value _returnvalue) (Utilities|Map|Find _gridtiles Index))
  (if _returnvalue
    (bind _output_get (LocalVariables|SetData _value))
    (bind _returnvalue_2 (Utilities|Array|AddUnique (.states _output_get) State))
    (if (>= _returnvalue_2 0)
      (Utilities|Map|Add (Variables|Default|GetGridTiles) (.index (LocalVariables|GetData)) (LocalVariables|GetData))
      (bind _indexes (CallFunction|FGetAllTileswithState State))
      (Utilities|Array|Add _indexes Index)
      (Utilities|Map|Add (Variables|Default|GetTileStateToIndexes) State (Utilities|Struct|MakeStruct_IntPointArray _indexes))
      (Default|FUpdateTileVisual (Variables|Default|GetGridVisual) (LocalVariables|GetData))
      (Default|CallOnTileStateUpdated Index))))

(fn FRemoveStatefromTile
  (params (Index :type Int%20Point%20Structure) (State :type E_TileState%20Enum :default "NewEnumerator0"))
  (bind _gridtiles (Variables|Default|GetGridTiles))
  (bind (_value _returnvalue) (Utilities|Map|Find _gridtiles Index))
  (if _returnvalue
    (bind _output_get (LocalVariables|SetData _value))
    (bind _returnvalue_2 (Utilities|Array|RemoveItem (.states _output_get) State))
    (if _returnvalue_2
      (Utilities|Map|Add (Variables|Default|GetGridTiles) (.index (LocalVariables|GetData)) (LocalVariables|GetData))
      (bind _indexes (CallFunction|FGetAllTileswithState State))
      (Utilities|Array|RemoveItem _indexes Index)
      (Utilities|Map|Add (Variables|Default|GetTileStateToIndexes) State (Utilities|Struct|MakeStruct_IntPointArray _indexes))
      (Default|FUpdateTileVisual (Variables|Default|GetGridVisual) (LocalVariables|GetData))
      (Default|CallOnTileStateUpdated Index))))

(fn FIsIndexValid
  (params (Index :type Int%20Point%20Structure))
  (return (Utilities|Map|Contains (Variables|Default|GetGridTiles) Index)))

(fn FGetTileScale
  (return (/ (Variables|Public|GetGrid%20Tile%20Size) (.MeshSize (Utilities|Struct|BreakStruct_GridShapeData (.ReturnValue (CallFunction|FGetCurrentShapeData)))))))

(fn FRemoveGridTile
  (params (Index :type Int%20Point%20Structure))
  (bind _returnvalue (Utilities|Map|Remove (Variables|Default|GetGridTiles) Index))
  (if _returnvalue
    (Default|FUpdateTileVisual (Variables|Default|GetGridVisual) (Utilities|Struct|MakeStruct_TileData Index "NewEnumerator0" "0.000000,0.000000,0.000000|0.000000,0.000000,0.000000|1.000000,1.000000,1.000000" "NewEnumerator0" 0))
    (Default|CallOnTileDataUpdated Index)))

(fn FGetAllTileswithState
  (params (State :type E_TileState%20Enum :default "NewEnumerator0"))
  (return (.intpointarray (.Value (Utilities|Map|Find (Variables|Default|GetTileStateToIndexes) State)))))

(fn FClearStatefromTiles
  (params (State :type E_TileState%20Enum :default "NewEnumerator0"))
  (bind _indexes (CallFunction|FGetAllTileswithState State))
  (for _array_element _indexes
    (CallFunction|FRemoveStatefromTile _array_element State)))

(fn FIsTileWalkable
  (params (Index :type Int%20Point%20Structure))
  (return (CallFunction|FIsTileTypeWalkable (.TileType (Utilities|Struct|BreakStruct_TileData (.Value (Utilities|Map|Find (Variables|Default|GetGridTiles) Index)))))))