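; BP_SpellAnimation is a short-lived actor that plays a spell's visual on a tactical grid and reports when tiles are hit.
; On BeginPlay it spawns one BP_AnimatedShape per attacked tile, using the grid's shape mesh, animating from a tiny copy at the origin tile to the target's transform.
; Red brightness and play rate are randomized per shape.
; Each finished shape broadcasts a tile hit; the last triggers completion and self-destruction.
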(event Custom|ePlaySpellAnimation
  (bind _grid (Variables|Default|GetGrid))
  (bind _originindex (Variables|Default|GetOriginIndex))
  (bind _returnvalue (Default|FGetCurrentShapeData _grid))
  (bind _transform (CallFunction|FGetTileTransform _originindex))
  (bind (_meshsize _mesh _meshmaterial) (Utilities|Struct|BreakStruct_GridShapeData _returnvalue))
  (for _array_element (Variables|Default|GetAttackIndexes)
    (bind _returnvalue_2 (Game|SpawnActorfromClass "/Game/TacticalStrategy/Blueprints/Core/Combat/Spells/SpellAnimations/Components/BP_AnimatedShape.BP_AnimatedShape_C" (Math|Transform|MakeTransform "0, 0, 0" "0, 0, 0" "1.000000,1.000000,1.000000") "AlwaysSpawn" "MultiplyWithRoot" 0 _mesh _meshmaterial (* "(R=1.000000,G=0.000000,B=0.000000,A=1.000000)" (Math|Random|RandomFloatinRange 0.5 1.5)) (Math|Transform|MakeTransform (.location _transform) (.rotation _transform) "0.010000,0.010000,0.010000") (CallFunction|FGetTileTransform _array_element) (Math|Random|RandomFloatinRange 0.5 1.5) _array_element 0))
    (EventDispatchers|AssignOnShapeAnimationCompleted _returnvalue_2 (delegate Custom|OnShapeAnimationCompleted_Event))))

(event Custom|OnShapeAnimationCompleted_Event
  (params (AnimatedShape :type BP%20Animated%20Shape%20Object%20Reference))
  (bind _index (Variables|/Game/TacticalStrategy/Blueprints/Core/Combat/Spells/SpellAnimations/Components/BP_AnimatedShape.BP_AnimatedShape_C|GetIndex AnimatedShape))
  (bind _attackindexes (Variables|Default|GetAttackIndexes))
  (Default|CallOnSpellAnimationHitTile self _index)
  (Utilities|Array|RemoveItem _attackindexes _index)
  (if (== (Utilities|Array|Length _attackindexes) 0)
    (CallFunction|ECompleteSpellAnimation)))

(event Custom|eCompleteSpellAnimation
  (Default|CallOnSpellAnimationCompleted self)
  (Actor|DestroyActor))

(event EventBeginPlay
  (CallFunction|EPlaySpellAnimation))

(fn ConstructionScript)

(fn FGetTileTransform
  (params (Index :type Int%20Point%20Structure%20%28by%20ref%29))
  (return (.Transform (Utilities|Struct|BreakStruct_TileData (.Value (Utilities|Map|Find (Variables|/Game/TacticalStrategy/Blueprints/Core/Grid/BP_Grid.BP_Grid_C|GetGridTiles (Variables|Default|GetGrid)) Index))))))