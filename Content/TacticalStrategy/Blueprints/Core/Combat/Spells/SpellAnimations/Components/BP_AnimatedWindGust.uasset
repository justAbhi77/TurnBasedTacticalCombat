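; Animated wind gust spell effect actor that moves a translucent green shape between two transforms.
; Construction gives both material slots dynamic instances with randomized brightness.
; On BeginPlay, a timeline at a configurable play rate drives the transform lerp and opacity.
; It signals shape animation completion once playback passes a threshold before the timeline ends, then destroys itself shortly after it finishes.
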(event EventBeginPlay
  (Components|Timeline|SetPlayRate (Variables|Default|GetTimeline_PlayAnimation) (Variables|Default|GetPlayRate))
  (bind (_direction _transformalpha _opacity) (Timeline|Timeline_PlayAnimation PlayFromStart)
    (:Update
      (Transformation|SetActorTransform (Math|Transform|Lerp(Transform) (Variables|Default|GetOriginTransform) (Variables|Default|GetTargetTransform) _transformalpha))
      (Rendering|Material|SetScalarParameterValueonMaterials (Variables|Default|GetAnimatedShape) "Opacity" _opacity)
      (if (> (Components|Timeline|GetPlaybackPosition (Variables|Default|GetTimeline_PlayAnimation)) 0.35)
        (Utilities|FlowControl|DoOnce false
          (:Completed
            (Default|CallOnShapeAnimationCompleted self)))))
    (:Finished
      (Utilities|FlowControl|Delay 0.5)
      (Actor|DestroyActor))))

(fn ConstructionScript
  (Utilities|FlowControl|Sequence
    (:then_0
      (bind _returnvalue (Rendering|Material|CreateDynamicMaterialInstance (Variables|Default|GetAnimatedShape) 0 "/Game/TacticalStrategy/Demo/Art/Materials/Colors/MI_Color_Translucent_Two_Sided.MI_Color_Translucent_Two_Sided" "None" :!class /Script/Engine.PrimitiveComponent))
      (Rendering|Material|SetVectorParameterValue _returnvalue "BaseColor" (* "(R=0.105016,G=0.705000,B=0.255012,A=1.000000)" (Math|Random|RandomFloatinRange 0.8 1.5)) :!class /Script/Engine.MaterialInstanceDynamic))
    (:then_1
      (bind _returnvalue_2 (Rendering|Material|CreateDynamicMaterialInstance (Variables|Default|GetAnimatedShape) 1 "/Game/TacticalStrategy/Demo/Art/Materials/Colors/MI_Color_Translucent_Two_Sided.MI_Color_Translucent_Two_Sided" "None" :!class /Script/Engine.PrimitiveComponent))
      (Rendering|Material|SetVectorParameterValue _returnvalue_2 "BaseColor" (* "(R=0.200000,G=0.750000,B=0.400000,A=1.000000)" (Math|Random|RandomFloatinRange 0.8 1.5)) :!class /Script/Engine.MaterialInstanceDynamic))))