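; Spell animation for Wind Gust that blows animated gusts outward from the target tile to every other affected tile.
; After a short delay it reports a hit on the target tile, then spawns a growing BP_AnimatedWindGust toward each remaining attack index at a random play rate.
; Each gust's completion reports a hit on its tile, and the spell completes once no attack indexes remain.
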(event Custom|OnShapeAnimationCompleted_Event_0
  (params (AnimatedShape :type BP%20Animated%20Wind%20Gust%20Object%20Reference))
  (bind _index (Variables|/Game/TacticalStrategy/Blueprints/Core/Combat/Spells/SpellAnimations/Components/BP_AnimatedWindGust.BP_AnimatedWindGust_C|GetIndex AnimatedShape))
  (bind _attackindexes (Variables|Default|GetAttackIndexes))
  (Default|CallOnSpellAnimationHitTile self _index)
  (Utilities|Array|RemoveItem _attackindexes _index)
  (if (== (Utilities|Array|Length _attackindexes) 0)
    (CallFunction|ECompleteSpellAnimation)))

(event EventEPlaySpellAnimation
  (bind _targetindex (Variables|Default|GetTargetIndex))
  (bind _transform (CallFunction|FGetTileTransform _targetindex))
  (Utilities|FlowControl|Delay 0.1)
  (Utilities|FlowControl|Sequence
    (:then_0
      (Default|CallOnSpellAnimationHitTile self (Variables|Default|GetTargetIndex))
      (Utilities|Array|RemoveItem (Variables|Default|GetAttackIndexes) (Variables|Default|GetTargetIndex)))
    (:then_1
      (for _array_element (Variables|Default|GetAttackIndexes)
        (bind _returnvalue (Game|SpawnActorfromClass "/Game/TacticalStrategy/Blueprints/Core/Combat/Spells/SpellAnimations/Components/BP_AnimatedWindGust.BP_AnimatedWindGust_C" (Math|Transform|MakeTransform "0, 0, 0" "0, 0, 0" "1.000000,1.000000,1.000000") "Undefined" "MultiplyWithRoot" 0 (Math|Transform|MakeTransform (.location _transform) (Math|Rotator|FindLookatRotation (.location _transform) (.location (CallFunction|FGetTileTransform _array_element))) "0.500000,0.500000,0.500000") (Math|Transform|MakeTransform (.location (CallFunction|FGetTileTransform _array_element)) (Math|Rotator|FindLookatRotation (.location _transform) (.location (CallFunction|FGetTileTransform _array_element))) "1.200000,1.200000,1.200000") (Math|Random|RandomFloatinRange 0.8 1.5) _array_element 0))
        (EventDispatchers|AssignOnShapeAnimationCompleted _returnvalue (delegate Custom|OnShapeAnimationCompleted_Event_0))))))

(fn ConstructionScript
  (|CallParentFunction))