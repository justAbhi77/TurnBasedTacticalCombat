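; Spell animation actor for Run Chicken Run in a tactical strategy game, showing the spell's icon over the target tile.
; It moves to the tile's transform and sets the icon on an image widget component, then a Timeline animates that widget's height, size and opacity.
; Shortly into the Timeline, a DoOnce raises the tile-hit callback a single time, and the spell animation completes when the Timeline finishes.
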(event EventEPlaySpellAnimation
  (Transformation|SetActorLocation (.location (CallFunction|FGetTileTransform (Variables|Default|GetTargetIndex))) false false)
  (bind _output_get (Variables|Default|SetWBPImage (.AsWBP%20Image (Utilities|Casting|CastToWBP_Image (UserInterface|GetUserWidgetObject (Variables|Default|GetWidget))))))
  (Appearance|SetBrushfromTexture (Variables|/Game/TacticalStrategy/Blueprints/Core/Combat/Spells/SpellAnimations/Components/WBP_Image.WBP_Image_C|GetImage_Comp _output_get) "/Game/TacticalStrategy/Blueprints/Core/Combat/Spells/SpellAnimations/Assests/TX_Icon_RunChickenRun_NoBackground.TX_Icon_RunChickenRun_NoBackground" false)
  (bind (_direction _locationz _drawsize _opacity) (Timeline|Timeline PlayFromStart)
    (:Update
      (Transformation|SetRelativeLocation (Variables|Default|GetWidget) (Math|Vector|MakeVector 0.0 0.0 _locationz) false false)
      (Class|WidgetComponent|SetDrawSize (Variables|Default|GetWidget) (Math|Vector2D|MakeVector2D _drawsize _drawsize))
      (Widget|SetRenderOpacity (Variables|Default|GetWBPImage) _opacity)
      (if (> (Components|Timeline|GetPlaybackPosition (Variables|Default|GetTimeline)) 0.2)
        (Utilities|FlowControl|DoOnce false
          (:Completed
            (Default|CallOnSpellAnimationHitTile self (Variables|Default|GetTargetIndex))))))
    (:Finished
      (CallFunction|ECompleteSpellAnimation))))

(fn ConstructionScript
  (|CallParentFunction))