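; Player action that moves the selected unit across the tactical grid to a target tile.
; It requests a path from the grid's pathfinding using the unit's diagonal rule, valid tile types and current movement points.
; On completion it marks the path tiles, hands movement to the combat system and calls the unit's MP reset.
; Path highlights clear when walking finishes or the action re-executes, including with an off-grid index on EndPlay.
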(event EventEndPlay
  (params (EndPlayReason :type EEndPlayReason%20Enum :default "Destroyed"))
  (CallFunction|FExecuteAction (Utilities|Struct|MakeIntPoint -999 -999)))

(fn ConstructionScript
  (|CallParentFunction))

(fn FExecuteAction
  (params (index :type Int%20Point%20Structure))
  (bind _playeractions (Variables|Default|GetPlayerActions))
  (|CallParentFunction index)
  (Variables|Default|GetPlayerActions
    (:then
      (Default|FClearStatefromTiles (Variables|/Game/TacticalStrategy/Blueprints/Core/Player/BP_PlayerActions.BP_PlayerActions_C|GetGrid (Variables|Default|GetPlayerActions)) "NewEnumerator5")
      (bind _output_get (Variables|Default|SetCurrentUnit (Variables|/Game/TacticalStrategy/Blueprints/Core/Player/BP_PlayerActions.BP_PlayerActions_C|GetSelectedUnit (Variables|Default|GetPlayerActions))))
      (Utilities|IsValid _output_get
        (:Is%20Valid
          (EventDispatchers|BindEventtoOnUnitFinishedWalking (Variables|Default|GetCurrentUnit) (EventDispatchers|CreateEvent :!event FonUnitFinishedWalking))
          (EventDispatchers|BindEventtoOnPathfindingCompleted (Variables|/Game/TacticalStrategy/Blueprints/Core/Grid/BP_Grid.BP_Grid_C|GetGridPathfinding (Variables|/Game/TacticalStrategy/Blueprints/Core/Player/BP_PlayerActions.BP_PlayerActions_C|GetGrid (Variables|Default|GetPlayerActions))) (EventDispatchers|CreateEvent :!event FonPathFindingCompleted))
          (Default|FFindPath (Variables|/Game/TacticalStrategy/Blueprints/Core/Grid/BP_Grid.BP_Grid_C|GetGridPathfinding (Variables|/Game/TacticalStrategy/Blueprints/Core/Player/BP_PlayerActions.BP_PlayerActions_C|GetGrid _playeractions)) (Variables|/Game/TacticalStrategy/Blueprints/Core/Player/BP_PlayerActions.BP_PlayerActions_C|GetSelectedTile _playeractions) index (.bCanMoveDiagonally (Utilities|Struct|BreakStruct_UnitData_Stats (.Stats (Utilities|Struct|BreakStruct_UnitData (Variables|/Game/TacticalStrategy/Blueprints/Core/Units/BP_Unit.BP_Unit_C|GetUnitData (Variables|Default|GetCurrentUnit)))))) (.ValidTileTypes (Utilities|Struct|BreakStruct_UnitData_Stats (.Stats (Utilities|Struct|BreakStruct_UnitData (Variables|/Game/TacticalStrategy/Blueprints/Core/Units/BP_Unit.BP_Unit_C|GetUnitData (Variables|Default|GetCurrentUnit)))))) 0.1 15.0 false (.MP_Current (Utilities|Struct|BreakStruct_UnitData_Stats (.Stats (Utilities|Struct|BreakStruct_UnitData (Variables|/Game/TacticalStrategy/Blueprints/Core/Units/BP_Unit.BP_Unit_C|GetUnitData (Variables|Default|GetCurrentUnit))))))))))
    (:else)))

(fn FonPathFindingCompleted
  (params (Path :type Array%20of%20Int%20Point%20Structures))
  (Utilities|IsValid (Variables|Default|GetCurrentUnit)
    (:Is%20Valid
      (if (== (Variables|Default|GetCurrentUnit) (Variables|/Game/TacticalStrategy/Blueprints/Core/Player/BP_PlayerActions.BP_PlayerActions_C|GetSelectedUnit (Variables|Default|GetPlayerActions)))
        (for _array_element Path
          (Default|FAddStatetoTile (Variables|/Game/TacticalStrategy/Blueprints/Core/Player/BP_PlayerActions.BP_PlayerActions_C|GetGrid (Variables|Default|GetPlayerActions)) _array_element "NewEnumerator5"))
        (Variables|/Game/TacticalStrategy/Blueprints/Core/Units/BP_Unit.BP_Unit_C|SetMoveDurationPerTile (Variables|Default|GetCurrentUnit) (Variables|Default|GetMoveDuration))
        (Default|FMoveUnit (Variables|/Game/TacticalStrategy/Blueprints/Core/Player/BP_PlayerActions.BP_PlayerActions_C|GetCombatSystem (Variables|Default|GetPlayerActions)) (Variables|Default|GetCurrentUnit) Path)
        (Default|FResetMp (Variables|Default|GetCurrentUnit))))))

(fn FonUnitFinishedWalking
  (params (Unit :type BP%20Unit%20Object%20Reference))
  (if (== Unit (Variables|Default|GetCurrentUnit))
    (Default|FClearStatefromTiles (Variables|/Game/TacticalStrategy/Blueprints/Core/Player/BP_PlayerActions.BP_PlayerActions_C|GetGrid (Variables|Default|GetPlayerActions)) "NewEnumerator5")))