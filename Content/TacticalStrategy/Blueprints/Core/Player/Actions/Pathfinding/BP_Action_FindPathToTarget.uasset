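; Player action that finds a path on the tactical grid from the selected tile to a target tile and highlights it.
; Executing clears the previous path state, then starts GridPathfinding with configurable diagonals, flying-only tiles, length limit and time slicing.
; The completion callback marks each returned tile with the path state.
; Selection changes and EndPlay rerun the action with an off-grid sentinel index to reset the highlight.
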(event Custom|OnSelectedTileChanged
  (params (Index :type Int%20Point%20Structure))
  (CallFunction|FExecuteAction (Utilities|Struct|MakeIntPoint -999 -999)))

(event EventEndPlay
  (params (EndPlayReason :type EEndPlayReason%20Enum :default "Destroyed"))
  (CallFunction|FExecuteAction (Utilities|Struct|MakeIntPoint -999 -999)))

(event EventBeginPlay
  (EventDispatchers|BindEventtoOnSelectedTileChanged (Variables|Default|GetPlayerActions) (delegate Custom|OnSelectedTileChanged)))

(fn ConstructionScript
  (|CallParentFunction))

(fn FExecuteAction
  (params (index :type Int%20Point%20Structure))
  (bind _playeractions (Variables|Default|GetPlayerActions))
  (|CallParentFunction index)
  (Variables|Default|GetPlayerActions
    (:then
      (Default|FClearStatefromTiles (Variables|/Game/TacticalStrategy/Blueprints/Core/Player/BP_PlayerActions.BP_PlayerActions_C|GetGrid (Variables|Default|GetPlayerActions)) "NewEnumerator5")
      (EventDispatchers|BindEventtoOnPathfindingCompleted (Variables|/Game/TacticalStrategy/Blueprints/Core/Grid/BP_Grid.BP_Grid_C|GetGridPathfinding (Variables|/Game/TacticalStrategy/Blueprints/Core/Player/BP_PlayerActions.BP_PlayerActions_C|GetGrid (Variables|Default|GetPlayerActions))) (EventDispatchers|CreateEvent :!event FonPathFindingCompleted))
      (Default|FFindPath (Variables|/Game/TacticalStrategy/Blueprints/Core/Grid/BP_Grid.BP_Grid_C|GetGridPathfinding (Variables|/Game/TacticalStrategy/Blueprints/Core/Player/BP_PlayerActions.BP_PlayerActions_C|GetGrid _playeractions)) (Variables|/Game/TacticalStrategy/Blueprints/Core/Player/BP_PlayerActions.BP_PlayerActions_C|GetSelectedTile _playeractions) index (Variables|Default|GetbIncludeDiagonals) (select (Variables|Default|GetbIncludeFlyingOnly) (Utilities|Array|MakeArray "NewEnumerator1" "NewEnumerator3" "NewEnumerator4" "NewEnumerator5") (Utilities|Array|MakeArray "NewEnumerator1" "NewEnumerator3" "NewEnumerator4")) (Variables|Default|GetDelayBetweenIterations) (Variables|Default|GetMaxMsPerFrame) false (Variables|Default|GetMaxPathLength)))
    (:else)))

(fn FonPathFindingCompleted
  (params (Path :type Array%20of%20Int%20Point%20Structures))
  (for _array_element Path
    (Default|FAddStatetoTile (Variables|/Game/TacticalStrategy/Blueprints/Core/Player/BP_PlayerActions.BP_PlayerActions_C|GetGrid (Variables|Default|GetPlayerActions)) _array_element "NewEnumerator5")))