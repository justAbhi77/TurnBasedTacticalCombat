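; Grid action for the player's actions system that raises or lowers a single tile in the tactical grid.
; When executed on a valid index, it looks up the tile's data and shifts its Z location by one tile height, with the Increase flag choosing up or down.
; It writes the change back through the grid's add-tile function, keeping type, rotation, scale, states and unit unchanged.
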(fn ConstructionScript
  (|CallParentFunction))

(fn FExecuteAction
  (params (index :type Int%20Point%20Structure))
  (|CallParentFunction index)
  (bind _playeractions (Variables|Default|GetPlayerActions)
    (:then
      (if (Default|FIsIndexValid (Variables|/Game/TacticalStrategy/Blueprints/Core/Player/BP_PlayerActions.BP_PlayerActions_C|GetGrid _playeractions) index)
        (LocalVariables|SetData (.Value (Utilities|Map|Find (Variables|/Game/TacticalStrategy/Blueprints/Core/Grid/BP_Grid.BP_Grid_C|GetGridTiles (Variables|/Game/TacticalStrategy/Blueprints/Core/Player/BP_PlayerActions.BP_PlayerActions_C|GetGrid (Variables|Default|GetPlayerActions))) index)))
        (Default|FAddGridTile (Variables|/Game/TacticalStrategy/Blueprints/Core/Player/BP_PlayerActions.BP_PlayerActions_C|GetGrid (Variables|Default|GetPlayerActions)) (Utilities|Struct|MakeStruct_TileData (.index (LocalVariables|GetData)) (.tiletype (LocalVariables|GetData)) (Math|Transform|MakeTransform (+ (.location (.transform (LocalVariables|GetData))) (Math|Vector|MakeVector 0.0 0.0 (* (.z (Variables|/Game/TacticalStrategy/Blueprints/Core/Grid/BP_Grid.BP_Grid_C|GetGrid%20Tile%20Size (Variables|/Game/TacticalStrategy/Blueprints/Core/Player/BP_PlayerActions.BP_PlayerActions_C|GetGrid (Variables|Default|GetPlayerActions)))) (Math|Float|SelectFloat 1.0 -1.0 (Variables|Default|GetbIncrease))))) (.rotation (.transform (LocalVariables|GetData))) (.scale (.transform (LocalVariables|GetData)))) (.states (LocalVariables|GetData)) (.unitontile (LocalVariables|GetData))))))
    (:else)))