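; Player action for combat setup that selects a tile and unit and previews a spell's range pattern on the grid.
; On execute, it clears the range tile state and re-marks tiles from the CombatSystem's cast range around the selected tile.
; It then refreshes the area-of-effect preview, also rerun on hover.
; That preview marks the AoE pattern, or just the hovered tile, only when hovering inside the cast range.
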(event EventBeginPlay)

(fn ConstructionScript
  (|CallParentFunction))

(fn FExecuteAction
  (params (index :type Int%20Point%20Structure))
  (|CallParentFunction index)
  (CallFunction|FShowSpellRangePattern))

(fn FShowSpellRangePattern
  (bind _playeractions (Variables|Default|GetPlayerActions))
  (bind _playeractions_2 (Variables|Default|GetPlayerActions))
  (Utilities|FlowControl|Sequence
    (:then_0
      (Default|FClearStatefromTiles (Variables|/Game/TacticalStrategy/Blueprints/Core/Player/BP_PlayerActions.BP_PlayerActions_C|GetGrid (Variables|Default|GetPlayerActions)) "NewEnumerator9")
      (if (Default|FIsIndexValid (Variables|/Game/TacticalStrategy/Blueprints/Core/Player/BP_PlayerActions.BP_PlayerActions_C|GetGrid _playeractions_2) (Variables|/Game/TacticalStrategy/Blueprints/Core/Player/BP_PlayerActions.BP_PlayerActions_C|GetSelectedTile _playeractions_2))
        (bind _rangesindexes (Default|FGetSpellRange (Variables|/Game/TacticalStrategy/Blueprints/Core/Player/BP_PlayerActions.BP_PlayerActions_C|GetCombatSystem _playeractions) (Variables|/Game/TacticalStrategy/Blueprints/Core/Player/BP_PlayerActions.BP_PlayerActions_C|GetSelectedTile _playeractions) (Variables|Default|GetCast)))
        (for _array_element _rangesindexes
          (Default|FAddStatetoTile (Variables|/Game/TacticalStrategy/Blueprints/Core/Player/BP_PlayerActions.BP_PlayerActions_C|GetGrid (Variables|Default|GetPlayerActions)) _array_element "NewEnumerator9"))))
    (:then_1
      (CallFunction|FShowSpellRangePatternAoe))))

(fn FShowSpellRangePatternAoe
  (bind _playeractions (Variables|Default|GetPlayerActions))
  (Default|FClearStatefromTiles (Variables|/Game/TacticalStrategy/Blueprints/Core/Player/BP_PlayerActions.BP_PlayerActions_C|GetGrid (Variables|Default|GetPlayerActions)) "NewEnumerator10")
  (if (Utilities|Array|ContainsItem (Utilities|Struct|BreakStruct_IntPointArray (.Value (Utilities|Map|Find (Variables|/Game/TacticalStrategy/Blueprints/Core/Grid/BP_Grid.BP_Grid_C|GetTileStateToIndexes (Variables|/Game/TacticalStrategy/Blueprints/Core/Player/BP_PlayerActions.BP_PlayerActions_C|GetGrid (Variables|Default|GetPlayerActions))) "NewEnumerator9"))) (Variables|/Game/TacticalStrategy/Blueprints/Core/Player/BP_PlayerActions.BP_PlayerActions_C|GetHoveredTile (Variables|Default|GetPlayerActions)))
    (if (Utilities|Enum|NotEqual(Enum) (.RangePattern (Utilities|Struct|BreakStruct_SpellData_Cast (Variables|Default|GetCast_Aoe))) "NewEnumerator0")
      (bind _rangesindexes (Default|FGetSpellRange (Variables|/Game/TacticalStrategy/Blueprints/Core/Player/BP_PlayerActions.BP_PlayerActions_C|GetCombatSystem _playeractions) (Variables|/Game/TacticalStrategy/Blueprints/Core/Player/BP_PlayerActions.BP_PlayerActions_C|GetHoveredTile _playeractions) (Variables|Default|GetCast_Aoe)))
      (for _array_element _rangesindexes
        (Default|FAddStatetoTile (Variables|/Game/TacticalStrategy/Blueprints/Core/Player/BP_PlayerActions.BP_PlayerActions_C|GetGrid (Variables|Default|GetPlayerActions)) _array_element "NewEnumerator10"))
      (else
        (Default|FAddStatetoTile (Variables|/Game/TacticalStrategy/Blueprints/Core/Player/BP_PlayerActions.BP_PlayerActions_C|GetGrid (Variables|Default|GetPlayerActions)) (Variables|/Game/TacticalStrategy/Blueprints/Core/Player/BP_PlayerActions.BP_PlayerActions_C|GetHoveredTile (Variables|Default|GetPlayerActions)) "NewEnumerator10")))))

(fn FExecuteHoveredAction
  (params (index :type Int%20Point%20Structure))
  (|CallParentFunction index)
  (CallFunction|FShowSpellRangePatternAoe))