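; Combat move action for the tactical grid player, previewing where a unit can move and sending it along the chosen path.
; Hovering shows the hovered unit's reachable tiles, or the selected unit's plus a path to the hovered tile, limited by its movement points.
; Two grid pathfinders report results through completion events that set tile states; executing hands the path to the combat system.
; Reachables clear while the unit walks and refresh when it stops.
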(event EventBeginPlay
  (bind _playeractions (Variables|Default|GetPlayerActions))
  (bind _playeractions_2 (Variables|Default|GetPlayerActions))
  (bind _selectedunit (Variables|/Game/TacticalStrategy/Blueprints/Core/Player/BP_PlayerActions.BP_PlayerActions_C|GetSelectedUnit _playeractions))
  (bind _grid (Variables|/Game/TacticalStrategy/Blueprints/Core/Player/BP_PlayerActions.BP_PlayerActions_C|GetGrid _playeractions_2))
  (|CallParentFunction)
  (EventDispatchers|BindEventtoOnPathfindingCompleted (Variables|/Game/TacticalStrategy/Blueprints/Core/Grid/BP_Grid.BP_Grid_C|GetGridPathfinding_Reachables _grid) (EventDispatchers|CreateEvent :!event FonPathfindingCompletedReachables))
  (EventDispatchers|BindEventtoOnPathfindingCompleted (Variables|/Game/TacticalStrategy/Blueprints/Core/Grid/BP_Grid.BP_Grid_C|GetGridPathfinding _grid) (EventDispatchers|CreateEvent :!event FonPathfindingCompletedPath))
  (EventDispatchers|BindEventtoOnUnitStartedWalking _selectedunit (EventDispatchers|CreateEvent :!event FonUnitStartedWalking))
  (EventDispatchers|BindEventtoOnUnitFinishedWalking _selectedunit (EventDispatchers|CreateEvent :!event FonUnitFinishedWalking))
  (CallFunction|FGenerateReachables (Variables|/Game/TacticalStrategy/Blueprints/Core/Player/BP_PlayerActions.BP_PlayerActions_C|GetSelectedUnit (Variables|Default|GetPlayerActions))))

(event EventEndPlay
  (params (EndPlayReason :type EEndPlayReason%20Enum :default "Destroyed"))
  (bind _playeractions (Variables|Default|GetPlayerActions))
  (bind _grid (Variables|/Game/TacticalStrategy/Blueprints/Core/Player/BP_PlayerActions.BP_PlayerActions_C|GetGrid _playeractions))
  (|CallParentFunction EndPlayReason)
  (Default|FClearStatefromTiles _grid "NewEnumerator8")
  (Default|FClearStatefromTiles _grid "NewEnumerator5"))

(fn ConstructionScript
  (|CallParentFunction))

(fn FGenerateReachables
  (params (Unit :type BP%20Unit%20Object%20Reference))
  (if (!= Unit (Variables|Default|GetCurrentUnitForReachables))
    (Variables|Default|SetCurrentUnitForReachables Unit)
    (Default|FClearStatefromTiles (Variables|/Game/TacticalStrategy/Blueprints/Core/Player/BP_PlayerActions.BP_PlayerActions_C|GetGrid (Variables|Default|GetPlayerActions)) "NewEnumerator8")
    (Default|FFindPath (Variables|/Game/TacticalStrategy/Blueprints/Core/Grid/BP_Grid.BP_Grid_C|GetGridPathfinding_Reachables (Variables|/Game/TacticalStrategy/Blueprints/Core/Player/BP_PlayerActions.BP_PlayerActions_C|GetGrid (Variables|Default|GetPlayerActions))) (Variables|/Game/TacticalStrategy/Blueprints/Core/Units/BP_Unit.BP_Unit_C|GetIndex (Variables|Default|GetCurrentUnitForReachables)) (Utilities|Struct|MakeIntPoint -999 -999) (.bCanMoveDiagonally (Utilities|Struct|BreakStruct_UnitData_Stats (.Stats (Utilities|Struct|BreakStruct_UnitData (Variables|/Game/TacticalStrategy/Blueprints/Core/Units/BP_Unit.BP_Unit_C|GetUnitData (Variables|Default|GetCurrentUnitForReachables)))))) (.ValidTileTypes (Utilities|Struct|BreakStruct_UnitData_Stats (.Stats (Utilities|Struct|BreakStruct_UnitData (Variables|/Game/TacticalStrategy/Blueprints/Core/Units/BP_Unit.BP_Unit_C|GetUnitData (Variables|Default|GetCurrentUnitForReachables)))))) 0.1 15.0 true (.MP_Current (Utilities|Struct|BreakStruct_UnitData_Stats (.Stats (Utilities|Struct|BreakStruct_UnitData (Variables|/Game/TacticalStrategy/Blueprints/Core/Units/BP_Unit.BP_Unit_C|GetUnitData (Variables|Default|GetCurrentUnitForReachables)))))))))

(fn FonPathfindingCompletedReachables
  (params (Reachables :type Array%20of%20Int%20Point%20Structures))
  (if (not (Variables|Default|GetbIsUnitWalking))
    (for _array_element Reachables
      (Default|FAddStatetoTile (Variables|/Game/TacticalStrategy/Blueprints/Core/Player/BP_PlayerActions.BP_PlayerActions_C|GetGrid (Variables|Default|GetPlayerActions)) _array_element "NewEnumerator8"))))

(fn FExecuteHoveredAction
  (params (index :type Int%20Point%20Structure))
  (bind _playeractions (Variables|Default|GetPlayerActions))
  (bind _hoveredunit (Variables|/Game/TacticalStrategy/Blueprints/Core/Player/BP_PlayerActions.BP_PlayerActions_C|GetHoveredUnit _playeractions))
  (|CallParentFunction index)
  (if (not (Variables|Default|GetbIsUnitWalking))
    (Utilities|IsValid _hoveredunit
      (:Is%20Valid
        (CallFunction|FGenerateReachables _hoveredunit))
      (:Is%20Not%20Valid
        (CallFunction|FGenerateReachables (Variables|/Game/TacticalStrategy/Blueprints/Core/Player/BP_PlayerActions.BP_PlayerActions_C|GetSelectedUnit _playeractions))
        (CallFunction|FGeneratePath)))))

(fn FGeneratePath
  (bind _playeractions (Variables|Default|GetPlayerActions))
  (bind _selectedunit (Variables|/Game/TacticalStrategy/Blueprints/Core/Player/BP_PlayerActions.BP_PlayerActions_C|GetSelectedUnit _playeractions))
  (bind _unitdata (Variables|/Game/TacticalStrategy/Blueprints/Core/Units/BP_Unit.BP_Unit_C|GetUnitData _selectedunit))
  (bind _stats (Utilities|Struct|BreakStruct_UnitData _unitdata))
  (bind (_validtiletypes _bcanmovediagonally _mp_current) (Utilities|Struct|BreakStruct_UnitData_Stats _stats))
  (Default|FClearStatefromTiles (Variables|/Game/TacticalStrategy/Blueprints/Core/Player/BP_PlayerActions.BP_PlayerActions_C|GetGrid (Variables|Default|GetPlayerActions)) "NewEnumerator5")
  (Utilities|Array|Clear (Variables|Default|GetGeneratedPath))
  (Default|FFindPath (Variables|/Game/TacticalStrategy/Blueprints/Core/Grid/BP_Grid.BP_Grid_C|GetGridPathfinding (Variables|/Game/TacticalStrategy/Blueprints/Core/Player/BP_PlayerActions.BP_PlayerActions_C|GetGrid _playeractions)) (Variables|/Game/TacticalStrategy/Blueprints/Core/Units/BP_Unit.BP_Unit_C|GetIndex _selectedunit) (Variables|/Game/TacticalStrategy/Blueprints/Core/Player/BP_PlayerActions.BP_PlayerActions_C|GetHoveredTile (Variables|Default|GetPlayerActions)) _bcanmovediagonally _validtiletypes 0.1 15.0 false _mp_current))

(fn FonPathfindingCompletedPath
  (params (Path :type Array%20of%20Int%20Point%20Structures))
  (bind _output_get (Variables|Default|SetGeneratedPath Path))
  (for _array_element _output_get
    (Default|FAddStatetoTile (Variables|/Game/TacticalStrategy/Blueprints/Core/Player/BP_PlayerActions.BP_PlayerActions_C|GetGrid (Variables|Default|GetPlayerActions)) _array_element "NewEnumerator5")))

(fn FExecuteAction
  (params (index :type Int%20Point%20Structure))
  (bind _playeractions (Variables|Default|GetPlayerActions))
  (|CallParentFunction index)
  (if (> (Utilities|Array|Length (Variables|Default|GetGeneratedPath)) 0)
    (Default|FMoveUnit (Variables|/Game/TacticalStrategy/Blueprints/Core/Player/BP_PlayerActions.BP_PlayerActions_C|GetCombatSystem _playeractions) (Variables|/Game/TacticalStrategy/Blueprints/Core/Player/BP_PlayerActions.BP_PlayerActions_C|GetSelectedUnit _playeractions) (Variables|Default|GetGeneratedPath))
    (Utilities|Array|Clear (Variables|Default|GetGeneratedPath))))

(fn FonUnitStartedWalking
  (params (Unit :type BP%20Unit%20Object%20Reference))
  (Variables|Default|SetbIsUnitWalking true)
  (Default|FClearStatefromTiles (Variables|/Game/TacticalStrategy/Blueprints/Core/Player/BP_PlayerActions.BP_PlayerActions_C|GetGrid (Variables|Default|GetPlayerActions)) "NewEnumerator8")
  (Variables|Default|SetCurrentUnitForReachables 0))

(fn FonUnitFinishedWalking
  (params (Unit :type BP%20Unit%20Object%20Reference))
  (Variables|Default|SetbIsUnitWalking false)
  (CallFunction|FExecuteHoveredAction (Variables|/Game/TacticalStrategy/Blueprints/Core/Player/BP_PlayerActions.BP_PlayerActions_C|GetHoveredTile (Variables|Default|GetPlayerActions))))