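; Player action that selects the hovered unit on the overworld map.
; On execute, it selects the hovered unit through PlayerActions unless that unit's overworld group is flagged as an encounter in the OverWorldUnitGroupsManager.
; With no valid hovered unit, or when the action ends play, it clears the selection using the -999 sentinel tile index.
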(event EventEndPlay
  (params (EndPlayReason :type EEndPlayReason%20Enum :default "Destroyed"))
  (|CallParentFunction EndPlayReason)
  (Default|FSetSelectedTileandUnit (Variables|Default|GetPlayerActions) (Utilities|Struct|MakeIntPoint -999 -999) 0 false))

(fn ConstructionScript
  (|CallParentFunction))

(fn FExecuteAction
  (params (index :type Int%20Point%20Structure))
  (bind _playeractions (Variables|Default|GetPlayerActions))
  (bind _playeractions_2 (Variables|Default|GetPlayerActions))
  (|CallParentFunction index)
  (Variables|/Game/TacticalStrategy/Blueprints/Core/Player/BP_PlayerActions.BP_PlayerActions_C|GetHoveredUnit (Variables|Default|GetPlayerActions)
    (:then
      (if (not (Utilities|Struct|BreakStruct_OverworldUnitGroup (.Value (Utilities|Map|Find (Variables|/Game/TacticalStrategy/Blueprints/Core/Units/OverworldUnitGroups/BP_Overworld_UnitGroupsManager.BP_Overworld_UnitGroupsManager_C|GetUnitGroups (Variables|/Game/TacticalStrategy/Blueprints/Core/Player/BP_PlayerActions.BP_PlayerActions_C|GetOverWorldUnitGroupsManager _playeractions_2)) (Variables|/Game/TacticalStrategy/Blueprints/Core/Units/BP_Unit.BP_Unit_C|GetOverworldGroupId (Variables|/Game/TacticalStrategy/Blueprints/Core/Player/BP_PlayerActions.BP_PlayerActions_C|GetHoveredUnit _playeractions_2))))))
        (Default|FSetSelectedTileandUnit :self _playeractions :Unit (Variables|/Game/TacticalStrategy/Blueprints/Core/Player/BP_PlayerActions.BP_PlayerActions_C|GetHoveredUnit _playeractions))))
    (:else
      (Default|FSetSelectedTileandUnit (Variables|Default|GetPlayerActions) (Utilities|Struct|MakeIntPoint -999 -999) 0 false))))