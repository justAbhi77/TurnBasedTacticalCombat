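; Player input hub for a tactical grid game, handling tile and unit hover, selection and mouse-click actions in overworld and combat.
; Every tick it traces under the cursor, updates grid tile states, and lets the spawned left- and right-click action actors react, repeating while a button is held.
; Combat system events swap those actions for turns, movement and spell casting, and manage the combat HUD and end screen, with number keys picking spells.
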(event Custom|eExecuteActionOnHoveredTileChanged
  (bind _selectedaction_rightclick (Variables|Default|GetSelectedAction_RightClick))
  (bind _selectedaction_leftclick (Variables|Default|GetSelectedAction_LeftClick))
  (Utilities|FlowControl|Sequence
    (:then_0
      (Utilities|IsValid _selectedaction_leftclick
        (:Is%20Valid
          (Default|FExecuteHoveredAction _selectedaction_leftclick (Variables|Default|GetHoveredTile))
          (if (Variables|Default|GetbIsLeftMouseDown)
            (Default|FExecuteAction (Variables|Default|GetSelectedAction_LeftClick) (Variables|Default|GetHoveredTile))))))
    (:then_1
      (Utilities|IsValid _selectedaction_rightclick
        (:Is%20Valid
          (Default|FExecuteHoveredAction _selectedaction_rightclick (Variables|Default|GetHoveredTile))
          (if (Variables|Default|GetbIsRightMouseDown)
            (Default|FExecuteAction (Variables|Default|GetSelectedAction_RightClick) (Variables|Default|GetHoveredTile))))))))

(event Custom|eSimulateClickFromExternalSources
  (Utilities|FlowControl|Sequence
    (:then_0
      (Variables|Default|SetbIsLeftMouseDown true)
      (CallFunction|FUpdateHoveredTileandUnit)
      (Utilities|IsValid (Variables|Default|GetSelectedAction_LeftClick)
        (:Is%20Valid
          (Default|FExecuteAction (Variables|Default|GetSelectedAction_LeftClick) (Variables|Default|GetHoveredTile)))))
    (:then_1
      (Variables|Default|SetbIsLeftMouseDown false))))

(event EventBeginPlay
  (bind _combatsystem (Variables|Public|GetCombatSystem))
  (Input|EnableInput (Game|GetPlayerController 0))
  (Utilities|FlowControl|Sequence
    (:then_0
      (Variables|Default|SetGrid (Variables|/Game/TacticalStrategy/Blueprints/Core/Combat/BP_CombatSystem.BP_CombatSystem_C|GetGrid (Variables|Public|GetCombatSystem)))
      (bind _grid (Variables|Default|GetGrid)
        (:then
          (EventDispatchers|BindEventtoOnGridGenerated _grid (EventDispatchers|CreateEvent :!event FonGridGenerated))
          (EventDispatchers|BindEventtoOnTileDataUpdated _grid (EventDispatchers|CreateEvent :!event FonTileDataUpdated)))
        (:else)))
    (:then_1
      (EventDispatchers|BindEventtoOnUnitGridIndexChanged (Variables|Public|GetCombatSystem) (EventDispatchers|CreateEvent :!event FonUnitGridIndexChanged)))
    (:then_2
      (bind _combatsystem_2 (Variables|Public|GetCombatSystem)
        (:then
          (EventDispatchers|BindEventtoOnCombatStarted _combatsystem_2 (EventDispatchers|CreateEvent :!event FonCombatStarted))
          (EventDispatchers|BindEventtoOnCombatEnded _combatsystem_2 (EventDispatchers|CreateEvent :!event FonCombatEnded))
          (EventDispatchers|BindEventtoOnUnitTurnStarted _combatsystem (EventDispatchers|CreateEvent :!event FonUnitTurnStarted))
          (EventDispatchers|BindEventtoOnUnitTurnEnded _combatsystem (EventDispatchers|CreateEvent :!event FonUnitTurnEnded))
          (EventDispatchers|BindEventtoOnCombatFinishing (Variables|Public|GetCombatSystem) (EventDispatchers|CreateEvent :!event FonCombatFinishing)))
        (:else)))
    (:then_3
      (bind _overworldunitgroupsmanager (Variables|Public|GetOverWorldUnitGroupsManager)
        (:then
          (Default|FSetCombatSystem _overworldunitgroupsmanager (Variables|Public|GetCombatSystem))
          (if (Variables|Public|GetAutoSelectOverworldMovementAction)
            (CallFunction|FSetSelectedActions "/Game/TacticalStrategy/Blueprints/Core/Player/Actions/Overworld/BP_Action_SelectUnitOverworld.BP_Action_SelectUnitOverworld_C" "/Game/TacticalStrategy/Blueprints/Core/Player/Actions/Overworld/BP_Action_MoveUnitOverworld.BP_Action_MoveUnitOverworld_C")))
        (:else)))))

(event EventTick
  (params (DeltaSeconds :type Float%20%28single-precision%29))
  (CallFunction|FUpdateHoveredTileandUnit))

(event Input|MouseEvents|LeftMouseButton
  (params (Key :type Key%20Structure))
  (:Pressed
    (Variables|Default|SetbIsLeftMouseDown true)
    (CallFunction|FUpdateHoveredTileandUnit)
    (Utilities|IsValid (Variables|Default|GetSelectedAction_LeftClick)
      (:Is%20Valid
        (Default|FExecuteAction (Variables|Default|GetSelectedAction_LeftClick) (Variables|Default|GetHoveredTile)))))
  (:Released
    (Variables|Default|SetbIsLeftMouseDown false)))

(event Input|MouseEvents|RightMouseButton
  (params (Key :type Key%20Structure))
  (:Pressed
    (Variables|Default|SetbIsRightMouseDown true)
    (CallFunction|FUpdateHoveredTileandUnit)
    (Utilities|IsValid (Variables|Default|GetSelectedAction_RightClick)
      (:Is%20Valid
        (Default|FExecuteAction (Variables|Default|GetSelectedAction_RightClick) (Variables|Default|GetHoveredTile)))))
  (:Released
    (Variables|Default|SetbIsRightMouseDown false)))

(event Input|KeyboardEvents|AnyKey
  (params (Key :type Key%20Structure))
  (bind _returnvalue (Class|KismetInputLibrary|KeyGetDisplayName Key true))
  (bind _combatsystem (Variables|Public|GetCombatSystem))
  (bind _returnvalue_2 (Utilities|String|ToString(Text) _returnvalue))
  (:Pressed
    (if (Math|Boolean|ANDBoolean (Variables|/Game/TacticalStrategy/Blueprints/Core/Combat/BP_CombatSystem.BP_CombatSystem_C|GetbIsInCombat _combatsystem) (not (Variables|/Game/TacticalStrategy/Blueprints/Core/Combat/BP_CombatSystem.BP_CombatSystem_C|GetbIsFinishingCombat _combatsystem)) (== (Variables|/Game/TacticalStrategy/Blueprints/Core/Combat/BP_CombatSystem.BP_CombatSystem_C|GetCurrentUnit _combatsystem) (Variables|Default|GetSelectedUnit)))
      (if (Class|KismetStringLibrary|IsNumeric _returnvalue_2)
        (Default|FSetSelectedSpellfromIndex (Variables|/Game/TacticalStrategy/Blueprints/Core/Combat/Widgets/WBP_Combat.WBP_Combat_C|GetWBP_ButtonList_Spells (Variables|Default|GetWBPCombat)) (- (Math|Conversions|ToInteger(Byte) _returnvalue_2) 1))))))

(fn ConstructionScript)

(fn FUpdateHoveredTileandUnit
  (Utilities|FlowControl|Sequence
    (:then_0
      (Utilities|FlowControl|Sequence
        (:then_0
          (Variables|Default|GetHoveredUnitOverride
            (:then
              (LocalVariables|SetU (Variables|Default|GetHoveredUnitOverride)))
            (:else
              (bind _unit (CallFunction|FGetUnitUnderCursor))
              (LocalVariables|SetU _unit))))
        (:then_1
          (if (!= (LocalVariables|GetU) (Variables|Default|GetHoveredUnit))
            (Utilities|FlowControl|Sequence
              (:then_0
                (bind _hoveredunit (Variables|Default|GetHoveredUnit)
                  (:then
                    (Default|FSetIsHovered _hoveredunit false))
                  (:else)))
              (:then_1
                (Variables|Default|SetHoveredUnit (LocalVariables|GetU))
                (bind _hoveredunit_2 (Variables|Default|GetHoveredUnit)
                  (:then
                    (Default|FSetIsHovered _hoveredunit_2 true))
                  (:else))))))))
    (:then_1
      (bind _hoveredunit_3 (Variables|Default|GetHoveredUnit)
        (:then
          (LocalVariables|SetNewIndex (Variables|/Game/TacticalStrategy/Blueprints/Core/Units/BP_Unit.BP_Unit_C|GetIndex _hoveredunit_3)))
        (:else
          (bind _index (Default|FGetTileIndexUnderCursor (Variables|Default|GetGrid) 0 (CallFunction|FCanHoverGround) (CallFunction|FCanHoverEmptySpaces)))
          (LocalVariables|SetNewIndex _index))))
    (:then_2
      (if (!= (LocalVariables|GetNewIndex) (Variables|Default|GetHoveredTile))
        (Default|FRemoveStatefromTile (Variables|Default|GetGrid) (Variables|Default|GetHoveredTile) "NewEnumerator1")
        (Variables|Default|SetHoveredTile (LocalVariables|GetNewIndex))
        (Default|FAddStatetoTile (Variables|Default|GetGrid) (Variables|Default|GetHoveredTile) "NewEnumerator1")
        (CallFunction|EExecuteActiononHoveredTileChanged)
        (Default|CallOnHoveredTileChanged (Variables|Default|GetHoveredTile))))))

(fn FSetSelectedActions
  (params (LeftAction :type BP%20Action%20Class%20Reference) (RightAction :type BP%20Action%20Class%20Reference))
  (Utilities|FlowControl|Sequence
    (:then_0
      (bind _selectedaction_leftclick (Variables|Default|GetSelectedAction_LeftClick)
        (:then
          (Actor|DestroyActor _selectedaction_leftclick)
          (Variables|Default|SetSelectedAction_LeftClick 0))
        (:else
          _))
      (if (Utilities|IsValidClass LeftAction)
        (bind _returnvalue (Game|SpawnActorfromClass LeftAction (Math|Transform|MakeTransform "0, 0, 0" "0, 0, 0" "1.000000,1.000000,1.000000") "AlwaysSpawn" "MultiplyWithRoot" 0 self 0))
        (Variables|Default|SetSelectedAction_LeftClick _returnvalue)))
    (:then_1
      (bind _selectedaction_rightclick (Variables|Default|GetSelectedAction_RightClick)
        (:then
          (Actor|DestroyActor _selectedaction_rightclick)
          (Variables|Default|SetSelectedAction_RightClick 0))
        (:else
          _))
      (if (Utilities|IsValidClass RightAction)
        (bind _returnvalue_2 (Game|SpawnActorfromClass RightAction (Math|Transform|MakeTransform "0, 0, 0" "0, 0, 0" "1.000000,1.000000,1.000000") "AlwaysSpawn" "MultiplyWithRoot" 0 self 0))
        (Variables|Default|SetSelectedAction_RightClick _returnvalue_2)))
    (:then_2
      (Default|CallOnSelectedActionsChanged (Variables|Default|GetSelectedAction_LeftClick) (Variables|Default|GetSelectedAction_RightClick)))))

(fn FGetUnitUnderCursor
  (params (PlayerIndex :type Integer))
  (bind _returnvalue (Game|GetPlayerController PlayerIndex))
  (bind (_hitresult _returnvalue_2) (Game|Player|GetHitResultUnderCursorbyChannel _returnvalue "TraceTypeQuery5" true))
  (if _returnvalue_2
    (return (.AsBP%20Unit (Utilities|Casting|CastToBP_Unit (.HitActor (Collision|BreakHitResult _hitresult)))))
    (else
      (bind _index (Default|FGetTileIndexUnderCursor (Variables|Default|GetGrid) PlayerIndex (CallFunction|FCanHoverGround) (CallFunction|FCanHoverEmptySpaces)))
      (return (.UnitOnTile (Utilities|Struct|BreakStruct_TileData (.Value (Utilities|Map|Find (Variables|/Game/TacticalStrategy/Blueprints/Core/Grid/BP_Grid.BP_Grid_C|GetGridTiles (Variables|Default|GetGrid)) _index))))))))

(fn FSetSelectedTileandUnit
  (params (Index :type Int%20Point%20Structure) (Unit :type BP%20Unit%20Object%20Reference) (bForce :type Boolean))
  (LocalVariables|SetDesiredIndex Index)
  (Utilities|FlowControl|Sequence
    (:then_0
      (Utilities|IsValid Unit
        (:Is%20Valid
          (LocalVariables|SetDesiredIndex (Variables|/Game/TacticalStrategy/Blueprints/Core/Units/BP_Unit.BP_Unit_C|GetIndex Unit)))))
    (:then_1
      (Utilities|FlowControl|Sequence
        (:then_0
          (Utilities|FlowControl|Sequence
            (:then_0
              (if (or (!= (Variables|Default|GetSelectedTile) (LocalVariables|GetDesiredIndex)) bForce)
                (Default|FRemoveStatefromTile (Variables|Default|GetGrid) (Variables|Default|GetSelectedTile) "NewEnumerator2")
                (Variables|Default|SetSelectedTile (LocalVariables|GetDesiredIndex))
                (Default|FAddStatetoTile (Variables|Default|GetGrid) (Variables|Default|GetSelectedTile) "NewEnumerator2")
                (else
                  (Default|FRemoveStatefromTile (Variables|Default|GetGrid) (Variables|Default|GetSelectedTile) "NewEnumerator2")
                  (Variables|Default|SetSelectedTile (Utilities|Struct|MakeIntPoint -999 -999)))))
            (:then_1
              (Default|CallOnSelectedTileChanged (Variables|Default|GetSelectedTile)))))
        (:then_1
          (LocalVariables|SetNewUnit (select (Utilities|IsValid Unit) Unit (Utilities|Struct|BreakStruct_TileData (.Value (Utilities|Map|Find (Variables|/Game/TacticalStrategy/Blueprints/Core/Grid/BP_Grid.BP_Grid_C|GetGridTiles (Variables|Default|GetGrid)) (Variables|Default|GetSelectedTile))))))
          (if (or (!= (Variables|Default|GetSelectedUnit) (LocalVariables|GetNewUnit)) bForce)
            (Utilities|FlowControl|Sequence
              (:then_0
                (bind _selectedunit (Variables|Default|GetSelectedUnit)
                  (:then
                    (Default|FSetIsSelected _selectedunit false))
                  (:else)))
              (:then_1
                (Variables|Default|SetSelectedUnit (LocalVariables|GetNewUnit))
                (bind _selectedunit_2 (Variables|Default|GetSelectedUnit)
                  (:then
                    (Default|FSetIsSelected _selectedunit_2 true))
                  (:else))))))))))

(fn FonGridGenerated
  (if (Default|FIsIndexValid (Variables|Default|GetGrid) (Variables|Default|GetSelectedTile))
    (CallFunction|FSetSelectedTileandUnit (Variables|Default|GetSelectedTile) 0 true)
    (else
      (CallFunction|FSetSelectedTileandUnit (Utilities|Struct|MakeIntPoint -999 -999) 0 true))))

(fn FonTileDataUpdated
  (params (Index :type Int%20Point%20Structure))
  (if (Class|KismetMathLibrary|EqualIntPointIntPoint Index (Variables|Default|GetSelectedTile))
    (CallFunction|FonGridGenerated)))

(fn FonUnitGridIndexChanged
  (params (Unit :type BP%20Unit%20Object%20Reference))
  (if (== Unit (Variables|Default|GetSelectedUnit))
    (CallFunction|FSetSelectedTileandUnit (Variables|/Game/TacticalStrategy/Blueprints/Core/Units/BP_Unit.BP_Unit_C|GetIndex Unit) 0 false)))

(fn FonCombatStarted
  (CallFunction|FSetSelectedActions)
  (CallFunction|FSetSelectedTileandUnit (Utilities|Struct|MakeIntPoint -999 -999) 0 false)
  (bind _returnvalue (UserInterface|CreateWidget "/Game/TacticalStrategy/Blueprints/Core/Combat/Widgets/WBP_Combat.WBP_Combat_C" 0 self))
  (bind _output_get (Variables|Default|SetWBPCombat _returnvalue))
  (UserInterface|Viewport|AddtoPlayerScreen _output_get)
  (EventDispatchers|BindEventtoOnSelectedSpellButtonChanged (Variables|/Game/TacticalStrategy/Blueprints/Core/Combat/Widgets/WBP_Combat.WBP_Combat_C|GetWBP_ButtonList_Spells (Variables|Default|GetWBPCombat)) (EventDispatchers|CreateEvent :!event FonSelectedSpellChanged)))

(fn FonCombatEnded
  (Widget|RemovefromParent (Variables|Default|GetWBPCombatEndScreen))
  (Variables|Default|SetWBPCombatEndScreen 0)
  (if (Variables|Public|GetAutoSelectOverworldMovementAction)
    (CallFunction|FSetSelectedActions "/Game/TacticalStrategy/Blueprints/Core/Player/Actions/Overworld/BP_Action_SelectUnitOverworld.BP_Action_SelectUnitOverworld_C" "/Game/TacticalStrategy/Blueprints/Core/Player/Actions/Overworld/BP_Action_MoveUnitOverworld.BP_Action_MoveUnitOverworld_C")
    (else
      (CallFunction|FSetSelectedActions))))

(fn FonUnitTurnStarted
  (params (Unit :type BP%20Unit%20Object%20Reference))
  (Utilities|IsValid (Variables|/Game/TacticalStrategy/Blueprints/Core/Units/BP_Unit.BP_Unit_C|GetAi Unit)
    (:Is%20Valid
      (if (!= (Utilities|GetClass (Variables|Default|GetSelectedAction_LeftClick)) "/Game/TacticalStrategy/Blueprints/Core/Player/Actions/Combat/BP_Action_Cbt_WaitForTurn.BP_Action_Cbt_WaitForTurn_C")
        (CallFunction|FSetSelectedActions "/Game/TacticalStrategy/Blueprints/Core/Player/Actions/Combat/BP_Action_Cbt_WaitForTurn.BP_Action_Cbt_WaitForTurn_C")))
    (:Is%20Not%20Valid
      (CallFunction|FSetSelectedTileandUnit (Variables|/Game/TacticalStrategy/Blueprints/Core/Units/BP_Unit.BP_Unit_C|GetIndex Unit) 0 false)
      (CallFunction|FSetSelectedActions "/Game/TacticalStrategy/Blueprints/Core/Player/Actions/Combat/BP_Action_Cbt_Move.BP_Action_Cbt_Move_C")
      (bind _wbpcombat (Variables|Default|GetWBPCombat)
        (:then
          (Default|FLinkUnittoSpellsList (Variables|/Game/TacticalStrategy/Blueprints/Core/Combat/Widgets/WBP_Combat.WBP_Combat_C|GetWBP_ButtonList_Spells _wbpcombat) (Variables|Default|GetSelectedUnit)))
        (:else)))))

(fn FonUnitTurnEnded
  (params (Unit :type BP%20Unit%20Object%20Reference))
  (CallFunction|FSetSelectedTileandUnit (Utilities|Struct|MakeIntPoint -999 -999) 0 false)
  (bind _wbpcombat (Variables|Default|GetWBPCombat)
    (:then
      (Default|FLinkUnittoSpellsList (Variables|/Game/TacticalStrategy/Blueprints/Core/Combat/Widgets/WBP_Combat.WBP_Combat_C|GetWBP_ButtonList_Spells _wbpcombat)))
    (:else)))

(fn FonSelectedSpellChanged
  (params (Button :type WBP%20Button%20Spell%20Object%20Reference))
  (Utilities|IsValid Button
    (:Is%20Valid
      (CallFunction|FSetSelectedActions "/Game/TacticalStrategy/Blueprints/Core/Player/Actions/Combat/BP_Action_Cbt_CastSpell.BP_Action_Cbt_CastSpell_C")
      (bind _asbp_action_cbt_cast_spell (Utilities|Casting|CastToBP_Action_Cbt_CastSpell (Variables|Default|GetSelectedAction_LeftClick)))
      (Default|FSetSpell _asbp_action_cbt_cast_spell (Variables|/Game/TacticalStrategy/Blueprints/Core/Combat/Spells/Widgets/WBP_Button_Spell.WBP_Button_Spell_C|GetSpellType Button)))
    (:Is%20Not%20Valid
      (if (!= (Utilities|GetClass (Variables|Default|GetSelectedAction_LeftClick)) "/Game/TacticalStrategy/Blueprints/Core/Player/Actions/Combat/BP_Action_Cbt_Move.BP_Action_Cbt_Move_C")
        (CallFunction|FSetSelectedActions "/Game/TacticalStrategy/Blueprints/Core/Player/Actions/Combat/BP_Action_Cbt_Move.BP_Action_Cbt_Move_C")))))

(fn FonCombatFinishing
  (CallFunction|FSetSelectedActions)
  (CallFunction|FSetSelectedTileandUnit (Utilities|Struct|MakeIntPoint -999 -999) 0 false)
  (Widget|RemovefromParent (Variables|Default|GetWBPCombat))
  (Variables|Default|SetWBPCombat 0)
  (bind _returnvalue (UserInterface|CreateWidget "/Game/TacticalStrategy/Blueprints/Core/Combat/Widgets/WBP_CombatEndScreen.WBP_CombatEndScreen_C" 0 self (Variables|/Game/TacticalStrategy/Blueprints/Core/Combat/BP_CombatSystem.BP_CombatSystem_C|GetTeamIndexThatWonLastCombat (Variables|Public|GetCombatSystem))))
  (bind _output_get (Variables|Default|SetWBPCombatEndScreen _returnvalue))
  (UserInterface|Viewport|AddtoPlayerScreen _output_get))

(fn FSetHoveredUnitOverride
  (params (Unit :type BP%20Unit%20Object%20Reference))
  (Variables|Default|SetHoveredUnitOverride Unit)
  (CallFunction|FUpdateHoveredTileandUnit))

(fn FCanHoverGround
  (bind _selectedaction_leftclick (Variables|Default|GetSelectedAction_LeftClick))
  (bind _selectedaction_rightclick (Variables|Default|GetSelectedAction_RightClick))
  (bind _returnvalue (Utilities|GetClass _selectedaction_rightclick))
  (bind _returnvalue_2 (Utilities|GetClass _selectedaction_leftclick))
  (bind _array (Utilities|Array|MakeArray _returnvalue_2 _returnvalue))
  (return (or (Utilities|Array|ContainsItem _array "/Game/TacticalStrategy/Blueprints/Core/Player/Actions/Overworld/BP_Action_Add_RemoveUnitFromOverworld.BP_Action_Add_RemoveUnitFromOverworld_C") (Utilities|Array|ContainsItem _array "/Game/TacticalStrategy/Blueprints/Core/Player/Actions/Overworld/BP_Action_MoveUnitOverworld.BP_Action_MoveUnitOverworld_C"))))

(fn FCanHoverEmptySpaces
  (return (or (Utilities|Array|ContainsItem (Utilities|Array|MakeArray (Utilities|GetClass (Variables|Default|GetSelectedAction_LeftClick)) (Utilities|GetClass (Variables|Default|GetSelectedAction_RightClick))) "/Game/TacticalStrategy/Blueprints/Core/Player/Actions/Grid/BP_Action_AddTile.BP_Action_AddTile_C") false)))