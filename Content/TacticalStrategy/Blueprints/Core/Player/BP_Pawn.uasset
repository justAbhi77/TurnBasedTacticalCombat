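; BP_Pawn is the player's camera pawn for a tactical strategy game, handling pan, zoom and stepped yaw rotation.
; Input axes shift a desired location along the pawn's forward and right vectors and a clamped desired spring arm length.
; Left and right rotation actions add a fixed yaw step to a desired rotation.
; Tick interpolates location, rotation and arm length toward these targets for smooth camera motion.
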(event EventTick
  (params (DeltaSeconds :type Float%20%28single-precision%29))
  ;[1 1 1] Tick
  (Variables|/Script/Engine.SpringArmComponent|SetTargetArmLength (Variables|Default|GetSpringArm) (Math|Interpolation|FInterpTo (Variables|/Script/Engine.SpringArmComponent|GetTargetArmLength (Variables|Default|GetSpringArm)) (Variables|Zoom|GetZoom_Desired) DeltaSeconds (Variables|Zoom|GetZoom_Interp)))
  (Transformation|SetActorLocation (Math|Interpolation|VInterpTo (Transformation|GetActorLocation) (Variables|Location|GetLocation_Desired) DeltaSeconds (Variables|Location|GetLocation_Interp)) false false)
  (Transformation|SetActorRotation (Math|Interpolation|RInterpTo (Transformation|GetActorRotation) (Variables|Rotation|GetRotation_Desired) DeltaSeconds (Variables|Rotation|GetRotation_Interp))))

(event EventBeginPlay
  ;[1 1 1] Begin Play
  (Variables|Location|SetLocation_Desired (Transformation|GetActorLocation))
  (Variables|Zoom|SetZoom_Desired (Variables|/Script/Engine.SpringArmComponent|GetTargetArmLength (Variables|Default|GetSpringArm)))
  (Variables|Rotation|SetRotation_Desired (Transformation|GetActorRotation)))

(event Input|ActionEvents|InputActionInputAction_RotationRight
  (params (Key :type Key%20Structure))
  ;[1 1 1] Input Actions
  (:Pressed
    (Variables|Rotation|SetRotation_Desired (Math|Rotator|CombineRotators (Variables|Rotation|GetRotation_Desired) (Math|Rotator|MakeRotator 0.0 0.0 (Variables|Rotation|GetRotation_Speed))))))

(event Input|ActionEvents|InputActionInputAction_RotationLeft
  (params (Key :type Key%20Structure))
  ;[1 1 1] Input Actions
  (:Pressed
    (Variables|Rotation|SetRotation_Desired (Math|Rotator|CombineRotators (Variables|Rotation|GetRotation_Desired) (Math|Rotator|MakeRotator 0.0 0.0 (- 0.0 (Variables|Rotation|GetRotation_Speed)))))))

(event Input|AxisEvents|InputAxisInputAxis_Zoom
  (params (AxisValue :type Float%20%28single-precision%29))
  ;[1 1 1] Inut Axes
  (Variables|Zoom|SetZoom_Desired (Math|Float|Clamp(Float) (+ (* AxisValue (Variables|Zoom|GetZoom_Speed)) (Variables|Zoom|GetZoom_Desired)) (Variables|Zoom|GetZoom_Min) (Variables|Zoom|GetZoom_Max))))

(event Input|AxisEvents|InputAxisInputAxis_Forward
  (params (AxisValue :type Float%20%28single-precision%29))
  ;[1 1 1] Inut Axes
  (Variables|Location|SetLocation_Desired (+ (Variables|Location|GetLocation_Desired) (* (* AxisValue (Variables|Location|GetLocation_Speed)) (Transformation|GetActorForwardVector)))))

(event Input|AxisEvents|InputAxisInputAxis_Right
  (params (AxisValue :type Float%20%28single-precision%29))
  ;[1 1 1] Inut Axes
  (Variables|Location|SetLocation_Desired (+ (Variables|Location|GetLocation_Desired) (* (* AxisValue (Variables|Location|GetLocation_Speed)) (Transformation|GetActorRightVector)))))

(fn ConstructionScript)