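; Manager that organizes overworld units into ID-keyed groups, mirroring hover across members and moving them together.
; Encounter groups wander and scatter around the moving unit, while other groups follow in a chain.
; A non-encounter unit reaching an encounter starts quick combat on a randomly sized grid shaped by the loaded level, with uninvolved units disabled.
; Afterwards it heals or destroys combatants by team result, then restores survivors' positions and encounter wandering.
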(event EventBeginPlay)

(fn ConstructionScript)

(fn FAddUnittoGroup
  (params (Unit :type BP%20Unit%20Object%20Reference) (GroupId :type Integer))
  (if (!= GroupId (Variables|/Game/TacticalStrategy/Blueprints/Core/Units/BP_Unit.BP_Unit_C|GetOverworldGroupId Unit))
    (CallFunction|FRemoveUnitfromCurrentGroup Unit)
    (if (!= GroupId -999)
      (bind _output_get (LocalVariables|SetGroup (.Value (Utilities|Map|Find (Variables|Default|GetUnitGroups) GroupId))))
      (Utilities|Array|Add (Utilities|Struct|BreakStruct_OverworldUnitGroup _output_get) Unit)
      (Utilities|Struct|SetmembersinStruct_OverworldUnitGroup (LocalVariables|GetGroup) GroupId)
      (Utilities|Map|Add (Variables|Default|GetUnitGroups) GroupId (LocalVariables|GetGroup))
      (Variables|/Game/TacticalStrategy/Blueprints/Core/Units/BP_Unit.BP_Unit_C|SetOverworldGroupId Unit GroupId)
      (Game|BindEventtoOnDestroyed Unit (EventDispatchers|CreateEvent :!event FonUnitDestroyed))
      (EventDispatchers|BindEventtoOnUnitHoveredChanged Unit (EventDispatchers|CreateEvent :!event FonUnitHoveredChanged))
      (EventDispatchers|BindEventtoOnUnitStartedWalkingOverworld Unit (EventDispatchers|CreateEvent :!event FonUnitStartedWalkingOverworld))
      (EventDispatchers|BindEventtoOnUnitReachedUnitOverworld Unit (EventDispatchers|CreateEvent :!event FonUnitReachedUnitOverworld)))))

(fn FRemoveUnitfromCurrentGroup
  (params (Unit :type BP%20Unit%20Object%20Reference))
  (if (!= (Variables|/Game/TacticalStrategy/Blueprints/Core/Units/BP_Unit.BP_Unit_C|GetOverworldGroupId Unit) -999)
    (bind _output_get (LocalVariables|SetGroup (.Value (Utilities|Map|Find (Variables|Default|GetUnitGroups) (Variables|/Game/TacticalStrategy/Blueprints/Core/Units/BP_Unit.BP_Unit_C|GetOverworldGroupId Unit)))))
    (Utilities|Array|RemoveItem (.Units (Utilities|Struct|BreakStruct_OverworldUnitGroup _output_get)) Unit)
    (Utilities|FlowControl|Sequence
      (:then_0
        (if (> (Utilities|Array|Length (.Units (Utilities|Struct|BreakStruct_OverworldUnitGroup _output_get))) 0)
          (Utilities|Map|Add (Variables|Default|GetUnitGroups) (Variables|/Game/TacticalStrategy/Blueprints/Core/Units/BP_Unit.BP_Unit_C|GetOverworldGroupId Unit) (LocalVariables|GetGroup))
          (else
            (Utilities|Map|Remove (Variables|Default|GetUnitGroups) (Variables|/Game/TacticalStrategy/Blueprints/Core/Units/BP_Unit.BP_Unit_C|GetOverworldGroupId Unit)))))
      (:then_1
        (Variables|/Game/TacticalStrategy/Blueprints/Core/Units/BP_Unit.BP_Unit_C|SetOverworldGroupId Unit -999)
        (EventDispatchers|UnbindEventfromOnUnitHoveredChanged Unit (EventDispatchers|CreateEvent :!event FonUnitHoveredChanged))
        (EventDispatchers|UnbindEventfromOnUnitStartedWalkingOverworld Unit (EventDispatchers|CreateEvent :!event FonUnitStartedWalkingOverworld))
        (EventDispatchers|UnbindEventfromOnUnitReachedUnitOverworld Unit (EventDispatchers|CreateEvent :!event FonUnitReachedUnitOverworld))))))

(fn FonUnitDestroyed
  (params (DestroyedActor :type Actor%20Object%20Reference))
  (bind _asbp_unit (Utilities|Casting|CastToBP_Unit DestroyedActor))
  (CallFunction|FRemoveUnitfromCurrentGroup _asbp_unit))

(fn FonUnitHoveredChanged
  (params (Unit :type BP%20Unit%20Object%20Reference))
  (bind _unitgroups (Variables|Default|GetUnitGroups))
  (bind _overworldgroupid (Variables|/Game/TacticalStrategy/Blueprints/Core/Units/BP_Unit.BP_Unit_C|GetOverworldGroupId Unit))
  (bind (_value _returnvalue) (Utilities|Map|Find _unitgroups _overworldgroupid))
  (if (not (Variables|/Game/TacticalStrategy/Blueprints/Core/Combat/BP_CombatSystem.BP_CombatSystem_C|GetbIsInCombat (Variables|Default|GetCombatSystem)))
    (if _returnvalue
      (bind _output_get (LocalVariables|SetGroup _value))
      (for _array_element (.Units (Utilities|Struct|BreakStruct_OverworldUnitGroup _output_get))
        (LocalVariables|SetU _array_element)
        (if (!= (LocalVariables|GetU) Unit)
          (EventDispatchers|UnbindEventfromOnUnitHoveredChanged (LocalVariables|GetU) (EventDispatchers|CreateEvent :!event FonUnitHoveredChanged))
          (Default|FSetIsHovered (LocalVariables|GetU) (Variables|/Game/TacticalStrategy/Blueprints/Core/Units/BP_Unit.BP_Unit_C|GetbIsHovered Unit))
          (EventDispatchers|BindEventtoOnUnitHoveredChanged (LocalVariables|GetU) (EventDispatchers|CreateEvent :!event FonUnitHoveredChanged)))))))

(fn FonUnitStartedWalkingOverworld
  (params (Unit :type BP%20Unit%20Object%20Reference))
  (if (Utilities|Struct|BreakStruct_OverworldUnitGroup (.Value (Utilities|Map|Find (Variables|Default|GetUnitGroups) (Variables|/Game/TacticalStrategy/Blueprints/Core/Units/BP_Unit.BP_Unit_C|GetOverworldGroupId Unit))))
    (for _array_element (.Units (Utilities|Struct|BreakStruct_OverworldUnitGroup (.Value (Utilities|Map|Find (Variables|Default|GetUnitGroups) (Variables|/Game/TacticalStrategy/Blueprints/Core/Units/BP_Unit.BP_Unit_C|GetOverworldGroupId Unit)))))
      (LocalVariables|SetU _array_element)
      (if (!= (LocalVariables|GetU) Unit)
        (EventDispatchers|UnbindEventfromOnUnitStartedWalkingOverworld (LocalVariables|GetU) (EventDispatchers|CreateEvent :!event FonUnitStartedWalkingOverworld))
        (bind _randomlocation (Default|FGetRandomReachableLocationinRadius (LocalVariables|GetU) (Variables|/Game/TacticalStrategy/Blueprints/Core/Units/BP_Unit.BP_Unit_C|GetTargetLocationInOverworld Unit) "(X=100.000000,Y=400.000000)"))
        (Default|EMoveUnitinOverworld (LocalVariables|GetU) _randomlocation 0 false)
        (EventDispatchers|BindEventtoOnUnitStartedWalkingOverworld (LocalVariables|GetU) (EventDispatchers|CreateEvent :!event FonUnitStartedWalkingOverworld))))
    (else
      (LocalVariables|SetPreviousUnitInChain Unit)
      (for _array_element_2 (.Units (Utilities|Struct|BreakStruct_OverworldUnitGroup (.Value (Utilities|Map|Find (Variables|Default|GetUnitGroups) (Variables|/Game/TacticalStrategy/Blueprints/Core/Units/BP_Unit.BP_Unit_C|GetOverworldGroupId Unit)))))
        (LocalVariables|SetU _array_element_2)
        (if (!= (LocalVariables|GetU) Unit)
          (EventDispatchers|UnbindEventfromOnUnitStartedWalkingOverworld (LocalVariables|GetU) (EventDispatchers|CreateEvent :!event FonUnitStartedWalkingOverworld))
          (Default|EMoveUnitinOverworld (LocalVariables|GetU) "0, 0, 0" (LocalVariables|GetPreviousUnitInChain) false)
          (LocalVariables|SetPreviousUnitInChain (LocalVariables|GetU))
          (EventDispatchers|BindEventtoOnUnitStartedWalkingOverworld (LocalVariables|GetU) (EventDispatchers|CreateEvent :!event FonUnitStartedWalkingOverworld)))))))

(fn FSetGroupIsEncounter
  (params (bIsEncounter :type Boolean) (GroupId :type Integer))
  (bind _unitgroups (Variables|Default|GetUnitGroups))
  (bind (_value _returnvalue) (Utilities|Map|Find _unitgroups GroupId))
  (if _returnvalue
    (bind _output_get (LocalVariables|SetGroup _value))
    (if (!= (Utilities|Struct|BreakStruct_OverworldUnitGroup _output_get) bIsEncounter)
      (Utilities|Struct|SetmembersinStruct_OverworldUnitGroup (LocalVariables|GetGroup) bIsEncounter)
      (Utilities|Map|Add (Variables|Default|GetUnitGroups) GroupId (LocalVariables|GetGroup))
      (for _array_element (Utilities|Struct|BreakStruct_OverworldUnitGroup (LocalVariables|GetGroup))
        (Default|EStopMovingUnitinOverworld _array_element))
      (if (.bIsEncounter (Utilities|Struct|BreakStruct_OverworldUnitGroup (LocalVariables|GetGroup)))
        (Default|EMoveUnitinOverworld (Utilities|Array|Get(acopy) (.Units (Utilities|Struct|BreakStruct_OverworldUnitGroup (LocalVariables|GetGroup)))) "0, 0, 0" 0 true)))))

(fn FSetCombatSystem
  (params (CombatSystem :type BP%20Combat%20System%20Object%20Reference))
  (Variables|Default|SetCombatSystem CombatSystem)
  (EventDispatchers|BindEventtoOnCombatEnded (Variables|Default|GetCombatSystem) (EventDispatchers|CreateEvent :!event FonCombatEnded)))

(fn FonUnitReachedUnitOverworld
  (params (Unit :type BP%20Unit%20Object%20Reference))
  (bind _unitgroups (Variables|Default|GetUnitGroups))
  (LocalVariables|SetGroup1 (.Value (Utilities|Map|Find _unitgroups (Variables|/Game/TacticalStrategy/Blueprints/Core/Units/BP_Unit.BP_Unit_C|GetOverworldGroupId Unit))))
  (LocalVariables|SetGroup2 (.Value (Utilities|Map|Find _unitgroups (Variables|/Game/TacticalStrategy/Blueprints/Core/Units/BP_Unit.BP_Unit_C|GetOverworldGroupId (Variables|/Game/TacticalStrategy/Blueprints/Core/Units/BP_Unit.BP_Unit_C|GetUnitToFollowOverworld Unit)))))
  (if (Math|Boolean|ANDBoolean (!= (.GroupId (Utilities|Struct|BreakStruct_OverworldUnitGroup (LocalVariables|GetGroup1))) (.GroupId (Utilities|Struct|BreakStruct_OverworldUnitGroup (LocalVariables|GetGroup2)))) (not (.bIsEncounter (Utilities|Struct|BreakStruct_OverworldUnitGroup (LocalVariables|GetGroup1)))) (.bIsEncounter (Utilities|Struct|BreakStruct_OverworldUnitGroup (LocalVariables|GetGroup2))))
    (CallFunction|FTriggerEncounter (Utilities|Array|MakeArray (LocalVariables|GetGroup1) (LocalVariables|GetGroup2)))))

(fn FTriggerEncounter
  (params (Group :type Array%20of%20Struct%20Overworld%20Unit%20Group%20Structures))
  (if (not (Variables|/Game/TacticalStrategy/Blueprints/Core/Combat/BP_CombatSystem.BP_CombatSystem_C|GetbIsInCombat (Variables|Default|GetCombatSystem)))
    (Utilities|FlowControl|Sequence
      (:then_0
        (Utilities|Map|Clear (Variables|Default|GetUnitPositionsWhenCombatStarted))
        (bind _values (Utilities|Map|Values (Variables|Default|GetUnitGroups)))
        (for _array_element _values
          (for _array_element_2 (Utilities|Struct|BreakStruct_OverworldUnitGroup _array_element)
            (Utilities|Map|Add (Variables|Default|GetUnitPositionsWhenCombatStarted) _array_element_2 (Transformation|GetActorLocation _array_element_2))
            (if (not (Utilities|Array|ContainsItem Group _array_element))
              (Default|FDisableUnit _array_element_2)))))
      (:then_1
        (LocalVariables|SetGridData (Utilities|Struct|MakeStruct_QuickCombat_Grid true (Transformation|GetActorLocation (Utilities|Array|Get(acopy) (Utilities|Struct|BreakStruct_OverworldUnitGroup (Utilities|Array|Get(acopy) Group)))) "200.000000,200.000000,100.000000" (Utilities|Struct|MakeIntPoint (Math|Random|RandomIntegerinRange 10 20) (Math|Random|RandomIntegerinRange 10 20)) (CallFunction|FGuessGridShapefromLoadedLevel)))
        (for _array_element_3 Group
          (Utilities|Array|Add (LocalVariables|GetUnitTeams) (Utilities|Struct|MakeStruct_UnitArray (.Units (Utilities|Struct|BreakStruct_OverworldUnitGroup _array_element_3))))
          (if (.bIsEncounter (Utilities|Struct|BreakStruct_OverworldUnitGroup _array_element_3))
            (Utilities|Array|AppendArray (LocalVariables|GetControlledByAi) (.Units (Utilities|Struct|BreakStruct_OverworldUnitGroup _array_element_3)))))
        (Default|FQuickStartCombat (Variables|Default|GetCombatSystem) (LocalVariables|GetGridData) (Utilities|Struct|MakeStruct_QuickCombat_UnitTeams (LocalVariables|GetUnitTeams) (LocalVariables|GetControlledByAi) (Utilities|Map|MakeMap)) self)))))

(fn FonCombatEnded
  (bind _combatsystem (Variables|Default|GetCombatSystem))
  (bind _teamindexthatwonlastcombat (Variables|/Game/TacticalStrategy/Blueprints/Core/Combat/BP_CombatSystem.BP_CombatSystem_C|GetTeamIndexThatWonLastCombat _combatsystem))
  (if (== (Variables|/Game/TacticalStrategy/Blueprints/Core/Combat/BP_CombatSystem.BP_CombatSystem_C|GetObjectThatStartedCombat (Variables|Default|GetCombatSystem)) self)
    (bind _keys (Utilities|Map|Keys (Variables|/Game/TacticalStrategy/Blueprints/Core/Combat/BP_CombatSystem.BP_CombatSystem_C|GetUnitTeams (Variables|Default|GetCombatSystem))))
    (for _array_element _keys
      (LocalVariables|SetTeamIndex _array_element)
      (bind _output_get (LocalVariables|SetUnitsInTeam (Utilities|Struct|BreakStruct_UnitArray (.Value (Utilities|Map|Find (Variables|/Game/TacticalStrategy/Blueprints/Core/Combat/BP_CombatSystem.BP_CombatSystem_C|GetUnitTeams (Variables|Default|GetCombatSystem)) (LocalVariables|GetTeamIndex))))))
      (for _array_element_2 _output_get
        (LocalVariables|SetUnit _array_element_2)
        (Default|FRemoveUnitfromCombat (Variables|Default|GetCombatSystem) (LocalVariables|GetUnit))
        (if (Math|Boolean|ORBoolean (== (LocalVariables|GetTeamIndex) 0) (== (LocalVariables|GetTeamIndex) _teamindexthatwonlastcombat) (== _teamindexthatwonlastcombat -1))
          (Default|FResetHp (LocalVariables|GetUnit))
          (else
            (Actor|DestroyActor (LocalVariables|GetUnit))))))
    (bind _keys_2 (Utilities|Map|Keys (Variables|Default|GetUnitPositionsWhenCombatStarted)))
    (for _array_element_3 _keys_2
      (bind _output_get_2 (LocalVariables|SetUnit _array_element_3))
      (Utilities|IsValid _output_get_2
        (:Is%20Valid
          (Transformation|SetActorLocation (LocalVariables|GetUnit) (.Value (Utilities|Map|Find (Variables|Default|GetUnitPositionsWhenCombatStarted) (LocalVariables|GetUnit))) false false)
          (Default|FEnableUnit (LocalVariables|GetUnit) "NewEnumerator1"))))
    (Utilities|Map|Clear (Variables|Default|GetUnitPositionsWhenCombatStarted))
    (bind _values (Utilities|Map|Values (Variables|Default|GetUnitGroups)))
    (for _array_element_4 _values
      (if (.bIsEncounter (Utilities|Struct|BreakStruct_OverworldUnitGroup _array_element_4))
        (Default|EMoveUnitinOverworld (Utilities|Array|Get(acopy) (.Units (Utilities|Struct|BreakStruct_OverworldUnitGroup _array_element_4))) "0, 0, 0" 0 true)))
    (Default|FDestroyGrid (Variables|/Game/TacticalStrategy/Blueprints/Core/Combat/BP_CombatSystem.BP_CombatSystem_C|GetGrid (Variables|Default|GetCombatSystem)))))

(fn FGuessGridShapefromLoadedLevel
  (bind _enumvalue (|ForEachE_GridShape)
    (:LoopBody
      (Utilities|IsValid (Class|GameplayStatics|GetStreamingLevel (Utilities|String|StringToName (Utilities|String|Append "L_" (Utilities|String|EnumtoString _enumvalue))))
        (:Is%20Valid
          (if (Variables|/Script/Engine.LevelStreaming|GetbShouldBeVisible (Class|GameplayStatics|GetStreamingLevel (Utilities|String|StringToName (Utilities|String|Append "L_" (Utilities|String|EnumtoString _enumvalue)))))
            (return _enumvalue)))))
    (:then
      (return "NewEnumerator1"))))