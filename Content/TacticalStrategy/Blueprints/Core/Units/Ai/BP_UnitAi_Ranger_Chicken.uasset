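; Unit AI for the Ranger "Chicken" in tactical combat, which picks a random spell at combat start and withholds it from its available spells.
; When the spell decision ends without a valid cast, it falls back to that withheld spell if castable, scoring each target in range before running the parent logic.
; The scoring loop is time-sliced with short delays and stops if the unit leaves combat; debug prints remain.
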(event EventEDecideWhichSpelltoCastDone
  (bind _unit (Variables|Default|GetUnit))
  (bind _index (Variables|/Game/TacticalStrategy/Blueprints/Core/Units/BP_Unit.BP_Unit_C|GetIndex _unit))
  (if (not (Utilities|Struct|BreakStruct_UnitAiSpellCastingData (Variables|Default|GetAiSpellCasting)))
    (bind _spelldata (CallFunction|FGetSpellDatafromSpell (Variables|Default|GetAvailableRandomSpell)))
    (bind _output_get (Variables|Default|SetSpellDataToCast _spelldata))
    (bind _bcancastspell (Default|FCanCastSpell (Variables|Default|GetUnit) _output_get))
    (if _bcancastspell
      (bind _rangesindexes (Default|FGetSpellRange (Variables|Default|GetCombatSystem) _index (Utilities|Struct|BreakStruct_SpellData (Variables|Default|GetSpellDataToCast))))
      (bind _array_element (Utilities|ManualforEachLoop _rangesindexes :!label _label)
        (:LoopBody
          (CallFunction|FCalculateSpellScoreandUpdateSpellCasting _array_element _index (Variables|Default|GetSpellDataToCast))
          (Utilities|DelayifTakingTooMuchTime)
          (goto _label NextLoop))
        (:Completed
          (Development|PrintString (Utilities|String|ToString(Boolean) (.bIsSpellValid (Utilities|Struct|BreakStruct_UnitAiSpellCastingData (Variables|Default|GetAiSpellCasting)))))
          (|CallParentFunction)))
      (else
        (|CallParentFunction)))
    (else
      (|CallParentFunction))))

(fn ConstructionScript
  (|CallParentFunction))

(fn FGetAvailableSpells
  (bind _output_get (LocalVariables|SetRet (|CallParentFunction)))
  (Utilities|Array|RemoveItem _output_get (Variables|Default|GetAvailableRandomSpell))
  (return (LocalVariables|GetRet)))

(fn FAiCombatStarted
  (|CallParentFunction)
  (bind _output_get (Variables|Default|SetAvailableRandomSpell (.OutItem (Utilities|Array|Random (CallFunction|FGetAvailableSpells)))))
  (Development|PrintString (Utilities|String|Append "Until Will not Cast This Spell For Combat " (Utilities|String|EnumtoString _output_get)) true true "(R=0.000000,G=0.660000,B=1.000000,A=1.000000)" 5.0))