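; Debug actor that overlays text on walkable BP_Grid tiles, showing toggleable tile indexes and pathfinding costs and sort order.
; Binds to grid and pathfinding delegates on BeginPlay, with a retriggerable delay event for debounced full refreshes.
; Lazily spawns one TextRenderActor per tile, cached in a map, scaled by longest entry to fit the tile.
; Destroys text actors when tiles have nothing to show or all toggles are off.
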(event Custom|eUpdatetextAfterDelay
  (params (Index :type Int%20Point%20Structure))
  (Utilities|FlowControl|RetriggerableDelay 0.2)
  (CallFunction|FUpdatetextonAllTiles))

(event EventBeginPlay
  (bind _returnvalue (Actor|GetActorOfClass "/Game/Blueprints/Core/Grid/BP_Grid.BP_Grid_C"))
  (bind _output_get (Variables|Default|SetGrid _returnvalue))
  (EventDispatchers|AssignOnTileDataUpdated _output_get (EventDispatchers|CreateEvent :!event FUpdateTextonTile))
  (EventDispatchers|BindEventtoOnGridDestroyed _output_get (EventDispatchers|CreateEvent :!event FClearAllTextActors))
  (EventDispatchers|BindEventtoOnPathFindingDataUpdated (Variables|/Game/Blueprints/Core/Grid/BP_Grid.BP_Grid_C|GetGridPathfinding (Variables|Default|GetGrid)) (EventDispatchers|CreateEvent :!event Custom|eUpdatetextAfterDelay))
  (EventDispatchers|BindEventtoOnPathFindingDataCleared (Variables|/Game/Blueprints/Core/Grid/BP_Grid.BP_Grid_C|GetGridPathfinding (Variables|Default|GetGrid)) (EventDispatchers|CreateEvent :!event FUpdatetextonAllTiles)))

(fn ConstructionScript)

(fn FGetTextActor
  (params (Index :type Int%20Point%20Structure))
  (bind _output_get (LocalVariables|SetActor (.Value (Utilities|Map|Find (Variables|Default|GetSpawnTexts) Index))))
  (Utilities|IsValid _output_get
    (:Is%20Valid
      (return (LocalVariables|GetActor)))
    (:Is%20Not%20Valid
      (bind _returnvalue (Game|SpawnActorfromClass "/Script/Engine.TextRenderActor" (Math|Transform|MakeTransform "0, 0, 0" "0, 0, 0" "1.000000,1.000000,1.000000") "AlwaysSpawn" "MultiplyWithRoot" 0 0))
      (LocalVariables|SetActor _returnvalue)
      (Utilities|Map|Add (Variables|Default|GetSpawnTexts) Index (LocalVariables|GetActor))
      (Actor|Tick|SetActorTickEnabled (LocalVariables|GetActor))
      (Collision|SetActorEnableCollision (LocalVariables|GetActor) false)
      (Rendering|Components|TextRender|SetHorizontalAlignment (Variables|/Script/Engine.TextRenderActor|GetTextRender (LocalVariables|GetActor)) "EHTA_Center")
      (Class|TextRenderComponent|SetVerticalAlignment (Variables|/Script/Engine.TextRenderActor|GetTextRender (LocalVariables|GetActor)) "EVRTA_TextCenter")
      (return (LocalVariables|GetActor)))))

(fn FDestroyTextActor
  (params (Index :type Int%20Point%20Structure))
  (bind _output_get (LocalVariables|SetActor (.Value (Utilities|Map|Find (Variables|Default|GetSpawnTexts) Index))))
  (Utilities|IsValid _output_get
    (:Is%20Valid
      (Actor|DestroyActor _output_get)
      (Utilities|Map|Remove (Variables|Default|GetSpawnTexts) Index))))

(fn FClearAllTextActors
  (bind _values (Utilities|Map|Values (Variables|Default|GetSpawnTexts)))
  (for _array_element _values
    (Actor|DestroyActor _array_element))
  (Utilities|Map|Clear (Variables|Default|GetSpawnTexts)))

(fn FUpdateTextonTile
  (params (Index :type Int%20Point%20Structure))
  (bind _returnvalue (Utilities|String|ToString(Integer) (.y Index)))
  (bind _returnvalue_2 (Utilities|String|ToString(Integer) (.x Index)))
  (bind _returnvalue_3 (Utilities|String|Append _returnvalue_2 "," _returnvalue))
  (if (CallFunction|FWanttoDisplayAnyText)
    (Variables|Default|GetGrid
      (:then
        _)
      (:else
        (bind _returnvalue_4 (Actor|GetActorOfClass "/Game/Blueprints/Core/Grid/BP_Grid.BP_Grid_C"))
        (Variables|Default|SetGrid _returnvalue_4)))
    (if (.ReturnValue (Utilities|Map|Find (Variables|/Game/Blueprints/Core/Grid/BP_Grid.BP_Grid_C|GetGridTiles (Variables|Default|GetGrid)) Index))
      (LocalVariables|SetData (.Value (Utilities|Map|Find (Variables|/Game/Blueprints/Core/Grid/BP_Grid.BP_Grid_C|GetGridTiles (Variables|Default|GetGrid)) Index)))
      (if (CallFunction|FIsTileTypeWalkable (.tiletype (LocalVariables|GetData)))
        (bind _textrender (CallFunction|FGetTextActor Index))
        (LocalVariables|SetTextRender _textrender)
        (Utilities|FlowControl|Sequence
          (:then_0
            (Utilities|FlowControl|Sequence
              (:then_0
                (if (Variables|Default|GetbSetShowTileIndexes)
                  (Utilities|Array|Add (LocalVariables|GetText) _returnvalue_3)
                  (Utilities|Array|Add (LocalVariables|GetTextLength) (Utilities|String|Len _returnvalue_3))))
              (:then_1
                (if (Math|Boolean|ORBoolean (Variables|Default|GetbSetShowCostToEnterTile) (Variables|Default|GetbSetShowMinCostToTarget) (Variables|Default|GetbSetShowCostFromStart) (Variables|Default|GetbSetShowSortOrder))
                  (if (.ReturnValue (Utilities|Map|Find (Variables|/Game/Blueprints/Core/Grid/BP_GridPathfinding.BP_GridPathfinding_C|GetPathFindingData (Variables|/Game/Blueprints/Core/Grid/BP_Grid.BP_Grid_C|GetGridPathfinding (Variables|Default|GetGrid))) Index))
                    (LocalVariables|SetPathFindingData (.Value (Utilities|Map|Find (Variables|/Game/Blueprints/Core/Grid/BP_GridPathfinding.BP_GridPathfinding_C|GetPathFindingData (Variables|/Game/Blueprints/Core/Grid/BP_Grid.BP_Grid_C|GetGridPathfinding (Variables|Default|GetGrid))) Index)))
                    (Utilities|FlowControl|Sequence
                      (:then_0
                        (if (Variables|Default|GetbSetShowCostToEnterTile)
                          (Utilities|Array|Add (LocalVariables|GetText) (Utilities|String|Append "Enter: " (Utilities|String|ToString(Integer) (.CostToEnterTile (Utilities|Struct|BreakStruct_PathfindingData (LocalVariables|GetPathFindingData))))))
                          (Utilities|Array|Add (LocalVariables|GetTextLength) (Utilities|String|Len (Utilities|String|Append "Enter: " (Utilities|String|ToString(Integer) (.CostToEnterTile (Utilities|Struct|BreakStruct_PathfindingData (LocalVariables|GetPathFindingData)))))))))
                      (:then_1
                        (if (Variables|Default|GetbSetShowMinCostToTarget)
                          (if (!= (.MinimumCostToTarget (Utilities|Struct|BreakStruct_PathfindingData (LocalVariables|GetPathFindingData))) 99999)
                            (Utilities|Array|Add (LocalVariables|GetText) (Utilities|String|Append "Min: " (Utilities|String|ToString(Integer) (.MinimumCostToTarget (Utilities|Struct|BreakStruct_PathfindingData (LocalVariables|GetPathFindingData))))))
                            (Utilities|Array|Add (LocalVariables|GetTextLength) (Utilities|String|Len (Utilities|String|Append "Min: " (Utilities|String|ToString(Integer) (.MinimumCostToTarget (Utilities|Struct|BreakStruct_PathfindingData (LocalVariables|GetPathFindingData))))))))))
                      (:then_2
                        (if (Variables|Default|GetbSetShowCostFromStart)
                          (if (!= (.MinimumCostToTarget (Utilities|Struct|BreakStruct_PathfindingData (LocalVariables|GetPathFindingData))) 99999)
                            (Utilities|Array|Add (LocalVariables|GetText) (Utilities|String|Append "Start: " (Utilities|String|ToString(Integer) (.MinimumCostToTarget (Utilities|Struct|BreakStruct_PathfindingData (LocalVariables|GetPathFindingData))))))
                            (Utilities|Array|Add (LocalVariables|GetTextLength) (Utilities|String|Len (Utilities|String|Append "Start: " (Utilities|String|ToString(Integer) (.MinimumCostToTarget (Utilities|Struct|BreakStruct_PathfindingData (LocalVariables|GetPathFindingData))))))))))
                      (:then_3
                        (if (Variables|Default|GetbSetShowSortOrder)
                          (if (!= (Utilities|Array|FindItem (Variables|/Game/Blueprints/Core/Grid/BP_GridPathfinding.BP_GridPathfinding_C|GetDiscoveredTileIndexes (Variables|/Game/Blueprints/Core/Grid/BP_Grid.BP_Grid_C|GetGridPathfinding (Variables|Default|GetGrid))) Index) -1)
                            (Utilities|Array|Add (LocalVariables|GetText) (Utilities|String|Append "Sort: " (Utilities|String|ToString(Integer) (Utilities|Array|FindItem (Variables|/Game/Blueprints/Core/Grid/BP_GridPathfinding.BP_GridPathfinding_C|GetDiscoveredTileIndexes (Variables|/Game/Blueprints/Core/Grid/BP_Grid.BP_Grid_C|GetGridPathfinding (Variables|Default|GetGrid))) Index)) "( " (Utilities|String|ToString(Integer) (Utilities|Array|Get(acopy) (Variables|/Game/Blueprints/Core/Grid/BP_GridPathfinding.BP_GridPathfinding_C|GetDiscoveredTileSortingCost (Variables|/Game/Blueprints/Core/Grid/BP_Grid.BP_Grid_C|GetGridPathfinding (Variables|Default|GetGrid))) (Utilities|Array|FindItem (Variables|/Game/Blueprints/Core/Grid/BP_GridPathfinding.BP_GridPathfinding_C|GetDiscoveredTileIndexes (Variables|/Game/Blueprints/Core/Grid/BP_Grid.BP_Grid_C|GetGridPathfinding (Variables|Default|GetGrid))) Index))) " )"))
                            (Utilities|Array|Add (LocalVariables|GetTextLength) (Utilities|String|Len (Utilities|String|Append "Sort: " (Utilities|String|ToString(Integer) (Utilities|Array|FindItem (Variables|/Game/Blueprints/Core/Grid/BP_GridPathfinding.BP_GridPathfinding_C|GetDiscoveredTileIndexes (Variables|/Game/Blueprints/Core/Grid/BP_Grid.BP_Grid_C|GetGridPathfinding (Variables|Default|GetGrid))) Index)) "( " (Utilities|String|ToString(Integer) (Utilities|Array|Get(acopy) (Variables|/Game/Blueprints/Core/Grid/BP_GridPathfinding.BP_GridPathfinding_C|GetDiscoveredTileSortingCost (Variables|/Game/Blueprints/Core/Grid/BP_Grid.BP_Grid_C|GetGridPathfinding (Variables|Default|GetGrid))) (Utilities|Array|FindItem (Variables|/Game/Blueprints/Core/Grid/BP_GridPathfinding.BP_GridPathfinding_C|GetDiscoveredTileIndexes (Variables|/Game/Blueprints/Core/Grid/BP_Grid.BP_Grid_C|GetGridPathfinding (Variables|Default|GetGrid))) Index))) " )"))))))))))))
          (:then_1
            (if (> (Utilities|Array|Length (LocalVariables|GetText)) 0)
              (Rendering|Components|TextRender|SetText (Variables|/Script/Engine.TextRenderActor|GetTextRender (LocalVariables|GetTextRender)) (Utilities|Text|ToText(String) (Utilities|String|JoinStringArray (LocalVariables|GetText) " 
 ")))
              (Transformation|SetActorTransform (LocalVariables|GetTextRender) (Math|Transform|MakeTransform (+ (.location (.transform (LocalVariables|GetData))) "0.000000,0.000000,1.000000") "90.000000,180.000000,0.000000" (Math|Conversions|ToVector(Float) (/ (.y (Variables|/Game/Blueprints/Core/Grid/BP_Grid.BP_Grid_C|GetGrid%20Tile%20Size (Variables|Default|GetGrid))) (* (.MaxValue (Math|Integer|MaxOfIntArray (LocalVariables|GetTextLength))) 30)))))
              (else
                (CallFunction|FDestroyTextActor Index)))))
        (else
          (CallFunction|FDestroyTextActor Index :!label _label)))
      (else
        (goto _label)))))

(fn FSetShowTileText
  (params (bSetShowTileIndexes :type Boolean) (bSetShowCostToEnterTile :type Boolean) (bSetShowMinCostToTarget :type Boolean) (bSetShowCostFromStart :type Boolean) (bSetShowSortOrder :type Boolean))
  (Utilities|FlowControl|Sequence
    (:then_0
      (Variables|Default|SetbSetShowTileIndexes bSetShowTileIndexes)
      (Variables|Default|SetbSetShowCostToEnterTile bSetShowCostToEnterTile)
      (Variables|Default|SetbSetShowMinCostToTarget bSetShowMinCostToTarget)
      (Variables|Default|SetbSetShowCostFromStart bSetShowCostFromStart)
      (Variables|Default|SetbSetShowSortOrder bSetShowSortOrder))
    (:then_1
      (CallFunction|FUpdatetextonAllTiles))))

(fn FUpdatetextonAllTiles
  (if (CallFunction|FWanttoDisplayAnyText)
    (bind _grid (Variables|Default|GetGrid)
      (:then
        (bind _keys (Utilities|Map|Keys (Variables|/Game/Blueprints/Core/Grid/BP_Grid.BP_Grid_C|GetGridTiles _grid)))
        (for _array_element _keys
          (CallFunction|FUpdateTextonTile _array_element)))
      (:else))
    (else
      (CallFunction|FClearAllTextActors))))

(fn FWanttoDisplayAnyText
  (return (Math|Boolean|ORBoolean (Variables|Default|GetbSetShowTileIndexes) (Variables|Default|GetbSetShowCostToEnterTile) (Variables|Default|GetbSetShowMinCostToTarget) (Variables|Default|GetbSetShowCostFromStart) (Variables|Default|GetbSetShowSortOrder))))