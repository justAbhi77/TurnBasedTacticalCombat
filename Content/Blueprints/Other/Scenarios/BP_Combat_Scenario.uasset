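; Combat scenario actor that quick-starts a battle from placed units on BeginPlay and opens the main menu when its combat ends.
; Outside gameplay, its construction script previews the grid at the actor's location and maps each unit to the tile beneath it.
; Separate helpers, not called within this Blueprint, build teams from unit display names and assign all teams except the first to AI.
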(event Custom|eOnCombatEnded
  (if (== (Variables|/Game/Blueprints/Core/Combat/BP_CombatSystem.BP_CombatSystem_C|GetObjectThatStartedCombat (Variables|Public|GetCombatSystem)) self)
    (Game|OpenLevel(byName) "L_MainMenu")))

(event EventBeginPlay
  (Utilities|FlowControl|Delay 0.05)
  (EventDispatchers|AssignOnCombatEnded (Variables|Public|GetCombatSystem) (delegate Custom|eOnCombatEnded))
  (Default|FQuickStartCombat (Variables|Public|GetCombatSystem) (Variables|Public|GetGridData) (Variables|Public|GetUnitsData) self))

(fn ConstructionScript
  (if (not (CallFunction|FIsinGame))
    (Utilities|Struct|SetmembersinStruct_QuickCombat_Grid (Variables|Public|GetGridData) (Transformation|GetActorLocation))
    (CallFunction|FSpawnGrid)
    (Public|FBuildDesiredGridIndexesBasedonUnitLocaations)))

(fn FBuildTeamsBasedonName
  (bind _outactors (Actor|GetAllActorsOfClass "/Game/Blueprints/Core/Units/BP_Unit.BP_Unit_C"))
  (for _array_element _outactors
    (LocalVariables|SetUnit _array_element)
    (LocalVariables|SetTeamIndex (Math|Conversions|ToInteger(Byte) (.LeftS (Utilities|String|Split (.RightS (Utilities|String|Split (Utilities|GetDisplayName (LocalVariables|GetUnit)) "Team")) "_"))))
    (Utilities|FlowControl|Sequence
      (:then_0
        (if (< (Utilities|Array|Length (LocalVariables|GetUnitsTeams)) (+ (LocalVariables|GetTeamIndex) 1))
          (Utilities|Array|Resize (LocalVariables|GetUnitsTeams) (+ (LocalVariables|GetTeamIndex) 1))))
      (:then_1
        (Utilities|Array|Add (Utilities|Struct|BreakStruct_UnitArray (Utilities|Array|Get(acopy) (LocalVariables|GetUnitsTeams) (LocalVariables|GetTeamIndex))) (LocalVariables|GetUnit)))))
  (Utilities|Array|RemoveItem :TargetArray (LocalVariables|GetUnitsTeams)) ; Remove Empty Groups
  (Utilities|Struct|SetmembersinStruct_QuickCombat_UnitTeams (Variables|Public|GetUnitsData) (LocalVariables|GetUnitsTeams)))

(fn FBuildAiListBasedonTeamIndexes
  (for (_array_element _array_index) (Utilities|Struct|BreakStruct_QuickCombat_UnitTeams (Variables|Public|GetUnitsData))
    (if (!= _array_index 0)
      (Utilities|Array|AppendArray (LocalVariables|GetAis) (Utilities|Struct|BreakStruct_UnitArray _array_element))))
  (Utilities|Struct|SetmembersinStruct_QuickCombat_UnitTeams (Variables|Public|GetUnitsData) (LocalVariables|GetAis)))

(fn FBuildDesiredGridIndexesBasedonUnitLocaations
  (for _array_element (Utilities|Struct|BreakStruct_QuickCombat_UnitTeams (Variables|Public|GetUnitsData))
    (for _array_element_2 (Utilities|Struct|BreakStruct_UnitArray _array_element)
      (bind _index (Default|FGetTileIndexfromWorldLocation (Variables|/Game/Blueprints/Core/Combat/BP_CombatSystem.BP_CombatSystem_C|GetGrid (Variables|Public|GetCombatSystem)) (Transformation|GetActorLocation _array_element_2)))
      (Utilities|Map|Add (LocalVariables|GetDesiredIndexes) _array_element_2 _index)))
  (Utilities|Struct|SetmembersinStruct_QuickCombat_UnitTeams (Variables|Public|GetUnitsData) (LocalVariables|GetDesiredIndexes)))

(fn FSpawnGrid
  (bind _griddata (Variables|Public|GetGridData))
  (bind (_bgenerategridbeforestartingcombat _centerlocation _tilesize _tilecount _shape _buseenvironment) (Utilities|Struct|BreakStruct_QuickCombat_Grid _griddata))
  (bind _combatsystem (Variables|Public|GetCombatSystem)
    (:then
      (bind _grid (Variables|/Game/Blueprints/Core/Combat/BP_CombatSystem.BP_CombatSystem_C|GetGrid _combatsystem)
        (:then
          (Default|FSpawnGrid _grid _centerlocation _tilesize _tilecount _shape _buseenvironment false))
        (:else)))
    (:else)))

(fn FRestartCombat
  (for _array_element (Utilities|Struct|BreakStruct_QuickCombat_UnitTeams (Variables|Public|GetUnitsData))
    (for _array_element_2 (Utilities|Struct|BreakStruct_UnitArray _array_element)
      (Default|FResetHp _array_element_2)))
  (Default|FQuickStartCombat (Variables|Public|GetCombatSystem) (Variables|Public|GetGridData) (Variables|Public|GetUnitsData) self))