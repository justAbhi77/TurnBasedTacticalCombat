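; BP_Overworld_Scenario sets up an overworld scenario, showing the back-to-main-menu widget and registering the unit groups at BeginPlay.
; FBuildUnitGroupsBasedOnName fills the UnitGroups map by parsing BP_Unit display names for a "Grp" ID, flagging groups with an "_Ai" unit as encounters.
; After a short delay, BeginPlay sets each mapped unit's context and passes units and encounter flags to OverworldUnitGroup.
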(event EventBeginPlay
  (Utilities|FlowControl|Sequence
    (:then_0
      (bind _returnvalue (UserInterface|CreateWidget "/Game/Blueprints/Other/MainMenu/WBP_BackToMainMenu.WBP_BackToMainMenu_C"))
      (UserInterface|Viewport|AddtoViewport _returnvalue 0))
    (:then_1
      (Utilities|FlowControl|Delay 0.1)
      (bind _values (Utilities|Map|Values (Variables|Default|GetUnitGroups)))
      (for _array_element _values
        (for _array_element_2 (.Units (Utilities|Struct|BreakStruct_OverworldUnitGroup _array_element))
          (Default|FSetUnitContext _array_element_2 "NewEnumerator1")
          (bind _overworldunitgroup (Variables|Default|GetOverworldUnitGroup)
            (:then
              (Default|FAddUnittoGroup _overworldunitgroup _array_element_2 (.GroupId (Utilities|Struct|BreakStruct_OverworldUnitGroup _array_element))))
            (:else)))
        (bind _overworldunitgroup_2 (Variables|Default|GetOverworldUnitGroup)
          (:then
            (Default|FSetGroupIsEncounter _overworldunitgroup_2 (.bIsEncounter (Utilities|Struct|BreakStruct_OverworldUnitGroup _array_element)) (.GroupId (Utilities|Struct|BreakStruct_OverworldUnitGroup _array_element))))
          (:else))))))

(fn ConstructionScript)

(fn FBuildUnitGroupsBasedonName
  (Utilities|Map|Clear (Variables|Default|GetUnitGroups))
  (bind _outactors (Actor|GetAllActorsOfClass "/Game/Blueprints/Core/Units/BP_Unit.BP_Unit_C"))
  (for _array_element _outactors
    (LocalVariables|SetUnit _array_element)
    (LocalVariables|SetGroupId (Math|Conversions|ToInteger(Byte) (.LeftS (Utilities|String|Split (.RightS (Utilities|String|Split (Utilities|GetDisplayName (LocalVariables|GetUnit)) "Grp")) "_"))))
    (LocalVariables|SetbIsEncounter (Utilities|String|Contains (Utilities|GetDisplayName (LocalVariables|GetUnit)) "_Ai"))
    (LocalVariables|SetGroup (.Value (Utilities|Map|Find (Variables|Default|GetUnitGroups) (LocalVariables|GetGroupId))))
    (Utilities|Struct|SetmembersinStruct_OverworldUnitGroup (LocalVariables|GetGroup) (LocalVariables|GetGroupId) (or (LocalVariables|GetbIsEncounter) (Utilities|Struct|BreakStruct_OverworldUnitGroup (LocalVariables|GetGroup))))
    (Utilities|Array|AddUnique (Utilities|Struct|BreakStruct_OverworldUnitGroup (LocalVariables|GetGroup)) (LocalVariables|GetUnit))
    (Utilities|Map|Add (Variables|Default|GetUnitGroups) (LocalVariables|GetGroupId) (LocalVariables|GetGroup))))