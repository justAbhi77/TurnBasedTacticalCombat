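; Main menu Blueprint that displays the WBP_MainMenu widget and endlessly cycles streamed levels while it runs.
; On BeginPlay it creates the widget, then loops through the Hexagon, Square and Triangle levels via the MLoadUnloadLevel macro.
; The macro stream-loads a level without blocking, shows and hides the widget's background around a fixed delay, waits a given duration, then unloads the level.
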(event EventBeginPlay
  (bind _returnvalue (UserInterface|CreateWidget "/Game/Blueprints/Other/MainMenu/WBP_MainMenu.WBP_MainMenu_C"))
  (bind _output_get (Variables|Default|SetAsWBPMainMenu _returnvalue))
  (UserInterface|Viewport|AddtoViewport _output_get 0)
  (Utilities|MLoadUnloadLevel "L_Hexagon" 5.0 :!label _label
    (:Completed
      (Utilities|MLoadUnloadLevel "L_Square" 5.0
        (:Completed
          (Utilities|MLoadUnloadLevel "L_Triangle" 5.0
            (:Completed
              (goto _label))))))))

(fn ConstructionScript)