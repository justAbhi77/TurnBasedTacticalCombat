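; Combat manager for a grid-based, turn-based tactics game, handling units, teams, turns and spells.
; It keeps unit occupancy synced with grid tiles, removing units left on invalid tiles, and cycles turns through living units, triggering optional AI actors.
; Spells derive range and AoE from patterns, filtered by walkability and optional multi-trace line of sight.
; Movement spends MP by path cost; deaths trigger combat finishing when one team survives.
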(event EventBeginPlay
  (bind _grid (Variables|Public|GetGrid)
    (:then
      (EventDispatchers|BindEventtoOnGridGenerated _grid (EventDispatchers|CreateEvent :!event FonGridGenerated))
      (EventDispatchers|BindEventtoOnTileDataUpdated _grid (EventDispatchers|CreateEvent :!event FonTileDataUpdated)))
    (:else)))

(fn ConstructionScript)

(fn FAddUnitinCombat
  (params (Unit :type BP%20Unit%20Object%20Reference) (Index :type Int%20Point%20Structure) (TeamIndex :type Integer) (bUseAi :type Boolean))
  (Utilities|Array|Add (Variables|Default|GetUnitsInCombat) Unit)
  (Default|FSetGrid Unit (Variables|Public|GetGrid))
  (CallFunction|FSetUnitIndexonGrid Unit Index false true)
  (EventDispatchers|BindEventtoOnUnitReachedNewTile Unit (EventDispatchers|CreateEvent :!event FonUnitReachedNewTile))
  (CallFunction|FSetUnitTeamIndex Unit TeamIndex)
  (CallFunction|FSetUnitUseAi Unit bUseAi))

(fn FRemoveUnitfromCombat
  (params (Unit :type BP%20Unit%20Object%20Reference) (bDestroyUnit :type Boolean))
  (Utilities|Array|RemoveItem (Variables|Default|GetUnitsInCombat) Unit)
  (CallFunction|FSetUnitIndexonGrid Unit (Utilities|Struct|MakeIntPoint -999 -999) false true)
  (CallFunction|FSetUnitTeamIndex Unit -1)
  (if bDestroyUnit
    (Actor|DestroyActor Unit)))

(fn FSetUnitIndexonGrid
  (params (Unit :type BP%20Unit%20Object%20Reference) (Index :type Int%20Point%20Structure) (bForce :type Boolean) (bSnapLocation :type Boolean))
  (bind _grid (Variables|Public|GetGrid))
  (bind _gridtiles (Variables|/Game/Blueprints/Core/Grid/BP_Grid.BP_Grid_C|GetGridTiles _grid))
  (bind (_value _returnvalue) (Utilities|Map|Find _gridtiles Index))
  (Utilities|FlowControl|Sequence
    (:then_0
      (if (or (!= (Variables|/Game/Blueprints/Core/Units/BP_Unit.BP_Unit_C|GetIndex Unit) Index) bForce)
        (Utilities|FlowControl|Sequence
          (:then_0
            (bind _output_get (LocalVariables|SetPreviousTile (.Value (Utilities|Map|Find (Variables|/Game/Blueprints/Core/Grid/BP_Grid.BP_Grid_C|GetGridTiles (Variables|Public|GetGrid)) (Variables|/Game/Blueprints/Core/Units/BP_Unit.BP_Unit_C|GetIndex Unit)))))
            (if (== (.UnitOnTile (Utilities|Struct|BreakStruct_TileData _output_get)) Unit)
              (bind _structout (Utilities|Struct|SetmembersinStruct_TileData (LocalVariables|GetPreviousTile)))
              (Utilities|Map|Add (Variables|/Game/Blueprints/Core/Grid/BP_Grid.BP_Grid_C|GetGridTiles (Variables|Public|GetGrid)) (.Index (Utilities|Struct|BreakStruct_TileData _structout)) _structout)))
          (:then_1
            (Default|FSetGridIndex Unit Index)
            (if (!= Index (Utilities|Struct|MakeIntPoint -999 -999))
              (bind _structout_2 (Utilities|Struct|SetmembersinStruct_TileData (.Value (Utilities|Map|Find (Variables|/Game/Blueprints/Core/Grid/BP_Grid.BP_Grid_C|GetGridTiles (Variables|Public|GetGrid)) Index)) Unit))
              (Utilities|Map|Add (Variables|/Game/Blueprints/Core/Grid/BP_Grid.BP_Grid_C|GetGridTiles (Variables|Public|GetGrid)) (.Index (Utilities|Struct|BreakStruct_TileData _structout_2)) _structout_2)))
          (:then_2
            (Default|CallOnUnitGridIndexChanged Unit)))))
    (:then_1
      (if bSnapLocation
        (Transformation|SetActorLocation Unit (select _returnvalue (.location (.Transform (Utilities|Struct|BreakStruct_TileData _value))) "-99999.000000,-99999.000000,-99999.000000") false false)))))

(fn FonGridGenerated
  (bind _output_get (LocalVariables|SetCopyOfUnitsInCombat (Variables|Default|GetUnitsInCombat))) ; Copy because we affect the list \nwhile looping through it\nthe loop breaks
  (for _array_element _output_get
    (if (Utilities|Array|ContainsItem (.ValidTileTypes (Utilities|Struct|BreakStruct_UnitData_Stats (.Stats (Utilities|Struct|BreakStruct_UnitData (Variables|/Game/Blueprints/Core/Units/BP_Unit.BP_Unit_C|GetUnitData _array_element))))) (.tiletype (.Value (Utilities|Map|Find (Variables|/Game/Blueprints/Core/Grid/BP_Grid.BP_Grid_C|GetGridTiles (Variables|Public|GetGrid)) (Variables|/Game/Blueprints/Core/Units/BP_Unit.BP_Unit_C|GetIndex _array_element)))))
      (CallFunction|FSetUnitIndexonGrid _array_element (Variables|/Game/Blueprints/Core/Units/BP_Unit.BP_Unit_C|GetIndex _array_element) true true)
      (else
        (CallFunction|FRemoveUnitfromCombat _array_element true)))))

(fn FonTileDataUpdated
  (params (Index :type Int%20Point%20Structure))
  (bind _output_get (LocalVariables|SetCopyOfUnitsInCombat (Variables|Default|GetUnitsInCombat))) ; Copy because we affect the list \nwhile looping through it\nthe loop breaks
  (bind _array_element (Utilities|Array|ForEachLoopwithBreak _output_get :!label _label)
    (:LoopBody
      (if (Class|KismetMathLibrary|EqualIntPointIntPoint Index (Variables|/Game/Blueprints/Core/Units/BP_Unit.BP_Unit_C|GetIndex _array_element))
        (Utilities|FlowControl|Sequence
          (:then_0
            (if (Utilities|Array|ContainsItem (.ValidTileTypes (Utilities|Struct|BreakStruct_UnitData_Stats (.Stats (Utilities|Struct|BreakStruct_UnitData (Variables|/Game/Blueprints/Core/Units/BP_Unit.BP_Unit_C|GetUnitData _array_element))))) (.tiletype (.Value (Utilities|Map|Find (Variables|/Game/Blueprints/Core/Grid/BP_Grid.BP_Grid_C|GetGridTiles (Variables|Public|GetGrid)) (Variables|/Game/Blueprints/Core/Units/BP_Unit.BP_Unit_C|GetIndex _array_element)))))
              (CallFunction|FSetUnitIndexonGrid _array_element (Variables|/Game/Blueprints/Core/Units/BP_Unit.BP_Unit_C|GetIndex _array_element) false true)
              (else
                (CallFunction|FRemoveUnitfromCombat _array_element true))))
          (:then_1
            (goto _label Break)))))))

(fn FonUnitReachedNewTile
  (params (Unit :type BP%20Unit%20Object%20Reference) (Index :type Int%20Point%20Structure))
  (Default|FSpawnAnimatedNumber Unit (- 0 (CallFunction|FGetTileTypeCost (Utilities|Struct|BreakStruct_TileData (.Value (Utilities|Map|Find (Variables|/Game/Blueprints/Core/Grid/BP_Grid.BP_Grid_C|GetGridTiles (Variables|Public|GetGrid)) Index))))) "NewEnumerator1"))

(fn FCastSpell
  (params (Spell :type E_Spells%20Enum :default "NewEnumerator0") (OriginIndex :type Int%20Point%20Structure) (TargetIndex :type Int%20Point%20Structure))
  (bind _grid (Variables|Public|GetGrid))
  (bind _grid_2 (Variables|Public|GetGrid))
  (bind _gridtiles (Variables|/Game/Blueprints/Core/Grid/BP_Grid.BP_Grid_C|GetGridTiles _grid))
  (bind _gridtiles_2 (Variables|/Game/Blueprints/Core/Grid/BP_Grid.BP_Grid_C|GetGridTiles _grid_2))
  (bind _value (Utilities|Map|Find _gridtiles OriginIndex))
  (bind _value_2 (Utilities|Map|Find _gridtiles_2 OriginIndex))
  (bind _unitontile (Utilities|Struct|BreakStruct_TileData _value_2))
  (bind _unitontile_2 (Utilities|Struct|BreakStruct_TileData _value))
  (bind _spelldata (CallFunction|FGetSpellDatafromSpell Spell))
  (LocalVariables|SetData _spelldata)
  (Utilities|IsValid _unitontile
    (:Is%20Valid
      (bind _bcancastspell (Default|FCanCastSpell _unitontile (LocalVariables|GetData)))
      (if _bcancastspell
        (bind _rangesindexes (CallFunction|FGetSpellRange OriginIndex (.cast (LocalVariables|GetData)) :!label _label))
        (if (Utilities|Array|ContainsItem _rangesindexes TargetIndex)
          (Utilities|FlowControl|Sequence
            (:then_0
              (bind _attackedindices (CallFunction|FGetAttackedIndices (LocalVariables|GetData) TargetIndex))
              (LocalVariables|SetAttackIndexes _attackedindices))
            (:then_1
              (bind _returnvalue (Game|SpawnActorfromClass (.Animation (Utilities|Struct|BreakStruct_SpellData_Assets (.assets (LocalVariables|GetData)))) (Math|Transform|MakeTransform "0, 0, 0" "0, 0, 0" "1.000000,1.000000,1.000000") "AlwaysSpawn" "MultiplyWithRoot" 0 (Variables|Public|GetGrid) OriginIndex TargetIndex (LocalVariables|GetAttackIndexes) 0))
              (LocalVariables|SetSpellAnimation _returnvalue)
              (Utilities|FlowControl|Sequence
                (:then_0
                  (Utilities|IsValid _unitontile_2
                    (:Is%20Valid
                      (Default|FUnitCastSpell _unitontile_2 TargetIndex (LocalVariables|GetData)))))
                (:then_1
                  (LocalVariables|SetSpellImpactReal (Utilities|Struct|MakeStruct_SpellData_Impact_Real (CallFunction|FMinMaxRandom (.MinMaxModifier_Hp (Utilities|Struct|BreakStruct_SpellData_Impact (Utilities|Struct|BreakStruct_SpellData (LocalVariables|GetData))))) (CallFunction|FMinMaxRandom (.MinMaxModifier_Mp (Utilities|Struct|BreakStruct_SpellData_Impact (Utilities|Struct|BreakStruct_SpellData (LocalVariables|GetData))))) (CallFunction|FMinMaxRandom (.MinMaxModifier_Ap (Utilities|Struct|BreakStruct_SpellData_Impact (Utilities|Struct|BreakStruct_SpellData (LocalVariables|GetData)))))))
                  (for _array_element (LocalVariables|GetAttackIndexes)
                    (bind _output_get (LocalVariables|SetUnit (Utilities|Struct|BreakStruct_TileData (.Value (Utilities|Map|Find (Variables|/Game/Blueprints/Core/Grid/BP_Grid.BP_Grid_C|GetGridTiles (Variables|Public|GetGrid)) _array_element)))))
                    (Utilities|IsValid _output_get
                      (:Is%20Valid
                        (if (Default|FIsAlive (LocalVariables|GetUnit))
                          (Default|FUnitHitbySpell (LocalVariables|GetUnit) (LocalVariables|GetSpellImpactReal) (LocalVariables|GetSpellAnimation))
                          (if (not (Default|FIsAlive (LocalVariables|GetUnit)))
                            (CallFunction|FProcessUnitDeath (LocalVariables|GetUnit))
                            (if (Variables|Default|GetbIsFinishingCombat)
                              (return)))))))
                  (bind _currentunit (Variables|Default|GetCurrentUnit)
                    (:then
                      (if (not (Default|FIsAlive _currentunit))
                        (CallFunction|FNextUnit)))
                    (:else)))))))))
    (:Is%20Not%20Valid
      (goto _label))))

(fn FGetSpellRange
  (params (OriginIndex :type Int%20Point%20Structure) (Cast :type Struct%20Spell%20Data%20Cast%20Structure))
  (bind (_rangepattern _rangeminmax _lineofsight) (Utilities|Struct|BreakStruct_SpellData_Cast Cast))
  (bind _rangeindexes (CallFunction|FGetIndexesfromPatternandRange OriginIndex (Variables|/Game/Blueprints/Core/Grid/BP_Grid.BP_Grid_C|GetGrid%20Shape (Variables|Public|GetGrid)) _rangepattern _rangeminmax))
  (bind _notwalkableindexes (CallFunction|FRemoveNotWalkableIndexes _rangeindexes))
  (if (.bRequireLineOfSight (Utilities|Struct|BreakStruct_SpellData_LineOfSight _lineofsight))
    (bind _indexeswithlineofsight (CallFunction|FRemoveIndexesWithoutLineOfSight OriginIndex _notwalkableindexes Cast))
    (return _indexeswithlineofsight)
    (else
      (return _notwalkableindexes))))

(fn FHasLineOfSight
  (params (OriginIndex :type Int%20Point%20Structure) (TargetIndex :type Int%20Point%20Structure) (Cast :type Struct%20Spell%20Data%20Cast%20Structure))
  (bind _grid (Variables|Public|GetGrid))
  (bind _grid_2 (Variables|Public|GetGrid))
  (bind _lineofsight (Utilities|Struct|BreakStruct_SpellData_Cast Cast))
  (bind _lineofsight_2 (Utilities|Struct|BreakStruct_SpellData_Cast Cast))
  (bind _gridtiles (Variables|/Game/Blueprints/Core/Grid/BP_Grid.BP_Grid_C|GetGridTiles _grid))
  (bind _grid_tile_size (Variables|/Game/Blueprints/Core/Grid/BP_Grid.BP_Grid_C|GetGrid%20Tile%20Size _grid_2))
  (bind _offsetfromcenter (Utilities|Struct|BreakStruct_SpellData_LineOfSight _lineofsight_2))
  (bind _heightfromground (Utilities|Struct|BreakStruct_SpellData_LineOfSight _lineofsight))
  (bind _returnvalue (Math|Vector|MakeVector 0.0 0.0 _heightfromground))
  (bind _returnvalue_2 (* _grid_tile_size _offsetfromcenter))
  (LocalVariables|SetOriginTile (.Value (Utilities|Map|Find _gridtiles OriginIndex)))
  (LocalVariables|SetTargetTile (.Value (Utilities|Map|Find _gridtiles TargetIndex)))
  (LocalVariables|SetStart (+ (.location (.Transform (Utilities|Struct|BreakStruct_TileData (LocalVariables|GetOriginTile)))) _returnvalue))
  (LocalVariables|SetEnd (+ _returnvalue (.location (.Transform (Utilities|Struct|BreakStruct_TileData (LocalVariables|GetTargetTile))))))
  (for _array_element (Utilities|Array|MakeArray (Math|Vector2D|MakeVector2D (.x _returnvalue_2) 0.0) (Math|Vector2D|MakeVector2D (- 0.0 (.x _returnvalue_2)) 0.0) (Math|Vector2D|MakeVector2D 0.0 (.y _returnvalue_2)) (Math|Vector2D|MakeVector2D 0.0 (- 0.0 (.y _returnvalue_2))))
    (bind _returnvalue_3 (Collision|LineTraceByChannel (+ (LocalVariables|GetStart) (Math|Conversions|ToVector(Vector2D) _array_element)) (LocalVariables|GetEnd) "TraceTypeQuery6" false (Utilities|Array|MakeArray (Utilities|Struct|BreakStruct_TileData (LocalVariables|GetOriginTile)) (Utilities|Struct|BreakStruct_TileData (LocalVariables|GetTargetTile))) (select (.DrawDebugLine (Utilities|Struct|BreakStruct_SpellData_LineOfSight (.LineOfSight (Utilities|Struct|BreakStruct_SpellData_Cast Cast)))) "ForDuration" "None")))
    (if (not _returnvalue_3)
      (return true)))
  (return false))

(fn FRemoveIndexesWithoutLineOfSight
  (params (OriginIndex :type Int%20Point%20Structure) (Indexes :type Array%20of%20Int%20Point%20Structures) (Cast :type Struct%20Spell%20Data%20Cast%20Structure))
  (for _array_element Indexes
    (if (CallFunction|FHasLineOfSight OriginIndex _array_element Cast)
      (Utilities|Array|Add (LocalVariables|GetRet) _array_element)))
  (return (LocalVariables|GetRet)))

(fn FRemoveNotWalkableIndexes
  (params (Indexes :type Array%20of%20Int%20Point%20Structures))
  (for _array_element Indexes
    (if (Default|FIsTileWalkable (Variables|Public|GetGrid) _array_element)
      (Utilities|Array|Add (LocalVariables|GetRet) _array_element)))
  (return (LocalVariables|GetRet)))

(fn FSetUnitTeamIndex
  (params (Unit :type BP%20Unit%20Object%20Reference) (TeamIndex :type Integer))
  (Utilities|FlowControl|Sequence
    (:then_0
      (if (!= (Variables|/Game/Blueprints/Core/Units/BP_Unit.BP_Unit_C|GetTeamIndex Unit) -1)
        (bind _output_get (LocalVariables|SetUnitSet (.unitset (.Value (Utilities|Map|Find (Variables|Default|GetUnitTeams) (Variables|/Game/Blueprints/Core/Units/BP_Unit.BP_Unit_C|GetTeamIndex Unit))))))
        (Utilities|Set|Remove _output_get Unit)
        (if (> (Utilities|Set|Length (LocalVariables|GetUnitSet)) 0)
          (Utilities|Map|Add (Variables|Default|GetUnitTeams) (Variables|/Game/Blueprints/Core/Units/BP_Unit.BP_Unit_C|GetTeamIndex Unit) (Utilities|Struct|MakeStruct_UnitSet (LocalVariables|GetUnitSet)))
          (else
            (Utilities|Map|Remove (Variables|Default|GetUnitTeams) (Variables|/Game/Blueprints/Core/Units/BP_Unit.BP_Unit_C|GetTeamIndex Unit))))))
    (:then_1
      (if (!= TeamIndex -1)
        (bind _output_get_2 (LocalVariables|SetUnitSet (.unitset (.Value (Utilities|Map|Find (Variables|Default|GetUnitTeams) TeamIndex)))))
        (Utilities|Set|Add _output_get_2 Unit)
        (Utilities|Map|Add (Variables|Default|GetUnitTeams) TeamIndex (Utilities|Struct|MakeStruct_UnitSet (LocalVariables|GetUnitSet)))))
    (:then_2
      (Default|FSetTeamIndex Unit TeamIndex)
      (Default|CallOnUnitTeamsChanged))))

(fn FCanStartCombat
  (bind _unitsincombat (Variables|Default|GetUnitsInCombat))
  (bind _unitteams (Variables|Default|GetUnitTeams))
  (bind _bisincombat (Variables|Default|GetbIsInCombat))
  (bind _returnvalue (Utilities|Array|Length _unitsincombat))
  (bind _returnvalue_2 (Utilities|Map|Length _unitteams))
  (bind _returnvalue_3 (not _bisincombat))
  (bind _returnvalue_4 (>= _returnvalue_2 2))
  (bind _returnvalue_5 (>= _returnvalue 2))
  (return (Math|Boolean|ANDBoolean _returnvalue_5 _returnvalue_4 _returnvalue_3) _returnvalue_5 _returnvalue_4 _returnvalue_3))

(fn FStartCombat
  (Variables|Default|SetbIsInCombat true)
  (for _array_element (Variables|Default|GetUnitsInCombat)
    (Default|FCombatStarted _array_element)
    (bind _ai (Variables|/Game/Blueprints/Core/Units/BP_Unit.BP_Unit_C|GetAi _array_element)
      (:then
        (Default|FAiCombatStarted _ai))
      (:else)))
  (Default|CallOnCombatStarted)
  (Variables|Default|SetCurrentUnit 0)
  (CallFunction|FNextUnit))

(fn FEndCombat
  (Variables|Default|SetbIsInCombat false)
  (Variables|Default|SetbIsFinishingCombat false)
  (for _array_element (Variables|Default|GetUnitsInCombat)
    (Default|FCombatEnded _array_element)
    (bind _ai (Variables|/Game/Blueprints/Core/Units/BP_Unit.BP_Unit_C|GetAi _array_element)
      (:then
        (Default|FAiCombatEnded _ai))
      (:else)))
  (Default|CallOnCombatEnded))

(fn FNextUnit
  (Utilities|FlowControl|Sequence
    (:then_0
      (bind _currentunit (Variables|Default|GetCurrentUnit)
        (:then
          (Default|FTurnEnded _currentunit)
          (Default|CallOnUnitTurnEnded _currentunit))
        (:else)))
    (:then_1
      (LocalVariables|SetCurrentIndex (Utilities|Array|FindItem (Variables|Default|GetUnitsInCombat) (Variables|Default|GetCurrentUnit)))
      (while (not (Utilities|IsValid (LocalVariables|GetNextLivingUnit)))
        (LocalVariables|SetCurrentIndex (Math|Integer|%(Integer) (+ (LocalVariables|GetCurrentIndex) 1) (Utilities|Array|Length (Variables|Default|GetUnitsInCombat))))
        (if (Default|FIsAlive (Utilities|Array|Get(acopy) (Variables|Default|GetUnitsInCombat) (LocalVariables|GetCurrentIndex)))
          (LocalVariables|SetNextLivingUnit (Utilities|Array|Get(acopy) (Variables|Default|GetUnitsInCombat) (LocalVariables|GetCurrentIndex)))))
      (bind _output_get (Variables|Default|SetCurrentUnit (LocalVariables|GetNextLivingUnit)))
      (Default|FTurnStarted _output_get)
      (Default|CallOnUnitTurnStarted _output_get)
      (bind _ai (Variables|/Game/Blueprints/Core/Units/BP_Unit.BP_Unit_C|GetAi (Variables|Default|GetCurrentUnit))
        (:then
          (Default|FAiPlayTurn _ai))
        (:else)))))

(fn FMoveUnit
  (params (Unit :type BP%20Unit%20Object%20Reference) (Path :type Array%20of%20Int%20Point%20Structures))
  (if (> (Utilities|Array|Length Path) 0)
    (Default|EFollowPath Unit Path)
    (bind _cost (Default|FGetPathCost (Variables|/Game/Blueprints/Core/Grid/BP_Grid.BP_Grid_C|GetGridPathfinding (Variables|Public|GetGrid)) Path))
    (Default|FModifyCurrentMp Unit (- 0 _cost) false)
    (CallFunction|FSetUnitIndexonGrid Unit (Utilities|Array|Get(acopy) Path (Utilities|Array|LastIndex Path)) false false)))

(fn FProcessUnitDeath
  (params (Unit :type BP%20Unit%20Object%20Reference))
  (if (Variables|Default|GetbIsInCombat)
    (Variables|/Game/Blueprints/Core/Units/BP_Unit.BP_Unit_C|SetIndexToRememberForSpellImpact Unit (Variables|/Game/Blueprints/Core/Units/BP_Unit.BP_Unit_C|GetIndex Unit))
    (CallFunction|FSetUnitIndexonGrid Unit (Utilities|Struct|MakeIntPoint -999 -999) false false)
    (Default|EHideUnitAfterFewSeconds Unit)
    (bind _keys (Utilities|Map|Keys (Variables|Default|GetUnitTeams)))
    (for _array_element _keys
      (bind _output_get (LocalVariables|SetTeamIndex _array_element))
      (bind _result (Utilities|Set|ToArray (Utilities|Struct|BreakStruct_UnitSet (.Value (Utilities|Map|Find (Variables|Default|GetUnitTeams) _output_get)))))
      (bind _array_element_2 (Utilities|Array|ForEachLoopwithBreak _result :!label _label)
        (:LoopBody
          (if (Default|FIsAlive _array_element_2)
            (Utilities|Array|Add (LocalVariables|GetTeamsWithAliveUnit) (LocalVariables|GetTeamIndex))
            (goto _label Break)))))
    (if (== 1 (Utilities|Array|Length (LocalVariables|GetTeamsWithAliveUnit)))
      (CallFunction|FFinishCombat (Utilities|Array|Get(acopy) (LocalVariables|GetTeamsWithAliveUnit))))
    (else
      (Default|EDebugRespawnAfterFewSeconds Unit))))

(fn FFinishCombat
  (params (WinningTeamIndex :type Integer))
  (Variables|Default|SetbIsFinishingCombat true)
  (Utilities|FlowControl|Sequence
    (:then_0
      (bind _currentunit (Variables|Default|GetCurrentUnit)
        (:then
          (Default|FSetIsActiveinCombat _currentunit false)
          (Variables|Default|SetCurrentUnit 0))
        (:else)))
    (:then_1
      (Default|CallOnCombatFinishing WinningTeamIndex))))

(fn FSetUnitUseAi
  (params (Unit :type BP%20Unit%20Object%20Reference) (bUseAi :type Boolean))
  (bind _ai (Variables|/Game/Blueprints/Core/Units/BP_Unit.BP_Unit_C|GetAi Unit))
  (if bUseAi
    (Utilities|IsValid (Variables|/Game/Blueprints/Core/Units/BP_Unit.BP_Unit_C|GetAi Unit)
      (:Is%20Not%20Valid
        (bind _returnvalue (Game|SpawnActorfromClass (Utilities|Struct|BreakStruct_UnitData_Ai (Utilities|Struct|BreakStruct_UnitData (Variables|/Game/Blueprints/Core/Units/BP_Unit.BP_Unit_C|GetUnitData Unit))) (Math|Transform|MakeTransform "0, 0, 0" "0, 0, 0" "1.000000,1.000000,1.000000") "Undefined" "MultiplyWithRoot" 0 self Unit 0))
        (Default|FSetUnitAi Unit _returnvalue)))
    (else
      (Utilities|IsValid _ai
        (:Is%20Valid
          (Actor|DestroyActor _ai)
          (Default|FSetUnitAi Unit))))))

(fn FGetAttackedIndices
  (params (SpellData :type Struct%20Spell%20Data%20Structure%20%28by%20ref%29) (TargetIndex :type Int%20Point%20Structure))
  (if (Utilities|Enum|Equal(Enum) (Utilities|Struct|BreakStruct_SpellData_Cast (Utilities|Struct|BreakStruct_SpellData SpellData)) "NewEnumerator0")
    (return (Utilities|Array|MakeArray TargetIndex))
    (else
      (bind _rangesindexes (CallFunction|FGetSpellRange TargetIndex (Utilities|Struct|BreakStruct_SpellData SpellData)))
      (return _rangesindexes))))