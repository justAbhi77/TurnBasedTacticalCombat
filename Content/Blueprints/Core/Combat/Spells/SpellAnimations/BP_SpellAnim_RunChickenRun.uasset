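; BP_SpellAnim_RunChickenRun is the visual animation actor for the Run Chicken Run spell.
; When played, it moves to the target tile and sets the spell's background-free icon on its image widget.
; A timeline then drives the widget's height, draw size and opacity, and signals spell animation completion when it finishes.
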(event EventEPlaySpellAnimation
  (Transformation|SetActorLocation (.location (CallFunction|FGetTileTransform (Variables|Default|GetTargetIndex))) false false)
  (bind _output_get (Variables|Default|SetWBPImage (.AsWBP%20Image (Utilities|Casting|CastToWBP_Image (UserInterface|GetUserWidgetObject (Variables|Default|GetWidget))))))
  (Appearance|SetBrushfromTexture (Variables|/Game/Blueprints/Core/Combat/Spells/SpellAnimations/Components/WBP_Image.WBP_Image_C|GetImage_Comp _output_get) "/Game/Blueprints/Core/Combat/Spells/SpellAnimations/Assests/Icon_RunChickenRun_NoBackground.Icon_RunChickenRun_NoBackground" false)
  (bind (_direction _locationz _drawsize _opacity) (Timeline|Timeline PlayFromStart)
    (:Update
      (Transformation|SetRelativeLocation (Variables|Default|GetWidget) (Math|Vector|MakeVector 0.0 0.0 _locationz) false false)
      (Class|WidgetComponent|SetDrawSize (Variables|Default|GetWidget) (Math|Vector2D|MakeVector2D _drawsize _drawsize))
      (Widget|SetRenderOpacity (Variables|Default|GetWBPImage) _opacity))
    (:Finished
      (CallFunction|ECompleteSpellAnimation))))

(fn ConstructionScript
  (|CallParentFunction))