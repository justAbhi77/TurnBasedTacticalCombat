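; Heal spell animation actor that plays a green visual effect on the target tile.
; On play it moves to the tile, then a timeline drives opacity on six meshes plus scale and yaw of a parent component.
; Partway through the timeline it signals the tile hit once, and it completes the spell animation when the timeline finishes.
; The construction script tints the meshes in three pairs of green shades.
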(event EventEPlaySpellAnimation
  (bind _anim_scale (Variables|Default|GetAnim_Scale))
  (Transformation|SetActorLocation (.location (CallFunction|FGetTileTransform (Variables|Default|GetTargetIndex))) false false)
  (bind (_direction _opacity _scale _rotation) (Timeline|Timeline PlayFromStart)
    (:Update
      (Rendering|Material|SetScalarParameterValueonMaterials (Variables|Default|GetStaticMesh) "Opacity" _opacity)
      (Transformation|SetRelativeScale3D _anim_scale _scale)
      (Transformation|SetRelativeRotation _anim_scale (Math|Rotator|MakeRotator 0.0 0.0 _rotation) false false)
      (if (> (Components|Timeline|GetPlaybackPosition (Variables|Default|GetTimeline)) 0.55)
        (Utilities|FlowControl|DoOnce false
          (:Completed
            (Default|CallOnSpellAnimationHitTile self (Variables|Default|GetTargetIndex))))))
    (:Finished
      (CallFunction|ECompleteSpellAnimation))))

(fn ConstructionScript
  (|CallParentFunction)
  (Utilities|FlowControl|Sequence
    (:then_0
      (Rendering|Material|SetVectorParameterValueonMaterials (Variables|Default|GetStaticMesh) "BaseColor" (Math|Conversions|ToVector(LinearColor) "(R=0.197389,G=1.000000,B=0.398042,A=1.000000)")))
    (:then_1
      (Rendering|Material|SetVectorParameterValueonMaterials (Variables|Default|GetStaticMesh1) "BaseColor" (Math|Conversions|ToVector(LinearColor) "(R=0.105882,G=1.000000,B=0.100000,A=1.000000)")))
    (:then_2
      (Rendering|Material|SetVectorParameterValueonMaterials (Variables|Default|GetStaticMesh2) "BaseColor" (Math|Conversions|ToVector(LinearColor) "(R=0.000000,G=0.895833,B=0.600000,A=1.000000)")))))