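; Spell animation actor that flies a short-range arrow from an origin tile to a target tile.
; On play, it snaps to the origin and faces the target using the grid indices as flat vectors.
; A timeline, still named Timeline_SwordThrow, lerps it between tiles with a height offset while animating pitch and scale on the AnimRotationAndScale component.
; When the timeline finishes, it signals spell animation completion.
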(event EventEPlaySpellAnimation
  (bind _anim_rotationandscale (Variables|Default|GetAnim_RotationAndScale))
  (Transformation|SetActorLocationAndRotation (.location (CallFunction|FGetTileTransform (Variables|Default|GetOriginIndex))) (Math|Rotator|FindLookatRotation (Math|Conversions|ToVector(Vector2D) (Math|Conversions|ToVector2D(IntPoint) (Variables|Default|GetOriginIndex))) (Math|Conversions|ToVector(Vector2D) (Math|Conversions|ToVector2D(IntPoint) (Variables|Default|GetTargetIndex)))))
  (bind (_direction _actorlocationalpha _locationz _rotationy _scale) (Timeline|Timeline_SwordThrow PlayFromStart)
    (:Update
      (Transformation|SetActorLocation (+ (Math|Vector|Lerp(Vector) (.location (CallFunction|FGetTileTransform (Variables|Default|GetOriginIndex))) (.location (CallFunction|FGetTileTransform (Variables|Default|GetTargetIndex))) _actorlocationalpha) (Math|Vector|MakeVector 0.0 0.0 _locationz)) false false)
      (Transformation|SetRelativeRotation _anim_rotationandscale (Math|Rotator|MakeRotator 0.0 _rotationy 0.0) false false)
      (Transformation|SetRelativeScale3D _anim_rotationandscale (Math|Conversions|ToVector(Float) _scale)))
    (:Finished
      (CallFunction|ECompleteSpellAnimation))))

(fn ConstructionScript
  (|CallParentFunction))