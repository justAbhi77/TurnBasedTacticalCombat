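; Spell animation actor for a sword throw, flying from the origin tile to the target tile.
; On play it snaps to the origin tile facing the target, then a timeline lerps its location between the two tile transforms.
; The same timeline drives a child component's sideways offset, yaw spin and scale for the throw motion.
; When the timeline finishes, it signals that the spell animation is complete.
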(event EventEPlaySpellAnimation
  (Transformation|SetActorLocationAndRotation (.location (CallFunction|FGetTileTransform (Variables|Default|GetOriginIndex))) (Math|Rotator|FindLookatRotation (Math|Conversions|ToVector(Vector2D) (Math|Conversions|ToVector2D(IntPoint) (Variables|Default|GetOriginIndex))) (Math|Conversions|ToVector(Vector2D) (Math|Conversions|ToVector2D(IntPoint) (Variables|Default|GetTargetIndex)))))
  (bind (_direction _actorlocationalpha _locationy _rotationz _scale) (Timeline|Timeline_SwordThrow PlayFromStart)
    (:Update
      (Transformation|SetActorLocation (Math|Vector|Lerp(Vector) (.location (CallFunction|FGetTileTransform (Variables|Default|GetOriginIndex))) (.location (CallFunction|FGetTileTransform (Variables|Default|GetTargetIndex))) _actorlocationalpha) false false)
      (Transformation|SetRelativeTransform (Variables|Default|GetAnim_RotationAndScale) (Math|Transform|MakeTransform (Math|Vector|MakeVector 0.0 _locationy 0.0) (Math|Rotator|MakeRotator 0.0 0.0 _rotationz) (Math|Conversions|ToVector(Float) _scale)) false false))
    (:Finished
      (CallFunction|ECompleteSpellAnimation))))

(fn ConstructionScript
  (|CallParentFunction))