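; Spell animation Blueprint for the Dark Wave spell, played at the target tile's location.
; A single timeline drives the opacity of three meshes and the scale of the AnimScale component, then completes the animation when finished.
; Once playback passes a short delay, a DoOnce reports a hit on every attack tile index.
; The construction script extends the parent's and tints each mesh a different shade of magenta.
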(event EventEPlaySpellAnimation
  (Transformation|SetActorLocation (.location (CallFunction|FGetTileTransform (Variables|Default|GetTargetIndex))) false false)
  (bind (_direction _opacity _scale) (Timeline|Timeline PlayFromStart)
    (:Update
      (Rendering|Material|SetScalarParameterValueonMaterials (Variables|Default|GetStaticMesh) "Opacity" _opacity)
      (Transformation|SetRelativeScale3D (Variables|Default|GetAnim_Scale) _scale)
      (if (> (Components|Timeline|GetPlaybackPosition (Variables|Default|GetTimeline)) 0.2)
        (Utilities|FlowControl|DoOnce false
          (:Completed
            (for _array_element (Variables|Default|GetAttackIndexes)
              (Default|CallOnSpellAnimationHitTile self _array_element))))))
    (:Finished
      (CallFunction|ECompleteSpellAnimation))))

(fn ConstructionScript
  (|CallParentFunction)
  (Utilities|FlowControl|Sequence
    (:then_0
      (Rendering|Material|SetVectorParameterValueonMaterials (Variables|Default|GetStaticMesh) "BaseColor" (Math|Conversions|ToVector(LinearColor) "(R=1.000000,G=0.197389,B=0.920835,A=1.000000)")))
    (:then_1
      (Rendering|Material|SetVectorParameterValueonMaterials (Variables|Default|GetStaticMesh1) "BaseColor" (Math|Conversions|ToVector(LinearColor) "(R=1.000000,G=0.105882,B=0.745098,A=1.000000)")))
    (:then_2
      (Rendering|Material|SetVectorParameterValueonMaterials (Variables|Default|GetStaticMesh2) "BaseColor" (Math|Conversions|ToVector(LinearColor) "(R=0.895833,G=0.000000,B=0.640442,A=1.000000)")))))