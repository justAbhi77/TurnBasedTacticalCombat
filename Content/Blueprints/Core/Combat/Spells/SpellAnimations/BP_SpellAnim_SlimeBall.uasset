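; Spell animation actor for a slime ball that flies from the origin tile to the target tile in combat.
; A timeline, still named SwordThrow, drives position, height offset, scale and opacity of three meshes tinted in green shades.
; Partway through playback, a DoOnce fires the hit callback for every attack tile index, and the timeline's end completes the spell animation.
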(event EventEPlaySpellAnimation
  (Transformation|SetActorLocationAndRotation (.location (CallFunction|FGetTileTransform (Variables|Default|GetOriginIndex))) "0, 0, 0")
  (bind (_direction _actorlocationalpha _locationz _opacity _scale) (Timeline|Timeline_SwordThrow PlayFromStart)
    (:Update
      (Transformation|SetActorLocation (+ (Math|Vector|Lerp(Vector) (.location (CallFunction|FGetTileTransform (Variables|Default|GetOriginIndex))) (.location (CallFunction|FGetTileTransform (Variables|Default|GetTargetIndex))) _actorlocationalpha) (Math|Vector|MakeVector 0.0 0.0 _locationz)) false false)
      (Rendering|Material|SetScalarParameterValueonMaterials (Variables|Default|GetStaticMesh1) "Opacity" _opacity)
      (Transformation|SetRelativeScale3D (Variables|Default|GetAnim_RotationAndScale) _scale)
      (if (> (Components|Timeline|GetPlaybackPosition (Variables|Default|GetTimeline_SwordThrow)) 0.55)
        (Utilities|FlowControl|DoOnce false
          (:Completed
            (for _array_element (Variables|Default|GetAttackIndexes)
              (Default|CallOnSpellAnimationHitTile self _array_element))))))
    (:Finished
      (CallFunction|ECompleteSpellAnimation))))

(fn ConstructionScript
  (|CallParentFunction)
  (Utilities|FlowControl|Sequence
    (:then_0
      (Rendering|Material|SetVectorParameterValueonMaterials (Variables|Default|GetStaticMesh) "BaseColor" (Math|Conversions|ToVector(LinearColor) "(R=0.197389,G=1.000000,B=0.398042,A=1.000000)")))
    (:then_1
      (Rendering|Material|SetVectorParameterValueonMaterials (Variables|Default|GetStaticMesh1) "BaseColor" (Math|Conversions|ToVector(LinearColor) "(R=0.105882,G=1.000000,B=0.100000,A=1.000000)")))
    (:then_2
      (Rendering|Material|SetVectorParameterValueonMaterials (Variables|Default|GetStaticMesh2) "BaseColor" (Math|Conversions|ToVector(LinearColor) "(R=0.000000,G=0.895833,B=0.600000,A=1.000000)")))))