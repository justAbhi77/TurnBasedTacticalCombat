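; BP_SpellAnim_WindGust is the spell animation for a wind gust spell on the tile grid.
; For each attacked tile except the target, it spawns a BP_AnimatedWindGust at the target tile, facing that tile and set to travel there while growing in scale.
; Each gust gets a random play rate, and a single gust's completion event, bound through a DoOnce, signals that the spell animation is complete.
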(event Custom|OnShapeAnimationCompleted_Event_0
  (params (AnimatedShape :type BP%20Animated%20Wind%20Gust%20Object%20Reference))
  (CallFunction|ECompleteSpellAnimation))

(event EventEPlaySpellAnimation
  (bind _targetindex (Variables|Default|GetTargetIndex))
  (bind _transform (CallFunction|FGetTileTransform _targetindex))
  (for _array_element (Variables|Default|GetAttackIndexes)
    (if (!= _array_element (Variables|Default|GetTargetIndex))
      (bind _returnvalue (Game|SpawnActorfromClass "/Game/Blueprints/Core/Combat/Spells/SpellAnimations/Components/BP_AnimatedWindGust.BP_AnimatedWindGust_C" (Math|Transform|MakeTransform "0, 0, 0" "0, 0, 0" "1.000000,1.000000,1.000000") "Undefined" "MultiplyWithRoot" 0 (Math|Transform|MakeTransform (.location _transform) (Math|Rotator|FindLookatRotation (.location _transform) (.location (CallFunction|FGetTileTransform _array_element))) "0.500000,0.500000,0.500000") (Math|Transform|MakeTransform (.location (CallFunction|FGetTileTransform _array_element)) (Math|Rotator|FindLookatRotation (.location _transform) (.location (CallFunction|FGetTileTransform _array_element))) "1.200000,1.200000,1.200000") (Math|Random|RandomFloatinRange 0.8 1.5) 0))
      (Utilities|FlowControl|DoOnce false
        (:Completed
          (EventDispatchers|AssignOnShapeAnimationCompleted _returnvalue (delegate Custom|OnShapeAnimationCompleted_Event_0)))))))

(fn ConstructionScript
  (|CallParentFunction))