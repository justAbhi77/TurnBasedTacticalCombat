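; Grid visual actor that draws tiles as instances of one InstancedStaticMesh, with mesh, material, collision and color mode set at initialization.
; A parallel index array maps grid indices to instances, so adding replaces any existing tile.
; Color comes from either tile type or the highest-priority active state, such as spell range, selection, hover or path.
; Per-instance custom data passes that RGB color and a filled flag to the material.
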(event EventBeginPlay
  (Actor|Tick|SetActorTickEnabled false))

(fn ConstructionScript)

(fn FAddInstance
  (params (Index :type Int%20Point%20Structure%20%28by%20ref%29) (TileType :type E_Tiletype%20Enum :default "NewEnumerator0") (Transform :type Transform%20%28by%20ref%29) (States :type Array%20of%20E_TileState%20Enums :default "NewEnumerator0"))
  (CallFunction|FRemoveInstance Index)
  (bind _returnvalue (Utilities|Array|Add (Variables|Private|GetInstanceIndexes) Index))
  (LocalVariables|SetInstanceIndex _returnvalue)
  (Components|InstancedStaticMesh|AddInstance (Variables|Default|GetInstancedStaticMesh) Transform false)
  (bind (_isfilled _color) (CallFunction|FGetColorfromStatesorTiles TileType States))
  (Components|InstancedStaticMesh|SetCustomDataValue (Variables|Default|GetInstancedStaticMesh) (LocalVariables|GetInstanceIndex) 0 (.R (Math|Color|BreakColor _color)) false) ; Red
  (Components|InstancedStaticMesh|SetCustomDataValue (Variables|Default|GetInstancedStaticMesh) (LocalVariables|GetInstanceIndex) 1 (.G (Math|Color|BreakColor _color)) false) ; Blue
  (Components|InstancedStaticMesh|SetCustomDataValue (Variables|Default|GetInstancedStaticMesh) (LocalVariables|GetInstanceIndex) 2 (.B (Math|Color|BreakColor _color)) false) ; Green
  (Components|InstancedStaticMesh|SetCustomDataValue (Variables|Default|GetInstancedStaticMesh) (LocalVariables|GetInstanceIndex) 3 _isfilled false) ; is Filled
)

(fn FRemoveInstance
  (params (Index :type Int%20Point%20Structure%20%28by%20ref%29))
  (if (Utilities|Array|ContainsItem (Variables|Private|GetInstanceIndexes) Index)
    (Class|InstancedStaticMeshComponent|RemoveInstance (Variables|Default|GetInstancedStaticMesh) (Utilities|Array|FindItem (Variables|Private|GetInstanceIndexes) Index))
    (Utilities|Array|RemoveItem (Variables|Private|GetInstanceIndexes) Index)))

(fn FClearInstances
  (Components|InstancedStaticMesh|ClearInstances (Variables|Default|GetInstancedStaticMesh))
  (Utilities|Array|Clear (Variables|Private|GetInstanceIndexes)))

(fn FInitializeGridMeshInst
  (params (Mesh :type Static%20Mesh%20Object%20Reference) (Material :type Material%20Interface%20Object%20Reference) (bColorBasedOnTileType :type Boolean) (Collision :type ECollisionEnabled%20Enum :default "NoCollision"))
  (Components|StaticMesh|SetStaticMesh (Variables|Default|GetInstancedStaticMesh) Mesh)
  (Rendering|Material|SetMaterial (Variables|Default|GetInstancedStaticMesh) 0 Material)
  (Variables|Default|SetbIsColorBasedOnTileType bColorBasedOnTileType)
  (Collision|SetCollisionEnabled (Variables|Default|GetInstancedStaticMesh) Collision))

(fn FGetColorfromStatesorTiles
  (params (TileType :type E_Tiletype%20Enum :default "NewEnumerator0") (States :type Array%20of%20E_TileState%20Enums :default "NewEnumerator0"))
  (if (Variables|Default|GetbIsColorBasedOnTileType)
    (return (LocalVariables|GetbRetIsFilled) (Utilities|Select :Index TileType :NewEnumerator0 "" :NewEnumerator1 "(R=0.500000,G=0.500000,B=0.500000,A=1.000000)" :NewEnumerator2 "(R=0.950000,G=0.047500,B=0.047500,A=1.000000)" :NewEnumerator3 "(R=0.300000,G=0.300000,B=0.300000,A=1.000000)" :NewEnumerator4 "(R=0.050000,G=0.050000,B=0.050000,A=1.000000)" :NewEnumerator5 "(R=0.700000,G=0.210000,B=0.700000,A=1.000000)"))
    (else
      (LocalVariables|SetbRetIsFilled 0.0)
      (LocalVariables|SetRetColor "")
      (Utilities|FlowControl|Sequence
        (:then_0
          (if (== (Utilities|Array|Length States) 0)
            (LocalVariables|SetRetColor "(R=0.000000,G=0.000000,B=0.000000,A=1.000000)")
            (else
              (bind _array_element (Utilities|Array|ForEachLoopwithBreak (Utilities|Array|MakeArray "NewEnumerator10" "NewEnumerator9" "NewEnumerator2" "NewEnumerator1" "NewEnumerator4" "NewEnumerator5" "NewEnumerator6" "NewEnumerator7" "NewEnumerator8") :!label _label)
                (:LoopBody
                  (if (Utilities|Array|ContainsItem States _array_element)
                    (LocalVariables|SetbRetIsFilled 1.0)
                    (LocalVariables|SetRetColor (Utilities|Select :Index _array_element :NewEnumerator0 "" :NewEnumerator1 "(R=1.000000,G=0.587559,B=0.205564,A=1.000000)" :NewEnumerator2 "(R=1.000000,G=0.139509,B=0.067812,A=1.000000)" :NewEnumerator4 "(R=1.000000,G=0.074391,B=0.532272,A=1.000000)" :NewEnumerator5 "(R=0.131729,G=0.000000,B=1.000000,A=1.000000)" :NewEnumerator6 "(R=1.000000,G=0.108441,B=0.540559,A=1.000000)" :NewEnumerator7 "(R=1.000000,G=0.128937,B=0.000000,A=1.000000)" :NewEnumerator8 "(R=0.000000,G=0.133333,B=0.286275,A=1.000000)" :NewEnumerator9 "(R=0.701961,G=0.243137,B=0.058824,A=1.000000)" :NewEnumerator10 "(R=1.000000,G=0.035684,B=0.205752,A=1.000000)"))
                    (goto _label Break)))))))
        (:then_1
          (return (LocalVariables|GetbRetIsFilled) (LocalVariables|GetRetColor)))))))