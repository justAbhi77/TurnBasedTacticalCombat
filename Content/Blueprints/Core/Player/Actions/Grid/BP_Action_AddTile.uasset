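; Player action Blueprint that adds a new tile to the grid at a chosen index.
; On execute, it only acts when that index is not already a valid tile.
; It traces for ground at the index's location and adds a tile there using the grid's rotation and scale with a fixed tile type.
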(fn ConstructionScript
  (|CallParentFunction))

(fn FExecuteAction
  (params (index :type Int%20Point%20Structure))
  (bind _playeractions (Variables|Default|GetPlayerActions))
  (bind _grid (Variables|/Game/Blueprints/Core/Player/BP_PlayerActions.BP_PlayerActions_C|GetGrid _playeractions))
  (|CallParentFunction index)
  (bind _playeractions_2 (Variables|Default|GetPlayerActions)
    (:then
      (if (not (Default|FIsIndexValid (Variables|/Game/Blueprints/Core/Player/BP_PlayerActions.BP_PlayerActions_C|GetGrid _playeractions_2) index))
        (bind _outlocation (Default|FTraceforGround (Variables|/Game/Blueprints/Core/Player/BP_PlayerActions.BP_PlayerActions_C|GetGrid (Variables|Default|GetPlayerActions)) (Default|FGetTileLocationfromGridIndex _grid index)))
        (Default|FAddGridTile (Variables|/Game/Blueprints/Core/Player/BP_PlayerActions.BP_PlayerActions_C|GetGrid (Variables|Default|GetPlayerActions)) (Utilities|Struct|MakeStruct_TileData index "NewEnumerator1" (Math|Transform|MakeTransform _outlocation (Default|FGetTileRotationfromGridIndex _grid index) (Default|FGetTileScale _grid)) "NewEnumerator0"))))
    (:else)))