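; BP_Action_SelectTile is a grid player action that selects a tile, or deselects it when the same tile is chosen again.
; It overrides FExecuteAction to move a tile state on PlayerActions' Grid from the previous tile to the new one and update SelectedTile.
; An index of (-999, -999) serves as the no-selection sentinel.
; EndPlay executes the action with that sentinel to clear the selection.
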(event EventEndPlay
  (params (EndPlayReason :type EEndPlayReason%20Enum :default "Destroyed"))
  (CallFunction|FExecuteAction (Utilities|Struct|MakeIntPoint -999 -999)))

(fn ConstructionScript
  (|CallParentFunction))

(fn FExecuteAction
  (params (index :type Int%20Point%20Structure))
  (bind _playeractions (Variables|Default|GetPlayerActions))
  (bind _playeractions_2 (Variables|Default|GetPlayerActions))
  (bind _playeractions_3 (Variables|Default|GetPlayerActions))
  (|CallParentFunction index)
  (bind _playeractions_4 (Variables|Default|GetPlayerActions)
    (:then
      (if (!= (Variables|/Game/Blueprints/Core/Player/BP_PlayerActions.BP_PlayerActions_C|GetSelectedTile _playeractions_4) index)
        (Default|FRemoveStatefromTile (Variables|/Game/Blueprints/Core/Player/BP_PlayerActions.BP_PlayerActions_C|GetGrid _playeractions) (Variables|/Game/Blueprints/Core/Player/BP_PlayerActions.BP_PlayerActions_C|GetSelectedTile _playeractions) "NewEnumerator2")
        (Variables|/Game/Blueprints/Core/Player/BP_PlayerActions.BP_PlayerActions_C|SetSelectedTile (Variables|Default|GetPlayerActions) index)
        (Default|FAddStatetoTile (Variables|/Game/Blueprints/Core/Player/BP_PlayerActions.BP_PlayerActions_C|GetGrid _playeractions_2) (Variables|/Game/Blueprints/Core/Player/BP_PlayerActions.BP_PlayerActions_C|GetSelectedTile _playeractions_2) "NewEnumerator2")
        (else
          (Default|FRemoveStatefromTile (Variables|/Game/Blueprints/Core/Player/BP_PlayerActions.BP_PlayerActions_C|GetGrid _playeractions_3) (Variables|/Game/Blueprints/Core/Player/BP_PlayerActions.BP_PlayerActions_C|GetSelectedTile _playeractions_3) "NewEnumerator2")
          (Variables|/Game/Blueprints/Core/Player/BP_PlayerActions.BP_PlayerActions_C|SetSelectedTile (Variables|Default|GetPlayerActions) (Utilities|Struct|MakeIntPoint -999 -999)))))
    (:else)))