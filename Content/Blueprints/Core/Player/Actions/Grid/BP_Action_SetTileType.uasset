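; BP_Action_SetTileType is a player action that changes the type of a grid tile.
; When executed on a tile index, it confirms the index is valid on the grid owned by PlayerActions and reads that tile's existing data.
; It then re-adds the tile with the action's TileType, keeping its index, transform, states and occupying unit.
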(fn ConstructionScript
  (|CallParentFunction))

(fn FExecuteAction
  (params (index :type Int%20Point%20Structure))
  (|CallParentFunction index)
  (bind _playeractions (Variables|Default|GetPlayerActions)
    (:then
      (if (Default|FIsIndexValid (Variables|/Game/Blueprints/Core/Player/BP_PlayerActions.BP_PlayerActions_C|GetGrid _playeractions) index)
        (LocalVariables|SetData (.Value (Utilities|Map|Find (Variables|/Game/Blueprints/Core/Grid/BP_Grid.BP_Grid_C|GetGridTiles (Variables|/Game/Blueprints/Core/Player/BP_PlayerActions.BP_PlayerActions_C|GetGrid (Variables|Default|GetPlayerActions))) index)))
        (Default|FAddGridTile (Variables|/Game/Blueprints/Core/Player/BP_PlayerActions.BP_PlayerActions_C|GetGrid (Variables|Default|GetPlayerActions)) (Utilities|Struct|MakeStruct_TileData (.index (LocalVariables|GetData)) (Variables|Default|GetTileType) (.transform (LocalVariables|GetData)) (.states (LocalVariables|GetData)) (.unitontile (LocalVariables|GetData))))))
    (:else)))