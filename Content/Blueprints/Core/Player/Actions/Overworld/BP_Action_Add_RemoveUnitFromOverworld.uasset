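; Player action that adds or removes units in the overworld, switched by an add/remove flag.
; Adding traces under the cursor, spawns a unit of the selected type at the navigation-projected hit point, sets its context and registers it with an overworld group.
; Removing destroys the hovered unit.
; The tile-type validation and combat-removal logic is disconnected and never runs.
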(fn ConstructionScript
  (|CallParentFunction))

(fn FExecuteAction
  (params (index :type Int%20Point%20Structure))
  (bind _returnvalue (Game|GetPlayerController 0))
  (bind (_hitresult _returnvalue_2) (Game|Player|GetHitResultUnderCursorbyChannel _returnvalue "TraceTypeQuery3" false))
  (|CallParentFunction index)
  (if (Variables|Default|GetbIsAddingUnit)
    (if (!= index (Utilities|Struct|MakeIntPoint -999 -999))
      (if _returnvalue_2
        (LocalVariables|SetHitLocation (.Location (Collision|BreakHitResult _hitresult)))
        (bind _returnvalue_3 (Game|SpawnActorfromClass "/Game/Blueprints/Core/Units/BP_Unit.BP_Unit_C" (Math|Transform|MakeTransform "0, 0, 0" "0, 0, 0" "1.000000,1.000000,1.000000") "AlwaysSpawn" "MultiplyWithRoot" 0 (Variables|Default|GetUnitType) 0))
        (bind _output_get (LocalVariables|SetUnit _returnvalue_3))
        (Transformation|SetActorLocation _output_get (Default|FAddCapsuleHeight _output_get (.ProjectedLocation (AI|Navigation|ProjectPointtoNavigation (LocalVariables|GetHitLocation) (Variables|/Game/Blueprints/Core/Units/BP_Unit.BP_Unit_C|GetNav%20Data _output_get) 0 "500.000000,500.000000,999999.000000"))) false false)
        (Default|FSetUnitContext (LocalVariables|GetUnit) "NewEnumerator1")
        (Default|FAddUnittoGroup (Variables|/Game/Blueprints/Core/Player/BP_PlayerActions.BP_PlayerActions_C|GetOverWorldUnitGroupsManager (Variables|Default|GetPlayerActions)) (LocalVariables|GetUnit) (Variables|Default|GetGroupId))))
    (else
      (bind _hoveredunit (Variables|/Game/Blueprints/Core/Player/BP_PlayerActions.BP_PlayerActions_C|GetHoveredUnit (Variables|Default|GetPlayerActions))
        (:then
          (Actor|DestroyActor _hoveredunit))
        (:else)))))