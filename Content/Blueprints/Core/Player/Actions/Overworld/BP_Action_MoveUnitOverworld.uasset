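; BP_Action_MoveUnitOverworld is a player action that orders the selected unit to move in the overworld.
; On execute it runs the parent logic, then, if a selected unit is valid, traces under the cursor on a dedicated trace channel.
; On a hit it sends the unit to that location, passing the hovered unit as the one to follow, with random locations off.
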(event EventBeginPlay)

(fn ConstructionScript
  (|CallParentFunction))

(fn FExecuteAction
  (params (index :type Int%20Point%20Structure))
  (bind _returnvalue (Game|GetPlayerController 0))
  (bind (_hitresult _returnvalue_2) (Game|Player|GetHitResultUnderCursorbyChannel _returnvalue "TraceTypeQuery3" false))
  (|CallParentFunction index)
  (bind _selectedunit (Variables|/Game/Blueprints/Core/Player/BP_PlayerActions.BP_PlayerActions_C|GetSelectedUnit (Variables|Default|GetPlayerActions))
    (:then
      (if _returnvalue_2
        (Default|EMoveUnitinOverworld _selectedunit (.Location (Collision|BreakHitResult _hitresult)) (Variables|/Game/Blueprints/Core/Player/BP_PlayerActions.BP_PlayerActions_C|GetHoveredUnit (Variables|Default|GetPlayerActions)) false)))
    (:else)))