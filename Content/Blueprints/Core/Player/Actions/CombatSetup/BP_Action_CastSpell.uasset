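; Player action Blueprint that casts a spell in the tile-based combat setup.
; On execute it runs the parent logic, then asks the combat system to cast its Spell from the selected tile onto the target tile index.
; It then calls FResetAp on the selected unit, if that unit is valid.
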(fn ConstructionScript
  (|CallParentFunction))

(fn FExecuteAction
  (params (index :type Int%20Point%20Structure))
  (bind _playeractions (Variables|Default|GetPlayerActions))
  (|CallParentFunction index)
  (Default|FCastSpell (Variables|/Game/Blueprints/Core/Player/BP_PlayerActions.BP_PlayerActions_C|GetCombatSystem _playeractions) (Variables|Default|GetSpell) (Variables|/Game/Blueprints/Core/Player/BP_PlayerActions.BP_PlayerActions_C|GetSelectedTile _playeractions) index)
  (bind _selectedunit (Variables|/Game/Blueprints/Core/Player/BP_PlayerActions.BP_PlayerActions_C|GetSelectedUnit (Variables|Default|GetPlayerActions))
    (:then
      (Default|FResetAp _selectedunit))
    (:else)))