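; Player action that computes the pathfinding minimum-cost heuristic from every grid tile to the currently selected tile.
; On execute it runs the parent action, clears the generated pathfinding data, then checks that the selected tile index is valid.
; It registers each grid tile as discovered with zero cost from start and its minimum cost to the selection, honoring the diagonals setting, without running a path search.
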(fn ConstructionScript
  (|CallParentFunction))

(fn FExecuteAction
  (params (index :type Int%20Point%20Structure))
  (bind _playeractions (Variables|Default|GetPlayerActions))
  (bind _playeractions_2 (Variables|Default|GetPlayerActions))
  (bind _grid (Variables|/Game/Blueprints/Core/Player/BP_PlayerActions.BP_PlayerActions_C|GetGrid _playeractions))
  (|CallParentFunction index)
  (Default|FClearGeneratedData (Variables|/Game/Blueprints/Core/Grid/BP_Grid.BP_Grid_C|GetGridPathfinding (Variables|/Game/Blueprints/Core/Player/BP_PlayerActions.BP_PlayerActions_C|GetGrid (Variables|Default|GetPlayerActions))))
  (if (Default|FIsIndexValid (Variables|/Game/Blueprints/Core/Player/BP_PlayerActions.BP_PlayerActions_C|GetGrid _playeractions_2) (Variables|/Game/Blueprints/Core/Player/BP_PlayerActions.BP_PlayerActions_C|GetSelectedTile _playeractions_2))
    (bind _keys (Utilities|Map|Keys (Variables|/Game/Blueprints/Core/Grid/BP_Grid.BP_Grid_C|GetGridTiles _grid)))
    (for _array_element _keys
      (Default|FDiscoverTile (Variables|/Game/Blueprints/Core/Grid/BP_Grid.BP_Grid_C|GetGridPathfinding (Variables|/Game/Blueprints/Core/Player/BP_PlayerActions.BP_PlayerActions_C|GetGrid (Variables|Default|GetPlayerActions))) (Utilities|Struct|MakeStruct_PathfindingData _array_element 1 0 (Default|FGetMinimumCostBetweenTwoTiles (Variables|/Game/Blueprints/Core/Grid/BP_Grid.BP_Grid_C|GetGridPathfinding _grid) _array_element (Variables|/Game/Blueprints/Core/Player/BP_PlayerActions.BP_PlayerActions_C|GetSelectedTile (Variables|Default|GetPlayerActions)) (Variables|Default|GetbIncludeDiagonals)) "(X=-999,Y=-999)")))))