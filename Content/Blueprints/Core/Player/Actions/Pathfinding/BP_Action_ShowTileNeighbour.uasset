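; Player action that highlights the valid neighbours of a given grid tile, likely as a visual check on grid pathfinding.
; On execute it clears the neighbour state from the grid, queries GridPathfinding for neighbours filtered by tile type and the diagonals setting, then tags each result with that state.
; EndPlay re-executes with an out-of-range sentinel index, so the highlight is cleared when the action is removed.
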(event EventEndPlay
  (params (EndPlayReason :type EEndPlayReason%20Enum :default "Destroyed"))
  (CallFunction|FExecuteAction (Utilities|Struct|MakeIntPoint -999 -999)))

(fn ConstructionScript
  (|CallParentFunction))

(fn FExecuteAction
  (params (index :type Int%20Point%20Structure))
  (|CallParentFunction index)
  (Variables|Default|GetPlayerActions
    (:then
      (Default|FClearStatefromTiles (Variables|/Game/Blueprints/Core/Player/BP_PlayerActions.BP_PlayerActions_C|GetGrid (Variables|Default|GetPlayerActions)) "NewEnumerator4")
      (bind _neighbours (Default|FGetValidTileNeighbour (Variables|/Game/Blueprints/Core/Grid/BP_Grid.BP_Grid_C|GetGridPathfinding (Variables|/Game/Blueprints/Core/Player/BP_PlayerActions.BP_PlayerActions_C|GetGrid (Variables|Default|GetPlayerActions))) index (Variables|Default|GetbIncludeDiagonals) (Utilities|Array|MakeArray "NewEnumerator1" "NewEnumerator3" "NewEnumerator4" "NewEnumerator5")))
      (for _array_element _neighbours
        (Default|FAddStatetoTile (Variables|/Game/Blueprints/Core/Player/BP_PlayerActions.BP_PlayerActions_C|GetGrid (Variables|Default|GetPlayerActions)) (.index _array_element) "NewEnumerator4")))
    (:else)))