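; Player action that, after the inherited select tile and unit step, highlights every tile reachable from the selected tile.
; It runs the grid's reachables pathfinder with the selected unit's movement stats, or the action's own path settings when no unit is selected.
; The completion callback marks returned tiles with a grid state.
; Highlights clear when the unit starts walking and regenerate when it finishes.
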(fn ConstructionScript
  (|CallParentFunction))

(fn FGenerateReachables
  (bind _playeractions (Variables|Default|GetPlayerActions))
  (bind _playeractions_2 (Variables|Default|GetPlayerActions))
  (bind _playeractions_3 (Variables|Default|GetPlayerActions))
  (bind _playeractions_4 (Variables|Default|GetPlayerActions))
  (bind _selectedunit (Variables|/Game/Blueprints/Core/Player/BP_PlayerActions.BP_PlayerActions_C|GetSelectedUnit _playeractions_3))
  (bind _selectedunit_2 (Variables|/Game/Blueprints/Core/Player/BP_PlayerActions.BP_PlayerActions_C|GetSelectedUnit _playeractions_4))
  (bind _unitdata (Variables|/Game/Blueprints/Core/Units/BP_Unit.BP_Unit_C|GetUnitData _selectedunit_2))
  (bind _stats (Utilities|Struct|BreakStruct_UnitData _unitdata))
  (bind (_validtiletypes _bcanmovediagonally _mp_current) (Utilities|Struct|BreakStruct_UnitData_Stats _stats))
  (Default|FClearStatefromTiles (Variables|/Game/Blueprints/Core/Player/BP_PlayerActions.BP_PlayerActions_C|GetGrid (Variables|Default|GetPlayerActions)) "NewEnumerator8")
  (EventDispatchers|BindEventtoOnPathfindingCompleted (Variables|/Game/Blueprints/Core/Grid/BP_Grid.BP_Grid_C|GetGridPathfinding_Reachables (Variables|/Game/Blueprints/Core/Player/BP_PlayerActions.BP_PlayerActions_C|GetGrid (Variables|Default|GetPlayerActions))) (EventDispatchers|CreateEvent :!event FonPathFindingCompleted))
  (Variables|/Game/Blueprints/Core/Player/BP_PlayerActions.BP_PlayerActions_C|GetSelectedUnit (Variables|Default|GetPlayerActions)
    (:then
      (EventDispatchers|BindEventtoOnUnitStartedWalking _selectedunit (EventDispatchers|CreateEvent :!event FonUnitStartedWalking))
      (EventDispatchers|BindEventtoOnUnitFinishedWalking _selectedunit (EventDispatchers|CreateEvent :!event FonUnitFinishedwalking))
      (Default|FFindPath (Variables|/Game/Blueprints/Core/Grid/BP_Grid.BP_Grid_C|GetGridPathfinding_Reachables (Variables|/Game/Blueprints/Core/Player/BP_PlayerActions.BP_PlayerActions_C|GetGrid _playeractions)) (Variables|/Game/Blueprints/Core/Player/BP_PlayerActions.BP_PlayerActions_C|GetSelectedTile _playeractions) (Utilities|Struct|MakeIntPoint -999 -999) _bcanmovediagonally _validtiletypes 0.1 15.0 true _mp_current))
    (:else
      (Default|FFindPath (Variables|/Game/Blueprints/Core/Grid/BP_Grid.BP_Grid_C|GetGridPathfinding_Reachables (Variables|/Game/Blueprints/Core/Player/BP_PlayerActions.BP_PlayerActions_C|GetGrid _playeractions_2)) (Variables|/Game/Blueprints/Core/Player/BP_PlayerActions.BP_PlayerActions_C|GetSelectedTile _playeractions_2) (Utilities|Struct|MakeIntPoint -999 -999) (Variables|Default|GetbIncludeDiagonals) (select (Variables|Default|GetbIncludeFlyingOnly) (Utilities|Array|MakeArray "NewEnumerator1" "NewEnumerator3" "NewEnumerator4" "NewEnumerator5") (Utilities|Array|MakeArray "NewEnumerator1" "NewEnumerator3" "NewEnumerator4")) (Variables|Default|GetDelayBetweenIterations) (Variables|Default|GetMaxMsPerFrame) true (Variables|Default|GetMaxPathLength)))))

(fn FExecuteAction
  (params (index :type Int%20Point%20Structure))
  (Utilities|FlowControl|Sequence
    (:then_0
      (|CallParentFunction index))
    (:then_1
      (CallFunction|FGenerateReachables))))

(fn FonPathFindingCompleted
  (params (Path :type Array%20of%20Int%20Point%20Structures))
  (for _array_element Path
    (Default|FAddStatetoTile (Variables|/Game/Blueprints/Core/Player/BP_PlayerActions.BP_PlayerActions_C|GetGrid (Variables|Default|GetPlayerActions)) _array_element "NewEnumerator8")))

(fn FonUnitStartedWalking
  (params (Unit :type BP%20Unit%20Object%20Reference))
  (Default|FClearStatefromTiles (Variables|/Game/Blueprints/Core/Player/BP_PlayerActions.BP_PlayerActions_C|GetGrid (Variables|Default|GetPlayerActions)) "NewEnumerator8"))

(fn FonUnitFinishedWalking
  (params (Unit :type BP%20Unit%20Object%20Reference))
  (CallFunction|FGenerateReachables))