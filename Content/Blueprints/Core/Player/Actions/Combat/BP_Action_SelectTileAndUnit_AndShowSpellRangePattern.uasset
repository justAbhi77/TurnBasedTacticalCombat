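; Player action that selects a tile and unit, judging by its name and parent call, then highlights the spell range pattern from that tile.
; On execute it runs the parent action, then clears the range tile state from the Grid.
; If the selected tile is valid, it asks the CombatSystem for the spell range from that origin and adds the state to each returned tile.
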(event EventBeginPlay)

(fn ConstructionScript
  (|CallParentFunction))

(fn FExecuteAction
  (params (index :type Int%20Point%20Structure))
  (|CallParentFunction index)
  (CallFunction|FShowSpellRangePattern))

(fn FShowSpellRangePattern
  (bind _playeractions (Variables|Default|GetPlayerActions))
  (bind _playeractions_2 (Variables|Default|GetPlayerActions))
  (Default|FClearStatefromTiles (Variables|/Game/Blueprints/Core/Player/BP_PlayerActions.BP_PlayerActions_C|GetGrid (Variables|Default|GetPlayerActions)) "NewEnumerator9")
  (if (Default|FIsIndexValid (Variables|/Game/Blueprints/Core/Player/BP_PlayerActions.BP_PlayerActions_C|GetGrid _playeractions_2) (Variables|/Game/Blueprints/Core/Player/BP_PlayerActions.BP_PlayerActions_C|GetSelectedTile _playeractions_2))
    (bind _rangesindexes (Default|FGetSpellRange (Variables|/Game/Blueprints/Core/Player/BP_PlayerActions.BP_PlayerActions_C|GetCombatSystem _playeractions) (Variables|/Game/Blueprints/Core/Player/BP_PlayerActions.BP_PlayerActions_C|GetSelectedTile _playeractions) (Variables|Default|GetCast)))
    (for _array_element _rangesindexes
      (Default|FAddStatetoTile (Variables|/Game/Blueprints/Core/Player/BP_PlayerActions.BP_PlayerActions_C|GetGrid (Variables|Default|GetPlayerActions)) _array_element "NewEnumerator9"))))