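; BP_Action_SetUnitTeamIndex is a player action that changes the team of the unit standing on a grid tile.
; When executed with a tile index, it runs the parent action, then looks up that tile in the grid's tile map.
; If a valid unit occupies the tile, it passes that unit and the action's TeamIndex to the combat system's FSetUnitTeamIndex.
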(fn ConstructionScript
  (|CallParentFunction))

(fn FExecuteAction
  (params (index :type Int%20Point%20Structure))
  (bind _playeractions (Variables|Default|GetPlayerActions))
  (bind _grid (Variables|/Game/Blueprints/Core/Player/BP_PlayerActions.BP_PlayerActions_C|GetGrid _playeractions))
  (bind _gridtiles (Variables|/Game/Blueprints/Core/Grid/BP_Grid.BP_Grid_C|GetGridTiles _grid))
  (bind _value (Utilities|Map|Find _gridtiles index))
  (bind _unitontile (Utilities|Struct|BreakStruct_TileData _value))
  (|CallParentFunction index)
  (Utilities|IsValid _unitontile
    (:Is%20Valid
      (Default|FSetUnitTeamIndex (Variables|/Game/Blueprints/Core/Player/BP_PlayerActions.BP_PlayerActions_C|GetCombatSystem (Variables|Default|GetPlayerActions)) _unitontile (Variables|Default|GetTeamIndex)))))