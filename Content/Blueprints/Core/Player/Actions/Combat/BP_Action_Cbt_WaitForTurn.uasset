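; Player combat action, named for waiting for a turn, that previews the movement range of the hovered unit, or the selected unit if none is hovered.
; When that unit changes, it clears the old tile highlights and runs grid pathfinding using the unit's current movement points, tile types and diagonal rule.
; A pathfinding completion callback marks reachable tiles with a grid state, which is cleared when the action ends.
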(event EventBeginPlay
  (|CallParentFunction)
  (EventDispatchers|BindEventtoOnPathfindingCompleted (Variables|/Game/Blueprints/Core/Grid/BP_Grid.BP_Grid_C|GetGridPathfinding_Reachables (Variables|/Game/Blueprints/Core/Player/BP_PlayerActions.BP_PlayerActions_C|GetGrid (Variables|Default|GetPlayerActions))) (EventDispatchers|CreateEvent :!event FonPathfindingCompletedReachables)))

(event EventEndPlay
  (params (EndPlayReason :type EEndPlayReason%20Enum :default "Destroyed"))
  (|CallParentFunction EndPlayReason)
  (Default|FClearStatefromTiles (Variables|/Game/Blueprints/Core/Player/BP_PlayerActions.BP_PlayerActions_C|GetGrid (Variables|Default|GetPlayerActions)) "NewEnumerator8"))

(fn ConstructionScript
  (|CallParentFunction))

(fn FGenerateReachables
  (params (Unit :type BP%20Unit%20Object%20Reference))
  (if (!= Unit (Variables|Default|GetCurrentUnitForReachables))
    (Variables|Default|SetCurrentUnitForReachables Unit)
    (Default|FClearStatefromTiles (Variables|/Game/Blueprints/Core/Player/BP_PlayerActions.BP_PlayerActions_C|GetGrid (Variables|Default|GetPlayerActions)) "NewEnumerator8")
    (Variables|Default|GetCurrentUnitForReachables
      (:then
        (Default|FFindPath (Variables|/Game/Blueprints/Core/Grid/BP_Grid.BP_Grid_C|GetGridPathfinding_Reachables (Variables|/Game/Blueprints/Core/Player/BP_PlayerActions.BP_PlayerActions_C|GetGrid (Variables|Default|GetPlayerActions))) (Variables|/Game/Blueprints/Core/Units/BP_Unit.BP_Unit_C|GetIndex (Variables|Default|GetCurrentUnitForReachables)) (Utilities|Struct|MakeIntPoint -999 -999) (.bCanMoveDiagonally (Utilities|Struct|BreakStruct_UnitData_Stats (.Stats (Utilities|Struct|BreakStruct_UnitData (Variables|/Game/Blueprints/Core/Units/BP_Unit.BP_Unit_C|GetUnitData (Variables|Default|GetCurrentUnitForReachables)))))) (.ValidTileTypes (Utilities|Struct|BreakStruct_UnitData_Stats (.Stats (Utilities|Struct|BreakStruct_UnitData (Variables|/Game/Blueprints/Core/Units/BP_Unit.BP_Unit_C|GetUnitData (Variables|Default|GetCurrentUnitForReachables)))))) 0.1 15.0 true (.MP_Current (Utilities|Struct|BreakStruct_UnitData_Stats (.Stats (Utilities|Struct|BreakStruct_UnitData (Variables|/Game/Blueprints/Core/Units/BP_Unit.BP_Unit_C|GetUnitData (Variables|Default|GetCurrentUnitForReachables))))))))
      (:else))))

(fn FonPathfindingCompletedReachables
  (params (Reachables :type Array%20of%20Int%20Point%20Structures))
  (for _array_element Reachables
    (Default|FAddStatetoTile (Variables|/Game/Blueprints/Core/Player/BP_PlayerActions.BP_PlayerActions_C|GetGrid (Variables|Default|GetPlayerActions)) _array_element "NewEnumerator8")))

(fn FExecuteHoveredAction
  (params (index :type Int%20Point%20Structure))
  (bind _playeractions (Variables|Default|GetPlayerActions))
  (bind _hoveredunit (Variables|/Game/Blueprints/Core/Player/BP_PlayerActions.BP_PlayerActions_C|GetHoveredUnit _playeractions))
  (|CallParentFunction index)
  (Utilities|IsValid _hoveredunit
    (:Is%20Valid
      (CallFunction|FGenerateReachables _hoveredunit))
    (:Is%20Not%20Valid
      (CallFunction|FGenerateReachables (Variables|/Game/Blueprints/Core/Player/BP_PlayerActions.BP_PlayerActions_C|GetSelectedUnit _playeractions)))))