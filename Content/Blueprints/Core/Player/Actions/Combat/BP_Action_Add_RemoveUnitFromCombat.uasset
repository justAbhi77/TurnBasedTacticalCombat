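; Player combat action that adds or removes a unit on the clicked grid tile, depending on IsAddingUnit.
; When adding, it checks that the tile type is valid for the chosen UnitType, destroys any unit already there, then spawns a BP_Unit and registers it with the CombatSystem at that index.
; When removing, it takes any unit on the tile out of combat and destroys it.
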(fn ConstructionScript
  (|CallParentFunction))

(fn FExecuteAction
  (params (index :type Int%20Point%20Structure))
  (bind _playeractions (Variables|Default|GetPlayerActions))
  (bind _grid (Variables|/Game/Blueprints/Core/Player/BP_PlayerActions.BP_PlayerActions_C|GetGrid _playeractions))
  (bind _gridtiles (Variables|/Game/Blueprints/Core/Grid/BP_Grid.BP_Grid_C|GetGridTiles _grid))
  (bind _value (Utilities|Map|Find _gridtiles index))
  (bind _unitontile (Utilities|Struct|BreakStruct_TileData _value))
  (|CallParentFunction index)
  (if (Variables|Default|GetbIsAddingUnit)
    (bind _unitdata (CallFunction|FGetDefaultUnitDatafromUnitType (Variables|Default|GetUnitType)))
    (if (Utilities|Array|ContainsItem (.validtiletypes (.stats _unitdata)) (.tiletype (.Value (Utilities|Map|Find (Variables|/Game/Blueprints/Core/Grid/BP_Grid.BP_Grid_C|GetGridTiles (Variables|/Game/Blueprints/Core/Player/BP_PlayerActions.BP_PlayerActions_C|GetGrid (Variables|Default|GetPlayerActions))) index))))
      (Utilities|FlowControl|Sequence
        (:then_0
          (Utilities|IsValid _unitontile :!label _label
            (:Is%20Valid
              (Default|FRemoveUnitfromCombat (Variables|/Game/Blueprints/Core/Player/BP_PlayerActions.BP_PlayerActions_C|GetCombatSystem (Variables|Default|GetPlayerActions)) _unitontile true))))
        (:then_1
          (bind _returnvalue (Game|SpawnActorfromClass "/Game/Blueprints/Core/Units/BP_Unit.BP_Unit_C" (Math|Transform|MakeTransform "0, 0, 0" "0, 0, 0" "1.000000,1.000000,1.000000") "Undefined" "MultiplyWithRoot" 0 (Variables|Default|GetUnitType) 0))
          (Default|FAddUnitinCombat (Variables|/Game/Blueprints/Core/Player/BP_PlayerActions.BP_PlayerActions_C|GetCombatSystem (Variables|Default|GetPlayerActions)) _returnvalue index))))
    (else
      (goto _label))))