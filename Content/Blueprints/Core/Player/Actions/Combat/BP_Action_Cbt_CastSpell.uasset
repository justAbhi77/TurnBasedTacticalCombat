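; Player combat action for casting spells on the tile grid, previewing cast range and area of effect.
; Setting a spell loads its cast and AoE data, then marks tiles in range from the selected tile.
; Hovering refreshes the AoE highlight, shown only for in-range tiles and falling back to the hovered tile without a pattern.
; Executing casts through CombatSystem and deselects the spell in the combat UI; EndPlay clears both highlights.
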(event EventBeginPlay)

(event Collision|EventActorBeginOverlap
  (params (OtherActor :type Actor%20Object%20Reference)))

(event EventTick
  (params (DeltaSeconds :type Float%20%28single-precision%29)))

(event EventEndPlay
  (params (EndPlayReason :type EEndPlayReason%20Enum :default "Destroyed"))
  (bind _playeractions (Variables|Default|GetPlayerActions))
  (bind _grid (Variables|/Game/Blueprints/Core/Player/BP_PlayerActions.BP_PlayerActions_C|GetGrid _playeractions))
  (|CallParentFunction EndPlayReason)
  (Default|FClearStatefromTiles _grid "NewEnumerator9")
  (Default|FClearStatefromTiles _grid "NewEnumerator10"))

(fn ConstructionScript
  (|CallParentFunction))

(fn FSetSpell
  (params (Spell :type E_Spells%20Enum :default "NewEnumerator0"))
  (bind _playeractions (Variables|Default|GetPlayerActions))
  (bind _grid (Variables|/Game/Blueprints/Core/Player/BP_PlayerActions.BP_PlayerActions_C|GetGrid _playeractions))
  (bind _output_get (Variables|Default|SetSpell Spell))
  (if (Utilities|Enum|NotEqual(Enum) _output_get "NewEnumerator0")
    (bind _spelldata (CallFunction|FGetSpellDatafromSpell Spell))
    (Variables|Default|SetSpell%20Data%20Cast (.cast _spelldata))
    (Variables|Default|SetSpell%20Data%20Cast%20Aoe (.castaoe _spelldata))
    (CallFunction|FShowSpellRangePattern)
    (else
      (Default|FClearStatefromTiles _grid "NewEnumerator9")
      (Default|FClearStatefromTiles _grid "NewEnumerator10"))))

(fn FShowSpellRangePattern
  (bind _playeractions (Variables|Default|GetPlayerActions))
  (Utilities|FlowControl|Sequence
    (:then_0
      (Default|FClearStatefromTiles (Variables|/Game/Blueprints/Core/Player/BP_PlayerActions.BP_PlayerActions_C|GetGrid (Variables|Default|GetPlayerActions)) "NewEnumerator9")
      (bind _rangesindexes (Default|FGetSpellRange (Variables|/Game/Blueprints/Core/Player/BP_PlayerActions.BP_PlayerActions_C|GetCombatSystem _playeractions) (Variables|/Game/Blueprints/Core/Player/BP_PlayerActions.BP_PlayerActions_C|GetSelectedTile _playeractions) (Variables|Default|GetSpell%20Data%20Cast)))
      (for _array_element _rangesindexes
        (Default|FAddStatetoTile (Variables|/Game/Blueprints/Core/Player/BP_PlayerActions.BP_PlayerActions_C|GetGrid (Variables|Default|GetPlayerActions)) _array_element "NewEnumerator9")))
    (:then_1
      (CallFunction|FShowSpellRangePatternAoe))))

(fn FExecuteAction
  (params (index :type Int%20Point%20Structure))
  (|CallParentFunction index)
  (Default|FCastSpell (Variables|/Game/Blueprints/Core/Player/BP_PlayerActions.BP_PlayerActions_C|GetCombatSystem (Variables|Default|GetPlayerActions)) (Variables|Default|GetSpell) (Variables|/Game/Blueprints/Core/Player/BP_PlayerActions.BP_PlayerActions_C|GetSelectedTile (Variables|Default|GetPlayerActions)) index)
  (bind _wbpcombat (Variables|/Game/Blueprints/Core/Player/BP_PlayerActions.BP_PlayerActions_C|GetWBPCombat (Variables|Default|GetPlayerActions))
    (:then
      (Default|FSetSelectedSpellfromIndex (Variables|/Game/Blueprints/Core/Combat/Widgets/WBP_Combat.WBP_Combat_C|GetWBP_ButtonList_Spells _wbpcombat) -1))
    (:else)))

(fn FShowSpellRangePatternAoe
  (bind _playeractions (Variables|Default|GetPlayerActions))
  (Default|FClearStatefromTiles (Variables|/Game/Blueprints/Core/Player/BP_PlayerActions.BP_PlayerActions_C|GetGrid (Variables|Default|GetPlayerActions)) "NewEnumerator10")
  (if (Utilities|Array|ContainsItem (Utilities|Struct|BreakStruct_IntPointArray (.Value (Utilities|Map|Find (Variables|/Game/Blueprints/Core/Grid/BP_Grid.BP_Grid_C|GetTileStateToIndexes (Variables|/Game/Blueprints/Core/Player/BP_PlayerActions.BP_PlayerActions_C|GetGrid (Variables|Default|GetPlayerActions))) "NewEnumerator9"))) (Variables|/Game/Blueprints/Core/Player/BP_PlayerActions.BP_PlayerActions_C|GetHoveredTile (Variables|Default|GetPlayerActions)))
    (if (Utilities|Enum|NotEqual(Enum) (.RangePattern (Utilities|Struct|BreakStruct_SpellData_Cast (Variables|Default|GetSpell%20Data%20Cast%20Aoe))) "NewEnumerator0")
      (bind _rangesindexes (Default|FGetSpellRange (Variables|/Game/Blueprints/Core/Player/BP_PlayerActions.BP_PlayerActions_C|GetCombatSystem _playeractions) (Variables|/Game/Blueprints/Core/Player/BP_PlayerActions.BP_PlayerActions_C|GetHoveredTile _playeractions) (Variables|Default|GetSpell%20Data%20Cast%20Aoe)))
      (for _array_element _rangesindexes
        (Default|FAddStatetoTile (Variables|/Game/Blueprints/Core/Player/BP_PlayerActions.BP_PlayerActions_C|GetGrid (Variables|Default|GetPlayerActions)) _array_element "NewEnumerator10"))
      (else
        (Default|FAddStatetoTile (Variables|/Game/Blueprints/Core/Player/BP_PlayerActions.BP_PlayerActions_C|GetGrid (Variables|Default|GetPlayerActions)) (Variables|/Game/Blueprints/Core/Player/BP_PlayerActions.BP_PlayerActions_C|GetHoveredTile (Variables|Default|GetPlayerActions)) "NewEnumerator10")))))

(fn FExecuteHoveredAction
  (params (index :type Int%20Point%20Structure))
  (|CallParentFunction index)
  (CallFunction|FShowSpellRangePatternAoe))