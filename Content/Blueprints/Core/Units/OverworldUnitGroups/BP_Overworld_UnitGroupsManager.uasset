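; Overworld manager that keeps units in groups by ID so they share hover state and move together.
; Adding or removing units updates the group map and event bindings, with destroyed units leaving automatically.
; When one unit walks, encounter groups scatter around its target while others follow in a chain; switching to encounter starts random roaming.
; Propagation temporarily unbinds each receiving unit's event to avoid recursive callbacks.
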(event EventBeginPlay)

(fn ConstructionScript)

(fn FAddUnittoGroup
  (params (Unit :type BP%20Unit%20Object%20Reference) (GroupId :type Integer))
  (if (!= GroupId (Variables|/Game/Blueprints/Core/Units/BP_Unit.BP_Unit_C|GetOverworldGroupId Unit))
    (CallFunction|FRemoveUnitfromCurrentGroup Unit)
    (if (!= GroupId -999)
      (bind _output_get (LocalVariables|SetGroup (.Value (Utilities|Map|Find (Variables|Default|GetUnitGroups) GroupId))))
      (Utilities|Array|Add (.Units (Utilities|Struct|BreakStruct_OverworldUnitGroup _output_get)) Unit)
      (Utilities|Map|Add (Variables|Default|GetUnitGroups) GroupId (LocalVariables|GetGroup))
      (Variables|/Game/Blueprints/Core/Units/BP_Unit.BP_Unit_C|SetOverworldGroupId Unit GroupId)
      (Game|BindEventtoOnDestroyed Unit (EventDispatchers|CreateEvent :!event FonUnitDestroyed))
      (EventDispatchers|BindEventtoOnUnitHoveredChanged Unit (EventDispatchers|CreateEvent :!event FonUnitHoveredChanged))
      (EventDispatchers|BindEventtoOnUnitStartedWalkingOverworld Unit (EventDispatchers|CreateEvent :!event FonUnitStartedWalkingOverworld)))))

(fn FRemoveUnitfromCurrentGroup
  (params (Unit :type BP%20Unit%20Object%20Reference))
  (if (!= (Variables|/Game/Blueprints/Core/Units/BP_Unit.BP_Unit_C|GetOverworldGroupId Unit) -999)
    (bind _output_get (LocalVariables|SetGroup (.Value (Utilities|Map|Find (Variables|Default|GetUnitGroups) (Variables|/Game/Blueprints/Core/Units/BP_Unit.BP_Unit_C|GetOverworldGroupId Unit)))))
    (Utilities|Array|RemoveItem (.Units (Utilities|Struct|BreakStruct_OverworldUnitGroup _output_get)) Unit)
    (Utilities|FlowControl|Sequence
      (:then_0
        (if (> (Utilities|Array|Length (.Units (Utilities|Struct|BreakStruct_OverworldUnitGroup _output_get))) 0)
          (Utilities|Map|Add (Variables|Default|GetUnitGroups) (Variables|/Game/Blueprints/Core/Units/BP_Unit.BP_Unit_C|GetOverworldGroupId Unit) (LocalVariables|GetGroup))
          (else
            (Utilities|Map|Remove (Variables|Default|GetUnitGroups) (Variables|/Game/Blueprints/Core/Units/BP_Unit.BP_Unit_C|GetOverworldGroupId Unit)))))
      (:then_1
        (Variables|/Game/Blueprints/Core/Units/BP_Unit.BP_Unit_C|SetOverworldGroupId Unit -999)
        (EventDispatchers|UnbindEventfromOnUnitHoveredChanged Unit (EventDispatchers|CreateEvent :!event FonUnitHoveredChanged))
        (EventDispatchers|UnbindEventfromOnUnitStartedWalkingOverworld Unit (EventDispatchers|CreateEvent :!event FonUnitStartedWalkingOverworld))))))

(fn FonUnitDestroyed
  (params (DestroyedActor :type Actor%20Object%20Reference))
  (bind _asbp_unit (Utilities|Casting|CastToBP_Unit DestroyedActor))
  (CallFunction|FRemoveUnitfromCurrentGroup _asbp_unit))

(fn FonUnitHoveredChanged
  (params (Unit :type BP%20Unit%20Object%20Reference))
  (bind _overworldgroupid (Variables|/Game/Blueprints/Core/Units/BP_Unit.BP_Unit_C|GetOverworldGroupId Unit))
  (bind _unitgroups (Variables|Default|GetUnitGroups))
  (bind (_value _returnvalue) (Utilities|Map|Find _unitgroups _overworldgroupid))
  (if _returnvalue
    (bind _output_get (LocalVariables|SetGroup _value))
    (for _array_element (.Units (Utilities|Struct|BreakStruct_OverworldUnitGroup _output_get))
      (LocalVariables|SetU _array_element)
      (if (!= (LocalVariables|GetU) Unit)
        (EventDispatchers|UnbindEventfromOnUnitHoveredChanged (LocalVariables|GetU) (EventDispatchers|CreateEvent :!event FonUnitHoveredChanged))
        (Default|FSetIsHovered (LocalVariables|GetU) (Variables|/Game/Blueprints/Core/Units/BP_Unit.BP_Unit_C|GetbIsHovered Unit))
        (EventDispatchers|BindEventtoOnUnitHoveredChanged (LocalVariables|GetU) (EventDispatchers|CreateEvent :!event FonUnitHoveredChanged))))))

(fn FonUnitStartedWalkingOverworld
  (params (Unit :type BP%20Unit%20Object%20Reference))
  (if (Utilities|Struct|BreakStruct_OverworldUnitGroup (.Value (Utilities|Map|Find (Variables|Default|GetUnitGroups) (Variables|/Game/Blueprints/Core/Units/BP_Unit.BP_Unit_C|GetOverworldGroupId Unit))))
    (for _array_element (.Units (Utilities|Struct|BreakStruct_OverworldUnitGroup (.Value (Utilities|Map|Find (Variables|Default|GetUnitGroups) (Variables|/Game/Blueprints/Core/Units/BP_Unit.BP_Unit_C|GetOverworldGroupId Unit)))))
      (LocalVariables|SetU _array_element)
      (if (!= (LocalVariables|GetU) Unit)
        (EventDispatchers|UnbindEventfromOnUnitStartedWalkingOverworld (LocalVariables|GetU) (EventDispatchers|CreateEvent :!event FonUnitStartedWalkingOverworld))
        (bind _randomlocation (Default|FGetRandomReachableLocationinRadius (LocalVariables|GetU) (Variables|/Game/Blueprints/Core/Units/BP_Unit.BP_Unit_C|GetTargetLocationInOverworld Unit) "(X=100.000000,Y=400.000000)"))
        (Default|EMoveUnitinOverworld (LocalVariables|GetU) _randomlocation 0 false)
        (EventDispatchers|BindEventtoOnUnitStartedWalkingOverworld (LocalVariables|GetU) (EventDispatchers|CreateEvent :!event FonUnitStartedWalkingOverworld))))
    (else
      (LocalVariables|SetPreviousUnitInChain Unit)
      (for _array_element_2 (.Units (Utilities|Struct|BreakStruct_OverworldUnitGroup (.Value (Utilities|Map|Find (Variables|Default|GetUnitGroups) (Variables|/Game/Blueprints/Core/Units/BP_Unit.BP_Unit_C|GetOverworldGroupId Unit)))))
        (LocalVariables|SetU _array_element_2)
        (if (!= (LocalVariables|GetU) Unit)
          (EventDispatchers|UnbindEventfromOnUnitStartedWalkingOverworld (LocalVariables|GetU) (EventDispatchers|CreateEvent :!event FonUnitStartedWalkingOverworld))
          (Default|EMoveUnitinOverworld (LocalVariables|GetU) "0, 0, 0" (LocalVariables|GetPreviousUnitInChain) false)
          (LocalVariables|SetPreviousUnitInChain (LocalVariables|GetU))
          (EventDispatchers|BindEventtoOnUnitStartedWalkingOverworld (LocalVariables|GetU) (EventDispatchers|CreateEvent :!event FonUnitStartedWalkingOverworld)))))))

(fn FSetGroupIsEncounter
  (params (bIsEncounter :type Boolean) (GroupId :type Integer))
  (bind _unitgroups (Variables|Default|GetUnitGroups))
  (bind (_value _returnvalue) (Utilities|Map|Find _unitgroups GroupId))
  (if _returnvalue
    (bind _output_get (LocalVariables|SetGroup _value))
    (if (!= (Utilities|Struct|BreakStruct_OverworldUnitGroup _output_get) bIsEncounter)
      (Utilities|Struct|SetmembersinStruct_OverworldUnitGroup (LocalVariables|GetGroup) bIsEncounter)
      (Utilities|Map|Add (Variables|Default|GetUnitGroups) GroupId (LocalVariables|GetGroup))
      (for _array_element (Utilities|Struct|BreakStruct_OverworldUnitGroup (LocalVariables|GetGroup))
        (Default|EStopMovingUnitinOverworld _array_element))
      (if (.bIsEncounter (Utilities|Struct|BreakStruct_OverworldUnitGroup (LocalVariables|GetGroup)))
        (Default|EMoveUnitinOverworld (Utilities|Array|Get(acopy) (.Units (Utilities|Struct|BreakStruct_OverworldUnitGroup (LocalVariables|GetGroup)))) "0, 0, 0" 0 true)))))