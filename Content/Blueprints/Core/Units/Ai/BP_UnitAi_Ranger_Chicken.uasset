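; Combat AI for the Chicken Ranger unit, which withholds one randomly chosen spell for each combat.
; At combat start it picks AvailableRandomSpell from the available spells and prints it, and the FGetAvailableSpells override removes it from the parent's list.
; The decision-done event only calls the parent; disconnected logic would score that spell across its range as a fallback, using time-sliced delays.
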(event EventEDecideWhichSpelltoCastDone
  (|CallParentFunction))

(fn ConstructionScript
  (|CallParentFunction))

(fn FGetAvailableSpells
  (bind _output_get (LocalVariables|SetRet (|CallParentFunction)))
  (Utilities|Array|RemoveItem _output_get (Variables|Default|GetAvailableRandomSpell))
  (return (LocalVariables|GetRet)))

(fn FAiCombatStarted
  (|CallParentFunction)
  (bind _output_get (Variables|Default|SetAvailableRandomSpell (.OutItem (Utilities|Array|Random (CallFunction|FGetAvailableSpells)))))
  (Development|PrintString (Utilities|String|Append "Until Will not Cast This Spell For Combat " (Utilities|String|EnumtoString _output_get)) true true "(R=0.000000,G=0.660000,B=1.000000,A=1.000000)" 5.0))