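; Ranger unit AI Blueprint that varies the unit's movement logic by turn number and whether it has dealt damage, extending a parent AI class.
; A turn counter resets at combat start and increments each turn, which also clears the damage flag.
; Casting a spell with a negative minimum HP modifier sets the flag.
; Movement logic switches to an alternate mode on even turns while the flag is unset.
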(event EventECastSpell
  (bind _spelldata (CallFunction|FGetSpellDatafromSpell (Utilities|Struct|BreakStruct_UnitAiSpellCastingData (Variables|Default|GetAiSpellCasting))))
  (Variables|Default|SetbDamagedUnitThisTurn (or (< (.X (Utilities|Struct|BreakIntPoint (Utilities|Struct|BreakStruct_SpellData_Impact (Utilities|Struct|BreakStruct_SpellData _spelldata)))) 0) (Variables|Default|GetbDamagedUnitThisTurn)))
  (|CallParentFunction))

(fn ConstructionScript
  (|CallParentFunction))

(fn FAiPlayTurn
  (Math|Integer|IncrementInt (Variables|Default|GetTurnCount)
    (:%20%20
      (Variables|Default|SetbDamagedUnitThisTurn false)
      (|CallParentFunction))))

(fn FGetUnitMovementLogic
  (return (select (and (CallFunction|FIsIntEven (Variables|Default|GetTurnCount)) (not (Variables|Default|GetbDamagedUnitThisTurn))) "NewEnumerator0" "NewEnumerator2")))

(fn FAiCombatStarted
  (Variables|Default|SetTurnCount 0)
  (|CallParentFunction))